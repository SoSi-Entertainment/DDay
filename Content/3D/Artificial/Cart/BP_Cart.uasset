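; BP_Cart is a cart prop with an optional hay mesh, toggled by the HayOnOff flag.
; The construction script sets the hay's collision from the flag and hides the mesh when off, but never explicitly shows it when on.
; BeginPlay reapplies the flag, setting both collision and visibility in either state.
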(event `self.ReceiveBeginPlay`
  (bind _sm_carthay (`self.SM_CartHay`))
  (if (`self.Hay On/Off`)
    (`PrimitiveComponent.SetCollisionEnabled` _sm_carthay "QueryAndPhysics")
    (`SceneComponent.SetVisibility` _sm_carthay true false)
    (else
      (`PrimitiveComponent.SetCollisionEnabled` _sm_carthay "NoCollision")
      (`SceneComponent.SetVisibility` _sm_carthay false false))))

(fn `UserConstructionScript`
  (bind _sm_carthay (`self.SM_CartHay`))
  (if (`self.Hay On/Off`)
    (`PrimitiveComponent.SetCollisionEnabled` _sm_carthay "QueryAndPhysics")
    (else
      (`PrimitiveComponent.SetCollisionEnabled` _sm_carthay "NoCollision")
      (`SceneComponent.SetVisibility` _sm_carthay false false))))