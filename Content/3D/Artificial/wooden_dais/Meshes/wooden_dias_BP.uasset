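; Wooden dais prop built from several stick meshes, with an adjustable wood tone.
; The construction script calls Set Tone, which reuses or creates one dynamic material instance, shares it across the stick meshes and sets its Tone parameter.
; Random Tone picks a value within Tone Interval in 0.1 steps and reapplies it, though nothing in this graph calls it.
; A custom Destroy event removes the actor.
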(event `/Game/Blueprints/System/Interfaces/Explosion_Desructable.Destroy`
  (`self.K2_DestroyActor`))

(fn `Random tone`
  (bind (_from _to) (break `/Game/Data/structs/Proportion_Interval` (`self.Tone Interval`)))
  (set `self.Tone` (/ (`KismetMathLibrary.Conv_IntToDouble` (`KismetMathLibrary.RandomIntegerInRange` (`KismetMathLibrary.FTrunc` (* _from 10.0)) (`KismetMathLibrary.FTrunc` (* _to 10.0)))) 10.0))
  (`self.Set tone`))

(fn `Set tone`
  (bind _wooden_dais_stick3_low (`self.wooden_dais_stick3_low`))
  (bind _returnvalue (`PrimitiveComponent.GetMaterial` _wooden_dais_stick3_low 0))
  (`/Engine/EditorBlueprintResources/StandardMacros.IsValid` _returnvalue
    (:`Is Valid`
      (bind _asmaterial_instance_dynamic (cast `MaterialInstanceDynamic` _returnvalue)
        (:`then`
          (`PrimitiveComponent.SetMaterial` _wooden_dais_stick3_low 0 _asmaterial_instance_dynamic)
          (`PrimitiveComponent.SetMaterial` (`self.wooden_dais_stick2_low1`) 0 _asmaterial_instance_dynamic)
          (`PrimitiveComponent.SetMaterial` (`self.wooden_dais_stick3_low1`) 0 _asmaterial_instance_dynamic)
          (`PrimitiveComponent.SetMaterial` (`self.wooden_dais_down_stick_low1`) 0 _asmaterial_instance_dynamic)
          (`PrimitiveComponent.SetMaterial` (`self.wooden_dais_stick4_low`) 0 _asmaterial_instance_dynamic)
          (`PrimitiveComponent.SetMaterial` (`self.wooden_dais_down_stick_low`) 0 _asmaterial_instance_dynamic)
          (`PrimitiveComponent.SetMaterial` (`self.wooden_dais_stick1_low`) 0 _asmaterial_instance_dynamic)
          (`PrimitiveComponent.SetMaterial` (`self.wooden_dais_stick2_low`) 0 _asmaterial_instance_dynamic)
          (`PrimitiveComponent.SetMaterial` (`self.wooden_dais_stick3_low`) 0 _asmaterial_instance_dynamic)
          (`MaterialInstanceDynamic.SetScalarParameterValue` _asmaterial_instance_dynamic "Tone" (`self.Tone`)))
        (:`CastFailed`
          (bind _returnvalue_2 (`KismetMaterialLibrary.CreateDynamicMaterialInstance` _returnvalue))
          (`MaterialInstanceDynamic.SetScalarParameterValue` _returnvalue_2 "Tone" (`self.Tone`))
          (`/Engine/EditorBlueprintResources/StandardMacros.IsValid` _returnvalue_2
            (:`Is Valid`
              (`PrimitiveComponent.SetMaterial` (`self.wooden_dais_stick3_low`) 0 _returnvalue_2)
              (`PrimitiveComponent.SetMaterial` (`self.wooden_dais_stick2_low`) 0 _returnvalue_2)
              (`PrimitiveComponent.SetMaterial` (`self.wooden_dais_stick1_low`) 0 _returnvalue_2)
              (`PrimitiveComponent.SetMaterial` (`self.wooden_dais_down_stick_low`) 0 _returnvalue_2)
              (`PrimitiveComponent.SetMaterial` (`self.wooden_dais_stick4_low`) 0 _returnvalue_2)
              (`PrimitiveComponent.SetMaterial` (`self.wooden_dais_down_stick_low1`) 0 _returnvalue_2)
              (`PrimitiveComponent.SetMaterial` (`self.wooden_dais_stick3_low1`) 0 _returnvalue_2)
              (`PrimitiveComponent.SetMaterial` (`self.wooden_dais_stick2_low1`) 0 _returnvalue_2))))))))

(fn `UserConstructionScript`
  (`self.Set tone`))