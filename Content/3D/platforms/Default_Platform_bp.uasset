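; Default platform actor that looks up its parent actor as a Tile and provides press, hide and highlight behavior.
; Press and unpress drive a timeline that moves the mesh vertically, with a short delay before it returns.
; Ownhide sets opacity on a dynamic material, animated or instant, and switches one collision channel between Ignore and Block.
; SetHiglight sets highlight color and intensity on the same material.
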(event `self.ReceiveBeginPlay`
  (`/Engine/EditorBlueprintResources/StandardMacros.IsValid` (`self.dynamic material`)
    (:`Is Not Valid`
      (bind _returnvalue (`PrimitiveComponent.CreateDynamicMaterialInstance` (`self.platform_mesh`) 0 null "None"))
      (set `self.dynamic material` _returnvalue))))

(event `press`
  (bind (_direction _press) (`Timeline|Timeline` :!label _label)
    (:`Update`
      (`SceneComponent.K2_SetRelativeLocation` (`self.platform_mesh`) (`KismetMathLibrary.MakeVector` 0.0 0.0 _press) false false))))

(event `unpress`
  (`KismetSystemLibrary.Delay` 0.7)
  (goto _label :!via `Reverse`))

(event `/Game/3D/platforms/Hidable.Create dinamic material`
  (params (Ruller :type "/Game/Blueprints/Logics/Hide_Area Object Reference"))
  (`/Engine/EditorBlueprintResources/StandardMacros.IsValid` (`self.dynamic material`)
    (:`Is Not Valid`
      (bind _returnvalue (`PrimitiveComponent.CreateDynamicMaterialInstance` (`self.platform_mesh`) 0 null "None"))
      (set `self.dynamic material` _returnvalue))))

(event `/Game/3D/platforms/Hidable.Hide`
  (params (Hided :type Boolean) (`Use animation` :type Boolean)))

(event `Own hide`
  (params (Hiden :type Boolean) (`use animation` :type Boolean))
  (bind _hide_coef (`self.Hide coef`))
  (if `use animation`
    (if Hiden
      (bind (_direction _newtrack_0) (`Timeline|Timeline_0` :!label _label_2)
        (:`Update`
          (`MaterialInstanceDynamic.SetScalarParameterValue` (`self.dynamic material`) "Opacity" (`KismetMathLibrary.SelectFloat` (+ _hide_coef (* (- 1.0 _hide_coef) _newtrack_0)) (`KismetMathLibrary.SelectFloat` (`self.Hide coef`) 1.0 Hiden) `use animation`) :!label _label_3)
          (`PrimitiveComponent.SetCollisionResponseToChannel` (`self.platform_mesh`) "ECC_GameTraceChannel7" (select `bool` Hiden :`false` "ECR_Block" :`true` "ECR_Ignore" :!type "ECollisionResponse Enum"))))
      (else
        (goto _label_2 :!via `ReverseFromEnd`)))
    (else
      (goto _label_3))))

(fn `Get tile`
  (returns (Tile :type "/Game/3D/platforms/Tile Object Reference"))
  (return (cast `/Game/3D/platforms/Tile` (`self.GetParentActor`) :!pure true)))

(fn `Set Higlight`
  (params (color :type "LinearColor Structure") (intense :type "Float (double-precision)"))
  (bind _dynamic_material (`self.dynamic material`))
  (`MaterialInstanceDynamic.SetScalarParameterValue` _dynamic_material "HighlightIntense" intense)
  (`MaterialInstanceDynamic.SetVectorParameterValue` _dynamic_material "HighlightColor" color))

(fn `UserConstructionScript`)