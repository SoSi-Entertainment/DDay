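; Undead proximity mine that explodes after a Base_Character from another team, or any team with BothTeamTrigger set, overlaps it.
; After the Timer delay it applies radial damage with falloff, ignoring only itself and using Pawn as the damage prevention channel.
; Explode then plays a sound, spawns two differently scaled Blast_bp actors and a flattened Blood_bp, and destroys the mine.
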(event `self.ReceiveActorBeginOverlap`
  (params (OtherActor :type "Actor Object Reference"))
  (bind _asbase_character (cast `/Game/Blueprints/Chars/Base_Character` OtherActor))
  (if (or (`|EnumInequality` (`/Game/Blueprints/Chars/Base_Character.Team` _asbase_character) (`self.Team`)) (`self.Both team trigger`))
    (`KismetSystemLibrary.Delay` (`self.Timer`))
    (`GameplayStatics.ApplyRadialDamageWithFalloff` (`self.Damage`) 0.0 (`self.K2_GetActorLocation`) 0.0 (`self.Radius`) 2.0 null (`|MakeArray` self :!type "Actor Object Reference") null null "ECC_Pawn")
    (`self.Explode`)))

(fn `Explode`
  (bind _returnvalue (`self.K2_GetActorLocation`))
  (bind _returnvalue_2 (+ _returnvalue (0.0 0.0 0.0)))
  (`GameplayStatics.PlaySoundAtLocation` "/Game/Movies/mine_explosion_sound.mine_explosion_sound" _returnvalue (struct) 1.0 1.0 0.0 null null null null)
  (`|SpawnActorFromClass` "/Game/Effects/blast_bp.blast_bp_C" (`KismetMathLibrary.MakeTransform` _returnvalue_2) "Undefined" "MultiplyWithRoot" null null)
  (`|SpawnActorFromClass` "/Game/Effects/blast_bp.blast_bp_C" (`KismetMathLibrary.MakeTransform` _returnvalue_2 (struct :`Yaw` 60.0) (1.5 1.5 1.5)) "Undefined" "MultiplyWithRoot" null null)
  (`|SpawnActorFromClass` "/Game/Effects/blood_bp.blood_bp_C" (`KismetMathLibrary.MakeTransform` _returnvalue (struct) (3.0 3.0 0.01)) "Undefined" "MultiplyWithRoot" null null)
  (`self.K2_DestroyActor`))

(fn `UserConstructionScript`)