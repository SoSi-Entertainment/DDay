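; Key holder Blueprint that tracks which movement inputs are held and reports the current navigation direction.
; The forward, backward, right and left action events add a direction enum to a Keys array on press and remove it on release.
; GetDirection returns the last entry, so the most recently pressed held key wins, or a fifth fallback enum value when the array is empty.
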(event `self.ReceiveTick`
  (params (DeltaSeconds :type "Float (single-precision)")))

(event `InputAction|GoForward`
  (params (Key :type "Key Structure"))
  (bind _keys (`self.Keys`))
  (:`Pressed`
    (`KismetArrayLibrary.Array_Add` _keys "NewEnumerator0"))
  (:`Released`
    (`KismetArrayLibrary.Array_RemoveItem` _keys "NewEnumerator0")))

(event `InputAction|GoBackward`
  (params (Key :type "Key Structure"))
  (bind _keys (`self.Keys`))
  (:`Pressed`
    (`KismetArrayLibrary.Array_Add` _keys "NewEnumerator1"))
  (:`Released`
    (`KismetArrayLibrary.Array_RemoveItem` _keys "NewEnumerator1")))

(event `InputAction|GoRight`
  (params (Key :type "Key Structure"))
  (bind _keys (`self.Keys`))
  (:`Pressed`
    (`KismetArrayLibrary.Array_Add` _keys "NewEnumerator2"))
  (:`Released`
    (`KismetArrayLibrary.Array_RemoveItem` _keys "NewEnumerator2")))

(event `InputAction|GoLeft`
  (params (Key :type "Key Structure"))
  (bind _keys (`self.Keys`))
  (:`Pressed`
    (`KismetArrayLibrary.Array_Add` _keys "NewEnumerator3"))
  (:`Released`
    (`KismetArrayLibrary.Array_RemoveItem` _keys "NewEnumerator3")))

(fn `Get Direction`
  (returns (NewParam :type "/Game/Data/enums/Dirrection Enum"))
  (bind _keys (`self.Keys`))
  (if (> (`KismetArrayLibrary.Array_Length` _keys) 0)
    (return (`|GetArrayItem` _keys (`KismetArrayLibrary.Array_LastIndex` _keys)))
    (else
      (return "NewEnumerator4"))))