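; Player controller for the DDay game, driving the character's grid movement, mouse aiming, shooting and pause.
; On start it possesses a fixed spectator pawn for the camera and hands the body to a spawned AI controller, whose grid navigator it steps tile by tile.
; Each tick it aims the gun and saves the player's state to a black box recorder.
; Debug keys toggle cheats or kill the player.
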(event `self.ReceiveBeginPlay`
  (bind _returnvalue (subsystem `EnhancedInputLocalPlayerSubsystem`))
  (bind _asdday_instance (cast `/Game/Blueprints/System/DDay_Instance` (`GameplayStatics.GetGameInstance`) :!pure true))
  (bind _grid_navigator (`/Game/Blueprints/Navigation/Player_AI_Controller.Grid_Navigator` (`self.Slave Ai`)))
  (`self.Block input`)
  (`self.Swap on ai controller`)
  (set `self.bShowMouseCursor` true)
  ;[1 1 1] Black box set up
  (bind _black_box (`/Game/Blueprints/System/DDay_Instance.New Box` _asdday_instance))
  (set `self.Black box` _black_box)
  (`KismetSystemLibrary.Delay` (`/Game/Blueprints/System/DDay_Instance.Player Spawn Delay` _asdday_instance))
  (`self.Unblock input`)
  ;[0.05098 0.05098 0.05098] Add Mapping Context
  (`/Engine/EditorBlueprintResources/StandardMacros.IsValid` _returnvalue
    (:`Is Valid`
      (`EnhancedInputSubsystemInterface.AddMappingContext` _returnvalue "/Game/Default/Input/IMC_Default.IMC_Default" 0 (struct))
      ;[1 1 1] Player movement control
      (bind _newparam (`/Game/Blueprints/Navigation/Key_Holder.Get Direction` (`self.Key_Holder`) :!label _label))
      (if (`/Game/Blueprints/Chars/Base_Character.Dead` (`self.Body`))
        _
        (elif (or (`|EnumEquality` _newparam "NewEnumerator4") (`self.Input blocked`))
          (`KismetSystemLibrary.Delay` 0.01)
          (goto _label)
          (else
            (`/Game/Blueprints/Navigation/Grid_Navigator.Go` _grid_navigator _newparam)
            (`/Game/Blueprints/System/DDayMacroLibrary.Wait condition` (`/Game/Blueprints/Navigation/Grid_Navigator.OnTile` _grid_navigator)
              (:`true`
                (goto _label)))))))))

(event `self.ReceivePossess`
  (params (PossessedPawn :type "Pawn Object Reference"))
  ;[1 1 1] Set body
  (bind _asmain_character (cast `/Game/Blueprints/Chars/Main_Character` PossessedPawn))
  (set `self.Body` _asmain_character))

(event `self.ReceiveTick`
  (params (DeltaSeconds :type "Float (single-precision)"))
  (bind _body (`self.Body`))
  (bind _body_2 (`self.Body`))
  (bind _new_aim_mode (`self.New aim mode`))
  ;[1 1 1] Save player state every frame
  (if (not (`/Game/Blueprints/Chars/Base_Character.Dead` _body))
    (if _new_aim_mode
      (if (not (`self.Input blocked`)) :!label _label_2
        (bind _rotation (`/Game/Blueprints/Chars/Base_Character.Set gun angle` _body (`KismetMathLibrary.SelectRotator` (`self.Shooting direction by mouse on screen`) (`self.Shooting direction by under cursor`) _new_aim_mode))))
      (elif (< (`KismetMathLibrary.Vector_Distance` (`.Location` (`self.GetLocationUnderCursor`)) (`/Game/Blueprints/Chars/Base_Character.Endpoint Location` _body_2)) 100.0)
        _
        (else
          (goto _label_2))))
    (`/Game/Blueprints/recording/Black_Box.Save Frame` (`self.Black box`) (`self.K2_GetActorLocation` _body_2) (.yaw (`self.K2_GetActorRotation` _body_2)) _rotation (`self.Shooting`))))

(event `EnhancedInput|/Game/Default/Input/Actions/IA_SetDestination_Click`
  (params (ActionValue :type Boolean) (ElapsedSeconds :type "Float (double-precision)") (TriggeredSeconds :type "Float (double-precision)") (InputAction :type "InputAction Object Reference" :default "/Game/Default/Input/Actions/IA_SetDestination_Click.IA_SetDestination_Click"))
  (bind _input_blocked (`self.Input blocked`))
  ;[1 1 1] gun shooting
  (:`Triggered`
    (if (not _input_blocked)
      (bind _done (`/Game/Blueprints/Chars/Base_Character.Shoot` (`self.Body`) (0.0 0.0 0.0)))
      (if _done
        (`GameplayStatics.PlaySound2D` "/Game/Movies/one_shot_tommy.one_shot_tommy" 0.2 1.0 0.0 null null))))
  (:`Started`
    (if (not _input_blocked)
      (set `self.Shooting` true)))
  (:`Canceled`
    (set `self.Shooting` false :!label _label_3))
  (:`Completed`
    (goto _label_3)))

(event `InputAction|Quit`
  (params (Key :type "Key Structure"))
  ;[1 1 1] Pressed Quit-button
  (:`Pressed`
    (if (not (`self.Input blocked`))
      (`/Game/Blueprints/System/DDay_GameMode.Set pause` (cast `/Game/Blueprints/System/DDay_GameMode` (`GameplayStatics.GetGameMode`) :!pure true) true))))

(event `InputAction|Respawn`
  (params (Key :type "Key Structure"))
  ;[1 1 1] Respawn
  (:`Pressed`
    (`/Game/Blueprints/Chars/Base_Character.Die` (`self.Body`))))

(event `InputAction|Titan mode`
  (params (Key :type "Key Structure"))
  (bind _titan_mode (`self.Titan mode`))
  (bind _body (`self.Body`))
  ;[1 1 1] Titan mode
  (:`Pressed`
    (if _titan_mode
      (set `/Game/Blueprints/Chars/Base_Character.Health` 100.0 _body)
      (`KismetSystemLibrary.PrintString` "Titan mode: OFF" true true (struct :`R` 1.0 :`B` 0.007021 :`A` 1.0))
      (else
        (set `/Game/Blueprints/Chars/Base_Character.Health` 10000.0 _body)
        (`KismetSystemLibrary.PrintString` "Titan mode: ON" true true (struct :`R` 1.0 :`B` 0.007021 :`A` 1.0))))
    (set `self.Titan mode` (not _titan_mode))))

(event `InputAction|Graphic debug`
  (params (Key :type "Key Structure"))
  ;[1 1 1] Graphic debug
  (:`Pressed`
    (bind _asdday_instance (cast `/Game/Blueprints/System/DDay_Instance` (`GameplayStatics.GetGameInstance`)))
    (bind _debug_graphics (`/Game/Blueprints/System/DDay_Instance.Debug Graphics` _asdday_instance))
    (if _debug_graphics
      (`KismetSystemLibrary.PrintString` "Graphics Debug: OFF" true true (struct :`R` 1.0 :`B` 0.007021 :`A` 1.0))
      (else
        (`KismetSystemLibrary.PrintString` "Graphics Debug: ON" true true (struct :`R` 1.0 :`B` 0.007021 :`A` 1.0))))
    (set `/Game/Blueprints/System/DDay_Instance.Debug Graphics` (not _debug_graphics) _asdday_instance)))

(event `InputAction|Fast run`
  (params (Key :type "Key Structure"))
  (bind _fast_run (`self.Fast run`))
  (bind _charactermovement (`Character.CharacterMovement` (`self.Body`)))
  (bind _maxwalkspeed (`CharacterMovementComponent.MaxWalkSpeed` _charactermovement))
  ;[1 1 1] Fast run
  (:`Pressed`
    (if _fast_run
      (set `CharacterMovementComponent.MaxWalkSpeed` (/ _maxwalkspeed 5.0) _charactermovement)
      (`KismetSystemLibrary.PrintString` "Fast run: OFF" true true (struct :`R` 1.0 :`B` 0.007021 :`A` 1.0))
      (else
        (set `CharacterMovementComponent.MaxWalkSpeed` (* _maxwalkspeed 5.0) _charactermovement)
        (`KismetSystemLibrary.PrintString` "Fast run: ON" true true (struct :`R` 1.0 :`B` 0.007021 :`A` 1.0))))
    (set `self.Fast run` (not _fast_run))))

(event `InputAxis|forward`
  (params (AxisValue :type "Float (single-precision)"))
  (bind _returnvalue (`Pawn.GetMovementComponent` (`self.Body`)))
  ;[1 1 1] debug move
  (set `MovementComponent.Velocity` (+ (* (`KismetMathLibrary.Normal` (`KismetMathLibrary.MakeVector` AxisValue (stale `InputAxis|right` AxisValue))) 20.0) (`MovementComponent.Velocity` _returnvalue)) _returnvalue :!label _label))

(event `InputAxis|right`
  (params (AxisValue :type "Float (single-precision)"))
  ;[1 1 1] debug move
  (goto _label))

(fn `Block input`
  (set `self.Input blocked` true)
  (set `self.Shooting` false))

(fn `Follow`
  (params (Location :type "Vector Structure"))
  (bind _returnvalue (`self.K2_GetPawn`))
  (`Pawn.AddMovementInput` _returnvalue (`KismetMathLibrary.GetDirectionUnitVector` (`self.K2_GetActorLocation` _returnvalue) Location) 1.0 false))

(fn `GetLocationUnderCursor`
  (returns (Hit :type Boolean) (Location :type "Vector Structure"))
  (bind (_bblockinghit _binitialoverlap _time _distance _location) (`GameplayStatics.BreakHitResult` (`self.GetHitResultUnderCursorByChannel` "TraceTypeQuery1")))
  (return _bblockinghit _location))

(fn `MoveTo`
  (params (Location :type "Vector Structure"))
  (`AIBlueprintHelperLibrary.SimpleMoveToLocation` self Location)
  (`NiagaraFunctionLibrary.SpawnSystemAtLocation` (`self.FXCursor`) Location))

(fn `Shooting direction by mouse on screen`
  (returns (direction :type "Rotator Structure"))
  (bind (_locationx _locationy) (`self.GetMousePosition`))
  (bind _returnvalue (`KismetMathLibrary.Normal2D` (- (`KismetMathLibrary.MakeVector2D` _locationx _locationy) (/ (`WidgetLayoutLibrary.GetViewportSize`) 2.0))))
  (bind _returnvalue_2 (`KismetMathLibrary.DegAcos` (`KismetMathLibrary.DotProduct2D` _returnvalue (0.0 -1.0))))
  (return (`KismetMathLibrary.MakeRotator` 0.0 0.0 (`KismetMathLibrary.SelectFloat` (* _returnvalue_2 -1.0) _returnvalue_2 (> (`KismetMathLibrary.DegAcos` (`KismetMathLibrary.DotProduct2D` _returnvalue (1.0 -0.0))) 90.0)))))

(fn `Shooting direction by under cursor`
  (returns (direction :type "Rotator Structure"))
  (return (`KismetMathLibrary.MakeRotator` 0.0 0.0 (`KismetMathLibrary.RadiansToDegrees` (`KismetMathLibrary.Vector_HeadingAngle` (- (`.Location` (`self.GetLocationUnderCursor`)) (`/Game/Blueprints/Chars/Base_Character.Endpoint Location` (`self.Body`))))))))

(fn `Swap on ai controller`
  (bind _body (`self.Body`))
  (`self.UnPossess`)
  (bind _returnvalue (`|SpawnActorFromClass` "/Game/Blueprints/Navigation/Fixed_Spectator_Pawn.Fixed_Spectator_Pawn_C" (`KismetMathLibrary.Conv_VectorToTransform` (+ (`self.K2_GetActorLocation` (`self.Body`)) (0.0 0.0 100.0))) "Undefined" "MultiplyWithRoot" null null))
  (`self.Possess` _returnvalue)
  (set `self.Camera body` _returnvalue)
  (set `/Game/Blueprints/Navigation/Fixed_Spectator_Pawn.Body Camera` (`/Game/Blueprints/Chars/Main_Character.Camera` _body) _returnvalue)
  (bind _returnvalue_2 (`|SpawnActorFromClass` "/Game/Blueprints/Navigation/Player_AI_Controller.Player_AI_Controller_C" (`self.GetTransform` _body) "Undefined" "MultiplyWithRoot" null _body))
  (bind _output_get (set `self.Slave Ai` _returnvalue_2))
  (`self.Possess` _output_get _body))

(fn `Unblock input`
  (set `self.Input blocked` false))

(fn `UserConstructionScript`)