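; Path manager component for an AI controller that steers a Base_Character along a path of tiles.
; It tracks the possessed pawn and loads tile lists into a Path object, taking the first tile as the goal.
; GetDirection pulls the next goal once the body is close in 2D, then returns one of four axis-aligned directions along the dominant offset, or a separate value at path end.
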(event `self.ReceiveBeginPlay`
  (bind _asaicontroller (cast `AIController` (`self.GetOwner`)))
  (add `Controller.OnPossessedPawnChanged` _asaicontroller (delegate `controller possessed`))
  (bind _asbase_character (cast `/Game/Blueprints/Chars/Abstract/Base_Character` (`Controller.K2_GetPawn` _asaicontroller)))
  (bind _output_get (set `self.body` _asbase_character))
  (set `self.Goal` (`KismetMathLibrary.Conv_VectorToVector2D` (`Actor.K2_GetActorLocation` _output_get))))

(event `controller possessed`
  (params (OldPawn :type "Pawn Object Reference") (NewPawn :type "Pawn Object Reference"))
  (bind _asbase_character (cast `/Game/Blueprints/Chars/Abstract/Base_Character` NewPawn))
  (bind _output_get (set `self.body` _asbase_character))
  (set `self.Goal` (`KismetMathLibrary.Conv_VectorToVector2D` (`Actor.K2_GetActorLocation` _output_get))))

(fn `from body to goal`
  (returns (vector :type "Vector2D Structure"))
  (return (- (`self.Goal`) (`KismetMathLibrary.Conv_VectorToVector2D` (`Actor.K2_GetActorLocation` (`self.body`))))))

(fn `Get direction`
  (returns (NewParam :type "/Game/Data/enums/Direction Enum"))
  (bind (_x _y) (`KismetMathLibrary.BreakVector2D` (`self.from body to goal`)))
  (if (< (`KismetMathLibrary.VSize2D` (`self.from body to goal`)) 50.0)
    (bind (_goal _end) (`/Game/Blueprints/Navigation/Path_holder.Get Goal` (`self.path`)))
    (if (not _end)
      (set `self.Goal` _goal)))
  (if _end
    (return "NewEnumerator4")
    (elif (> (`KismetMathLibrary.Abs` _x) (`KismetMathLibrary.Abs` _y))
      (if (> _x 0.0)
        (return "NewEnumerator0")
        (else
          (return "NewEnumerator1")))
      (elif (> _y 0.0)
        (return "NewEnumerator2")
        (else
          (return "NewEnumerator3"))))))

(fn `Load new path`
  (params (Tiles :type "Array of /Game/3D/platforms/Tile Object Reference"))
  (bind _path (`self.path`))
  (`/Game/Blueprints/Navigation/Path_holder.Reset` _path)
  (bind _output_get (set `/Game/Blueprints/Navigation/Path_holder.Points` Tiles _path))
  (set `self.Goal` (`KismetMathLibrary.Conv_VectorToVector2D` (`Actor.K2_GetActorLocation` (`|GetArrayItem` Tiles))))
  (`KismetArrayLibrary.Array_Remove` _output_get))