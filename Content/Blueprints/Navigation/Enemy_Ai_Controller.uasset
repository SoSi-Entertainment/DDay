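; AI controller for Enemy_Character pawns that aims and fires at the closest living ally in range.
; Each tick it scans the pawn's Field sphere for the Ally_Character nearest the endpoint location, skipping any within a minimum distance of the body.
; If a visibility trace ignoring Wire_bp actors is clear, it sets gun angle, optionally rotates the body, and shoots.
; A CanSeePlayer trace helper is defined but not called here.
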(event `self.ReceiveBeginPlay`
  (bind _asenemy_character (cast `/Game/Blueprints/Chars/Enemy_Character` (`self.K2_GetPawn`)))
  (bind _output_get (set `self.body` _asenemy_character))
  (set `self.Range` (`SphereComponent.GetScaledSphereRadius` (`/Game/Blueprints/Chars/Enemy_Character.Field` _output_get)))
  (bind _outactors (`GameplayStatics.GetAllActorsOfClass` "/Game/3D/wire/Wire_bp.Wire_bp_C"))
  (set `self.Wires` _outactors))

(event `self.ReceiveTick`
  (params (DeltaSeconds :type "Float (single-precision)"))
  (bind _clothest_target (`self.Clothest target`))
  (bind _body (`self.body`))
  (bind _body_2 (`self.body`))
  (bind _returnvalue (`self.K2_GetActorLocation` _clothest_target))
  (bind _asbase_character (cast `/Game/Blueprints/Chars/Base_Character` (`self.K2_GetPawn`)))
  (if (not (`/Game/Blueprints/Chars/Base_Character.Dead` _asbase_character))
    (set `self.Clothest dist` (`self.Range`))
    (set `self.Clothest target` null)
    (bind _location (`/Game/Blueprints/Chars/Base_Character.Endpoint Location` _body_2))
    (for _array_element (`PrimitiveComponent.GetOverlappingActors` (`/Game/Blueprints/Chars/Enemy_Character.Field` _body_2) "/Game/Blueprints/Chars/Ally_Character.Ally_Character_C")
      (bind _asbase_character_2 (cast `/Game/Blueprints/Chars/Base_Character` _array_element))
      (if (not (`/Game/Blueprints/Chars/Base_Character.Dead` _asbase_character_2))
        (bind _returnvalue_2 (`self.K2_GetActorLocation` _array_element))
        (`/Engine/EditorBlueprintResources/StandardMacros.CompareFloat` (`KismetMathLibrary.Vector_Distance` (`self.K2_GetActorLocation` _body_2) _returnvalue_2) 100.0
          (:`>`
            (bind _returnvalue_3 (`KismetMathLibrary.Vector_Distance` _location _returnvalue_2))
            (`/Engine/EditorBlueprintResources/StandardMacros.CompareFloat` _returnvalue_3 (`self.Clothest dist`)
              (:`<`
                (set `self.Clothest dist` _returnvalue_3)
                (set `self.Clothest target` _array_element)))))))
    (`/Engine/EditorBlueprintResources/StandardMacros.IsValid` _clothest_target
      (:`Is Valid`
        (bind (_outhit _returnvalue_4) (`KismetSystemLibrary.LineTraceSingle` _location _returnvalue "TraceTypeQuery1" false (`self.Wires`) "None" true (struct :`R` 1.0 :`A` 1.0) (struct :`G` 1.0 :`A` 1.0) 0.0))
        (if (not _returnvalue_4)
          (bind _returnvalue_5 (- _returnvalue _location))
          (`/Game/Blueprints/Chars/Base_Character.Set gun angle` _body (`KismetMathLibrary.Vector_HeadingAngle` _returnvalue_5))
          (if (`/Game/Blueprints/Chars/Enemy_Character.Rotate Body` _body)
            (`self.K2_SetActorRotation` _body (`KismetMathLibrary.Conv_VectorToRotator` _returnvalue_5) false))
          (`/Game/Blueprints/Chars/Base_Character.Shoot` _body _returnvalue))))))

(fn `CanSeePlayer`
  (returns (see :type Boolean))
  (bind (_outhit _returnvalue) (`KismetSystemLibrary.LineTraceSingle` :`Start` (`self.K2_GetActorLocation` (`self.K2_GetPawn`)) :`End` (`self.K2_GetActorLocation` (`GameplayStatics.GetPlayerPawn` 0)) :`TraceChannel` "TraceTypeQuery1" :`DrawDebugType` "ForOneFrame"))
  (return (not _returnvalue)))

(fn `UserConstructionScript`)