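; Navigation path holder that stores waypoint actors, a loop flag and a stop-to-shoot flag, and hands out 2D goals in order.
; GetGoal advances an iterator past invalid points, wrapping when looped or flagging End otherwise.
; A looped path with no valid points never exits that search.
; CopyData takes settings and points from another holder but not the iterator, while Reset clears everything.
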(fn `Copy Data`
  (params (From :type "/Game/Blueprints/Navigation/Path_holder Object Reference"))
  (set `self.Looped` (`/Game/Blueprints/Navigation/Path_holder.Looped` From))
  (set `self.Points` (`/Game/Blueprints/Navigation/Path_holder.Points` From))
  (set `self.Stop to shoot` (`/Game/Blueprints/Navigation/Path_holder.Stop to shoot` From)))

(fn `Get Goal`
  (returns (goal :type "Vector2D Structure") (end :type Boolean))
  (bind _points (`self.Points`))
  (bind _result (`self.result`))
  (bind _output (`|GetArrayItem` _points (`self.iterator`)))
  (`/Engine/EditorBlueprintResources/StandardMacros.CompareInt` (`self.iterator`) (`KismetArrayLibrary.Array_Length` _points) :!label _label
    (:`>`
      (if (`self.Looped`) :!label _label_2
        (set `self.iterator` 0)
        (`/Engine/EditorBlueprintResources/StandardMacros.IsValid` _output :!label _label_3
          (:`Is Valid`
            (set `self.result` (`KismetMathLibrary.Conv_VectorToVector2D` (`Actor.K2_GetActorLocation` _output)))
            (`/Engine/EditorBlueprintResources/StandardMacros.IncrementInt` (`self.iterator`)
              (:`  `
                (return _result false))))
          (:`Is Not Valid`
            (`/Engine/EditorBlueprintResources/StandardMacros.IncrementInt` (`self.iterator`)
              (:`  `
                (goto _label)))))
        (else
          _)))
    (:`==`
      (goto _label_2))
    (:`<`
      (goto _label_3)))
  (return _result true))

(fn `Reset`
  (set `self.Stop to shoot` false)
  (set `self.Looped` false)
  (set `self.iterator` 0)
  (`KismetArrayLibrary.Array_Clear` (`self.Points`)))