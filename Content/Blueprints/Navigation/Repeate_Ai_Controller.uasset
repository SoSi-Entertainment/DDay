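; AI controller that drives a Repeater pawn by replaying frames from an injected BlackBox, mimicking recorded movement and shooting.
; Each tick it extracts a frame and applies body angle, location, gun rotation and recoil directly, firing when the frame has a shot.
; When the frame's Done flag is false, it marks the Repeater dead and calls Die.
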(event `self.ReceiveTick`
  (params (DeltaSeconds :type "Float (single-precision)"))
  (bind (_location _body_angle _rotation _shot _done) (`/Game/Blueprints/recording/Black_Box_2.Extract Frame` (`self.Black box`)))
  (bind _asrepeater (cast `/Game/Blueprints/Chars/Repeater` (`self.K2_GetPawn`)))
  (if _done
    (`/Game/Blueprints/Chars/Repeater.Rotate body` _asrepeater _body_angle)
    (`self.K2_SetActorLocation` _asrepeater _location false false)
    (`/Game/Blueprints/Chars/Base_Character.Set gun angle` _asrepeater _rotation _shot)
    (if _shot
      (bind _done_2 (`/Game/Blueprints/Chars/Base_Character.Shoot` _asrepeater (0.0 0.0 0.0)))
      (if _done_2
        _))
    (else
      (set `/Game/Blueprints/Chars/Base_Character.Dead` true _asrepeater)
      (`/Game/Blueprints/Chars/Base_Character.Die` _asrepeater))))

(fn `Insert Black Box`
  (params (`Black box` :type "/Game/Blueprints/recording/Black_Box_2 Object Reference"))
  (set `self.Black box` `Black box`))

(fn `UserConstructionScript`)