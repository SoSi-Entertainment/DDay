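; NPC movement logic that walks a character along a SimplePath of tile points, looped or not, using straight MoveToLocation calls without pathfinding.
; On each tile entered it checks the current tile's gate in the path direction, continuing to the next point or walking to the tile middle at turns and blockages.
; Blocked NPCs shake and poll until the way frees, or turn and trench-jump on a Jump response.
; Pause stops the NPC on a tile-aligned location.
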(event `On way blocked`
  (params (Direction :type "/Game/Data/enums/Direction Enum" :default "NewEnumerator4") (`Jump request` :type Boolean))
  (bind _npc_body (`self.NPC Body`))
  (`Controller.SetControlRotation` (`self.NPC Controller`) (`KismetMathLibrary.Conv_VectorToRotator` (`/Game/Blueprints/System/Funtions/FunctionLibrary.Vector from direction` Direction)))
  (if `Jump request`
    (`/Game/Blueprints/System/Funtions/Component_Macro.Wait condition` (== (`KismetMathLibrary.Round` (.yaw (`KismetMathLibrary.NormalizedDeltaRotator` (`Actor.K2_GetActorRotation` _npc_body) (`Pawn.GetControlRotation` _npc_body)))) 0) 0.1
      (:`true`
        (`/Game/Blueprints/Chars/Abstract/Base_Character.Trench Jump` (`self.NPC Body`))
        (set `self.Jump Requested` false)
        (set `self.Way blocked` false)))
    (else
      (`/Game/Blueprints/Chars/Abstract/Base_Character.Shake body in dir` (`self.NPC Body`) Direction)
      (`self.Waiting for free way loop`))))

(event `Waiting for free way loop`
  (`/Game/Blueprints/Controllers/NPC_Controller.Set walking` (`self.NPC Controller`) false)
  (`KismetSystemLibrary.Delay` 0.1 :!label _label)
  (bind (_free _responce) (`self.Check way` (`self.Current Path Dir`)))
  (if _free
    _
    (elif (`|EnumEquality` _responce "NewEnumerator6")
      _
      (else
        (goto _label))))
  (set `self.Way blocked` false)
  (`self.Try To Go Next Tile` true))

(fn `Check next Dir`
  (returns (`Dir changed` :type Boolean) (`New dir` :type "/Game/Data/enums/Direction Enum"))
  (locals (`next point` :type "/Game/3D/platforms/Tile Object Reference"))
  (bind _iterator (`self.Iterator`))
  (bind _points (`self.Points`))
  (if (> _iterator (`KismetArrayLibrary.Array_LastIndex` _points))
    (if (`self.Looped`)
      (set `local.next point` (`|GetArrayItem` (`self.Points`)))
      (else
        (return false "NewEnumerator4")))
    (else
      (bind _output_get (set `local.next point` (`|GetArrayItem` _points _iterator)))))
  (bind _direction (`/Game/Blueprints/System/Funtions/FunctionLibrary.Direction from vector` (- (`Actor.K2_GetActorLocation` _output_get) (`Actor.K2_GetActorLocation` (`self.NPC Body`)))))
  (return (`|EnumInequality` (`self.Current Path Dir`) _direction) _direction))

(fn `Check way`
  (params (direction :type "/Game/Data/enums/Direction Enum" :default "NewEnumerator4"))
  (returns (Free :type Boolean) (responce :type "/Game/Blueprints/Navigation/Tile_Gate_Responce Enum"))
  (bind _responce (`/Game/3D/platforms/Tile.Check Gate` (`self.current tile`) direction (`self.NPC Body`)))
  (switch `/Game/Blueprints/Navigation/Tile_Gate_Responce` _responce
    (:`NewEnumerator0`
      _)
    (:`NewEnumerator8`
      (return false _responce))
    (:`NewEnumerator2`
      (return false _responce))
    (:`NewEnumerator3`
      (return false _responce))
    (:`NewEnumerator4`
      _)
    (:`NewEnumerator5`
      _)
    (:`NewEnumerator1`
      (return false _responce))
    (:`NewEnumerator6`
      (set `self.Jump Requested` true)
      (return false _responce))
    (:`NewEnumerator7`
      (return false _responce)))
  (return true "NewEnumerator0"))

(fn `Init`
  (params (`NPC body` :type "/Game/Blueprints/Chars/Abstract/Base_Character Object Reference") (`NPC controller` :type "/Game/Blueprints/Controllers/NPC_Controller Object Reference"))
  (bind _output_get (set `self.NPC Body` `NPC body`))
  (set `self.NPC capsule radius` (`CapsuleComponent.GetScaledCapsuleRadius` (`Character.CapsuleComponent` _output_get)))
  (bind _output_get_2 (set `self.NPC Controller` `NPC controller`))
  (add `AIController.ReceiveMoveCompleted` _output_get_2 (`|CreateDelegate` :!event `On Move Complete`))
  (add `/Game/Blueprints/Chars/Abstract/Base_Character.enter tile` (`self.NPC Body`) (`|CreateDelegate` :!event `On Enter Tile`))
  (bind _tile (`/Game/Blueprints/System/Funtions/FunctionLibrary.Get Tile Under` (`Actor.K2_GetActorLocation` (`self.NPC Body`))))
  (set `self.current tile` _tile)
  (add `/Game/Blueprints/Chars/Abstract/Base_Character.Jump finished` (`self.NPC Body`) (`|CreateDelegate` :!event `On Jump Finished`)))

(fn `Is end point`
  (params (Point :type "/Game/3D/platforms/Tile Object Reference (by ref)"))
  (returns (`return value` :type Boolean))
  (bind _points (`self.Points`))
  (return (== (`KismetArrayLibrary.Array_Find` _points Point) (`KismetArrayLibrary.Array_LastIndex` _points))))

(fn `On Enter Tile`
  (params (tile :type "/Game/3D/platforms/Tile Object Reference"))
  (set `self.current tile` tile)
  (if (`KismetMathLibrary.BooleanNOR` (`/Game/Blueprints/Chars/Abstract/Base_Character.Jumping` (`self.NPC Body`)) (`self.paused`))
    (`self.Try To Go Next Tile` false)))

(fn `On Jump Finished`
  (`self.Try To Go Next Tile` true))

(fn `On Move Complete`
  (params (RequestID :type "AIRequestID Structure") (Result :type "EPathFollowingResult Enum" :default "Success"))
  (switch `EPathFollowingResult` Result
    (:`Success`
      (if (`self.Walking to tile mid`)
        (set `self.Walking to tile mid` false)
        (if (not (`self.paused`))
          (if (`self.Way blocked`)
            (`self.On way blocked` (`self.Current Path Dir`) (`self.Jump Requested`))
            (else
              (bind _path_end (`self.Walk to next Point`))
              (if _path_end
                (`/Game/Blueprints/Controllers/NPC_Controller.Set walking` (`self.NPC Controller`) false)))))))))

(fn `Pause movement`
  (bind _returnvalue (`Actor.K2_GetActorLocation` (`self.NPC Body`)))
  (bind _normal_vector (`/Game/Blueprints/System/Funtions/FunctionLibrary.Vector from direction` (`self.Current Walk Dir`)))
  (bind _returnvalue_2 (`Actor.K2_GetActorLocation` (`self.NPC Body`)))
  (bind _returnvalue_3 (`KismetMathLibrary.Vector_GetAbs` _normal_vector))
  (bind _returnvalue_4 (`KismetMathLibrary.Conv_Vector2DToVector` (`/Game/Blueprints/System/Funtions/FunctionLibrary.Tiled location` _returnvalue) (.z _returnvalue)))
  (bind (_x _y) (`KismetMathLibrary.BreakVector2D` (`KismetMathLibrary.Conv_VectorToVector2D` (* (- (* (`KismetMathLibrary.Conv_Vector2DToVector` (`/Game/Blueprints/System/Funtions/FunctionLibrary.Tiled location` _returnvalue_2)) _returnvalue_3) (* _returnvalue_2 _returnvalue_3)) _normal_vector))))
  (bind _returnvalue_5 (select `bool` (> (`KismetMathLibrary.Abs` _y) (`KismetMathLibrary.Abs` _x)) :`false` _x :`true` _y))
  (`|ExecutionSequence`
    (:`then_0`
      (if (not (stale _output_get))
        (if (and (and (> _returnvalue_5 0.0) (< _returnvalue_5 50.0)) true)
          (`self.Walk to location` _returnvalue_4)
          (else
            (`self.Walk to location` (+ _returnvalue_4 (* (`/Game/Blueprints/System/Funtions/FunctionLibrary.Vector from direction` (`self.Current Walk Dir`)) 100.0)))))))
    (:`then_1`
      (bind _output_get (set `self.paused` true)))))

(fn `Retore walking last tile`
  (`self.Walk to point` (`self.Last target point`)))

(fn `Start Simple Path Walking`
  (params (`Simple Path` :type "/Game/Blueprints/Navigation/Path_holder Object Reference"))
  (bind _output_get (set `self.Simple Path` `Simple Path`))
  (bind _output_get_2 (set `self.Points` (`/Game/Blueprints/Navigation/Path_holder.Points` _output_get)))
  (if (> (`KismetArrayLibrary.Array_Length` _output_get_2) 0)
    (set `self.Looped` (`/Game/Blueprints/Navigation/Path_holder.Looped` _output_get))
    (set `self.Iterator` (`/Game/Blueprints/Navigation/Path_holder.iterator` _output_get))
    (`self.Walk to next Point`)
    (`self.Check way` "NewEnumerator4")))

(fn `Try To Go Next Tile`
  (params (`after interaption` :type Boolean))
  (bind (_dir_changed _new_dir) (`self.Check next Dir`))
  (bind _current_path_dir (`self.Current Path Dir`))
  (bind _current_tile (`self.current tile`))
  (bind _points (`self.Points`))
  (if (`self.Is end point` (`self.current tile`))
    (if (not (`local.after interaption`))
      (`self.Walk to tile mid` false))
    (elif (and (`KismetArrayLibrary.Array_Contains` _points _current_tile) (== (`KismetArrayLibrary.Array_Find` _points _current_tile) (+ (`self.Iterator`) -1)))
      (if _dir_changed
        (bind _output_get (set `self.Current Path Dir` _new_dir))
        (bind _free (`self.Check way` _output_get))
        (if (`local.after interaption`)
          (`self.Walk to next Point`)
          (else
            (bind _returnvalue (not _free))
            (`self.Walk to tile mid` _returnvalue)
            (if _returnvalue
              (set `self.Last target point` null))))
        (else
          (bind _free_2 (`self.Check way` _current_path_dir))
          (if _free_2
            (`self.Walk to next Point`)
            (else
              (set `self.Last target point` null)
              (`self.Walk to tile mid` true :!label _label)))))
      (else
        (bind _free_3 (`self.Check way` _current_path_dir))
        (if _free_3
          (if (`local.after interaption`)
            (`self.Last target point`
              (:`then`
                (`self.Retore walking last tile`))
              (:`else`
                (`self.Walk to next Point`))))
          (else
            (goto _label)))))))

(fn `Unpause movement`
  (`|ExecutionSequence`
    (:`then_0`
      (if (stale _output_get)
        (`self.Try To Go Next Tile` true)))
    (:`then_1`
      (bind _output_get (set `self.paused` false)))))

(fn `Walk to location`
  (params (`Target locaction` :type "Vector Structure"))
  (bind _npc_controller (`self.NPC Controller`))
  (`/Game/Blueprints/Controllers/NPC_Controller.Set walking` _npc_controller true)
  (`AIController.MoveToLocation` _npc_controller (+ `Target locaction` (* (`KismetMathLibrary.Normal2D` (- (`KismetMathLibrary.Conv_VectorToVector2D` `Target locaction`) (`KismetMathLibrary.Conv_VectorToVector2D` (`Actor.K2_GetActorLocation` (`self.NPC Body`))))) (`self.NPC capsule radius`))) -1.0 true false false true null true))

(fn `Walk to next Point`
  (returns (`Path end` :type Boolean))
  (bind _points (`self.Points`))
  (bind _iterator (`self.Iterator`))
  (if (> _iterator (`KismetArrayLibrary.Array_LastIndex` _points))
    (if (`self.Looped`)
      (set `self.Iterator` 0)
      (else
        (return true))))
  (bind _output_get (set `self.Last target point` (`|GetArrayItem` _points _iterator)))
  (`self.Walk to point` _output_get)
  (`/Engine/EditorBlueprintResources/StandardMacros.IncrementInt` (`self.Iterator`)
    (:`  `
      (return false))))

(fn `Walk to point`
  (params (Point :type "/Game/3D/platforms/Tile Object Reference"))
  (bind _returnvalue (`Actor.K2_GetActorLocation` Point))
  (`self.Walk to location` _returnvalue)
  (bind _output_get (set `self.Current Path Dir` (`/Game/Blueprints/System/Funtions/FunctionLibrary.Direction from vector` (- _returnvalue (`Actor.K2_GetActorLocation` (`self.NPC Body`))))))
  (set `self.Current Walk Dir` _output_get))

(fn `Walk to tile mid`
  (params (`Way blocked` :type Boolean))
  (set `self.Way blocked` `Way blocked`)
  (set `self.Walking to tile mid` true)
  (`self.Walk to location` (`Actor.K2_GetActorLocation` (`self.current tile`))))