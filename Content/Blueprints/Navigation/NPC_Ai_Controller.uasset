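; AI controller that walks an NPC tile by tile along the path supplied by its Ai_Character pawn.
; On possess it sizes its Field sphere from the pawn's trigger radius, then passes the path to PathManager.
; While the pawn is alive, PathManager directions drive GridNavigator one tile at a time, with a short retry delay on one special direction value.
; Helpers provide a player line-of-sight trace, path replacement and debug drawing.
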(event `self.ReceivePossess`
  (params (PossessedPawn :type "Pawn Object Reference"))
  (bind _grid_navigator (`self.Grid_Navigator`))
  (bind _path_manager (`self.Path_manager`))
  (`self.Get field radius` PossessedPawn)
  (bind _asai_character (cast `/Game/Blueprints/Chars/Components/Ai_Character` PossessedPawn))
  (bind _path (`/Game/Blueprints/Chars/Components/Ai_Character.Get path` _asai_character))
  (bind _asbase_character (cast `/Game/Blueprints/Chars/Base_Character` PossessedPawn))
  (`KismetSystemLibrary.Delay` 0.2)
  (set `/Game/Blueprints/Navigation/Path_manager.path` _path _path_manager)
  (bind _newparam (`/Game/Blueprints/Navigation/Path_manager.Get direction` _path_manager :!label _label))
  (if (`/Game/Blueprints/Chars/Base_Character.Dead` _asbase_character)
    _
    (elif (`|EnumEquality` _newparam "NewEnumerator4")
      (`KismetSystemLibrary.Delay` 0.2)
      (goto _label)
      (else
        (`/Game/Blueprints/Navigation/Grid_Navigator.Go` _grid_navigator _newparam)
        (`/Game/Blueprints/System/DDayMacroLibrary.Wait condition` (`/Game/Blueprints/Navigation/Grid_Navigator.OnTile` _grid_navigator)
          (:`true`
            (goto _label)))))))

(fn `add path`
  (params (path :type "/Game/Blueprints/Navigation/Path_holder Object Reference"))
  (set `/Game/Blueprints/Navigation/Path_manager.path` path (`self.Path_manager`)))

(fn `CanSeePlayer`
  (returns (see :type Boolean))
  (bind (_outhit _returnvalue) (`KismetSystemLibrary.LineTraceSingle` :`Start` (`self.K2_GetActorLocation` (`self.K2_GetPawn`)) :`End` (`self.K2_GetActorLocation` (`GameplayStatics.GetPlayerPawn` 0)) :`TraceChannel` "TraceTypeQuery1" :`DrawDebugType` "ForOneFrame"))
  (return (not _returnvalue)))

(fn `Get field radius`
  (params (Pawn :type "Pawn Object Reference"))
  (returns (updated :type Boolean))
  (bind _asai_character (cast `/Game/Blueprints/Chars/Components/Ai_Character` Pawn)
    (:`then`
      (bind (_has_collision_sphere _sphere_radius) (`/Game/Blueprints/Chars/Components/Ai_Character.Get trigger radius` _asai_character))
      (if _has_collision_sphere
        (`SphereComponent.SetSphereRadius` (`self.Field`) _sphere_radius true)
        (return true)
        (else
          _)))
    (:`CastFailed`
      _))
  (return false))

(fn `test draw`
  (`KismetSystemLibrary.DrawDebugCircle` (`self.K2_GetActorLocation` (`self.K2_GetPawn`)) 50.0 50 (struct :`G` 1.0 :`B` 0.058979 :`A` 1.0) 2.0 5.0 (0.0 1.0 0.0) (1.0 0.0 0.0)))

(fn `UserConstructionScript`)