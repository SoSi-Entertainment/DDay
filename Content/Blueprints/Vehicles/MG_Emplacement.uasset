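; Machine gun emplacement on a tile grid that marks its line of fire when play begins.
; BeginPlay finds the tile beneath it, then steps through neighbours opposite the root component's forward vector, up to a set tile count or the first missing neighbour.
; The collected tiles are highlighted faint red.
; This graph holds no firing or overlap logic.
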(event `self.ReceiveBeginPlay`
  (bind _fire_line_tiles (`self.fire line tiles`))
  (bind _direction (`/Game/Blueprints/System/FunctionLibrary.Direction from vector` (* (`SceneComponent.GetForwardVector` (`self.DefaultSceneRoot`)) -1.0)))
  (`parent.ReceiveBeginPlay`)
  (bind _tile (`/Game/Blueprints/System/FunctionLibrary.Get Tile Under` (`self.K2_GetActorLocation`) 50.0))
  (`KismetArrayLibrary.Array_Add` (`self.fire line tiles`) (`/Game/3D/platforms/Tile.Get Neighbour` _tile _direction))
  (for _index (range (+ (- (`self.fire line draw tiles`) 2) 1))
    (bind (_tile_2 _not_empty) (`/Game/3D/platforms/Tile.Get Neighbour` (`|GetArrayItem` _fire_line_tiles _index) _direction))
    (if _not_empty
      (`KismetArrayLibrary.Array_Add` _fire_line_tiles _tile_2)
      (else
        (break))))
  (for _array_element (`self.fire line tiles`)
    (`/Game/3D/platforms/Tile.Higlight` _array_element (struct :`R` 1.0 :`A` 1.0) 0.3)))

(fn `UserConstructionScript`
  (`parent.UserConstructionScript`))