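; Vehicle seat actor that holds one character and is linked to the Vehicle_Module found through its parent component's attachment.
; Enter accepts a character only when the seat is free, stores the entrance used and enables Tick.
; Tick polls the character's WantBeInVehicle flag and, once false, calls Out to notify module and character, then free the seat.
; The construction script shows either mannequin and arrow or a sphere, based on SeatMode.
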(event `self.ReceiveBeginPlay`
  (bind _asvehicle_module (cast `/Game/Blueprints/Vehicles/Vehicle_Module` (`SceneComponent.GetAttachParent` (`self.GetParentComponent`))))
  (set `self.Module` _asvehicle_module))

(event `self.ReceiveTick`
  (params (DeltaSeconds :type "Float (single-precision)"))
  (if (not (`/Game/Blueprints/Chars/Abstract/Base_Character.Want be in vehicle` (`self.Character`)))
    (`self.Out`)))

(fn `Enter`
  (params (Entrace :type "/Game/Blueprints/Vehicles/Vehicle_Entrace Object Reference") (Charcter :type "/Game/Blueprints/Chars/Abstract/Base_Character Object Reference"))
  (returns (Success :type Boolean))
  (if (`self.Is free`)
    (set `self.Entrace` Entrace)
    (bind _output_get (set `self.Character` Charcter))
    (`/Game/Blueprints/Chars/Abstract/Base_Character.Enter vehicle` _output_get self)
    (`self.SetActorTickEnabled` true)
    (return true)
    (else
      (return false))))

(fn `Is free`
  (returns (Free :type Boolean))
  (return (not (`KismetSystemLibrary.IsValid` (`self.Character`)))))

(fn `Out`
  (bind _character (`self.Character`))
  (`self.SetActorTickEnabled` false)
  (`/Game/Blueprints/Vehicles/Vehicle_Module.Out` (`self.Module`) _character)
  (`/Game/Blueprints/Chars/Abstract/Base_Character.Out vehicle` _character self)
  (set `self.Character` null))

(fn `UserConstructionScript`
  (bind _seat_mode (`self.Seat mode`))
  (`SceneComponent.SetVisibility` (`self.Mannequin`) (`|EnumEquality` _seat_mode "NewEnumerator0") false)
  (`SceneComponent.SetVisibility` (`self.Arrow`) (`|EnumEquality` _seat_mode "NewEnumerator0") false)
  (`SceneComponent.SetVisibility` (`self.Sphere`) (`|EnumEquality` _seat_mode "NewEnumerator1") false))