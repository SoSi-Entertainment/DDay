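; Vehicle entrance actor, placed as a child actor on a vehicle, that lets characters board it.
; On BeginPlay it resolves its vehicle, module and optional seat from the attachment hierarchy, targeting either that seat or the module.
; Each tick it shows or hides its marker based on free seats at the mode's scope: seat, module or vehicle.
; Overlapping characters flagged as wanting to board are passed to the vehicle's Enter function.
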(event `self.ReceiveBeginPlay`
  (bind _returnvalue (`SceneComponent.GetAttachParent` (`self.GetParentComponent`)))
  (bind _asvehicle (cast `/Game/Blueprints/Vehicles/Vehicle` (`self.GetParentActor`)))
  (set `self.vehicle` _asvehicle)
  (bind _aschild_actor_component (cast `ChildActorComponent` _returnvalue)
    (:`then`
      (bind _asvehicle_seat (cast `/Game/Blueprints/Vehicles/Vehicle_Seat` (`ChildActorComponent.ChildActor` _aschild_actor_component)))
      (set `self.Seat` _asvehicle_seat)
      (bind _asvehicle_module (cast `/Game/Blueprints/Vehicles/Vehicle_Module` (`SceneComponent.GetAttachParent` _aschild_actor_component)))
      (set `self.Module` _asvehicle_module)
      (set `self.Mode` "NewEnumerator0"))
    (:`CastFailed`
      (bind _asvehicle_module_2 (cast `/Game/Blueprints/Vehicles/Vehicle_Module` _returnvalue))
      (set `self.Module` _asvehicle_module_2)
      (set `self.Mode` "NewEnumerator1"))))

(event `self.ReceiveTick`
  (params (DeltaSeconds :type "Float (single-precision)"))
  (switch `/Game/Blueprints/Vehicles/Entrace_Mode` (`self.Mode`)
    (:`NewEnumerator0`
      (`self.Set Availability` (`/Game/Blueprints/Vehicles/Vehicle_Seat.Is free` (`self.Seat`))))
    (:`NewEnumerator1`
      (`self.Set Availability` (`/Game/Blueprints/Vehicles/Vehicle_Module.Has free sits` (`self.Module`))))
    (:`NewEnumerator2`
      (bind _has (`/Game/Blueprints/Vehicles/Vehicle.Has free seatts` (`self.vehicle`)))
      (`self.Set Availability` _has))))

(event `self.ReceiveActorBeginOverlap`
  (params (OtherActor :type "Actor Object Reference"))
  (bind _asbase_character (cast `/Game/Blueprints/Chars/Abstract/Base_Character` OtherActor))
  (if (`/Game/Blueprints/Chars/Abstract/Base_Character.Want be in vehicle` _asbase_character)
    (`self.Enter` _asbase_character)))

(fn `Enter`
  (params (Character :type "/Game/Blueprints/Chars/Abstract/Base_Character Object Reference"))
  (returns (Success :type Boolean))
  (bind _success (`/Game/Blueprints/Vehicles/Vehicle.Enter` (`self.vehicle`) (`self.Module`) (`self.Seat`) self Character))
  (return _success))

(fn `Find sit`)

(fn `Get entrace mode`)

(fn `Set Availability`
  (params (`Is available` :type Boolean))
  (`SceneComponent.SetVisibility` (`self.Marker`) `Is available` false))

(fn `UserConstructionScript`)