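; Stationary mounted gun that aims from player input, a clone's recorded aim, or its own AI, as set by the WorkerState passed to UpdateState.
; The AI picks the nearest living opposing character by angle, blind zone and line of sight, with a configurable fallback pass.
; Timers delay first fire and forgetting old targets.
; Yaw and pitch are interpolated within angle limits on a child-actor Gun, which handles the shot.
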(event `self.ReceiveBeginPlay`
  (`/Game/Blueprints/Arms/Gun.Hide arms` (`self.Get gun`)))

(event `CustomEvent`
  (set `self.Last target` null)
  (goto _label :!via `Reset`))

(event `self.ReceiveTick`
  (params (DeltaSeconds :type "Float (single-precision)"))
  (bind _clone_controled (`self.Clone Controled`))
  (bind _last_target (`self.Last target`))
  (if (`self.Available`)
    (if (`self.Player controled`)
      (`self.Aim on point` (`/Game/Blueprints/Controllers/DDay_Player_Controller.Get Plane Aim Location ` (`/Game/Blueprints/System/FunctionLibrary.Get PlayerController Troops`)))
      (else
        (`/Engine/EditorBlueprintResources/StandardMacros.IsValid` _clone_controled
          (:`Is Valid`
            (`self.Aim on point` (`/Game/Blueprints/Chars/Clones/Clone_Main.Recorded aim location` _clone_controled)))
          (:`Is Not Valid`
            (bind (_target_found _target_character) (`self.Find clothest target in range`))
            (set `self.Found target` _target_found)
            (if _target_found
              (`/Engine/EditorBlueprintResources/StandardMacros.IsValid` _last_target
                (:`Is Valid`
                  (if (!= _target_character _last_target)
                    (`|ExecutionSequence`
                      (:`then_0`
                        (`/Engine/EditorBlueprintResources/StandardMacros.DoOnce` false :!label _label
                          (:`Completed`
                            (`KismetSystemLibrary.K2_SetTimerDelegate` (delegate `CustomEvent`) (`self.Rememeber old target time`)))))
                      (:`then_1`
                        (if (not (`/Game/Blueprints/Chars/Abstract/Base_Character.Dead` (stale `CustomEvent_0` _output_get))) :!label _label_2
                          (bind _location (`/Game/Blueprints/Chars/Abstract/Base_Character.Pls shoot here` (stale `CustomEvent_0` _output_get)))
                          (bind _current_angle (`self.Aim on point` _location))
                          (if (or (< (`KismetMathLibrary.Abs` (- (.yaw (`self.Angle to target` _location)) (.yaw _current_angle))) (`self.allowed precision angle`)) (`self.Gun Locked`))
                            (`self.Gun Shoot` null false _location false (`|MakeArray` (stale `CustomEvent_0` _output_get)))))))
                    (else
                      (goto _label_2))))
                (:`Is Not Valid`
                  (`/Engine/EditorBlueprintResources/StandardMacros.DoOnce` false :!label _label_3
                    (:`Completed`
                      (`KismetSystemLibrary.K2_SetTimerDelegate` (delegate `CustomEvent_0`) (`self.Start fire lag`))))))
              (else
                (set `self.Last target` null)))))))))

(event `CustomEvent_0`
  (`|ExecutionSequence`
    (:`then_0`
      (goto _label_3 :!via `Reset`))
    (:`then_1`
      (bind _output_get (set `self.Last target` (stale `self.ReceiveTick` _target_character)))
      (`/Engine/EditorBlueprintResources/StandardMacros.IsValid` _output_get
        (:`Is Valid`
          (goto _label_2))))))

(event `/Game/Blueprints/Vehicles/Components/Vehicle_Worker.Broke`
  (`KismetSystemLibrary.PrintString` "Меня сломали ;(" true true (struct :`R` 1.0 :`B` 0.232469 :`A` 1.0) 10.0))

(event `/Game/Blueprints/Vehicles/Components/Vehicle_Worker.Update state`
  (params (`Worker state` :type "/Game/Blueprints/Vehicles/Components/Vehicle_Worker_State Structure"))
  (bind (_available _playercontroled _clonecontroled _team) (break `/Game/Blueprints/Vehicles/Components/Vehicle_Worker_State` `Worker state`))
  (set `self.Available` _available)
  (set `self.Player controled` _playercontroled)
  (set `self.Clone Controled` _clonecontroled)
  (set `self.Team` _team))

(fn `Aim on angle`
  (params (Angle :type "Rotator Structure"))
  (returns (`Current aim angle` :type "Rotator Structure") (`Angle blocked` :type Boolean))
  (bind _returnvalue (`self.GetTransform`))
  (bind _angle_lock (`self.Angle lock`))
  (bind _returnvalue_2 (`KismetMathLibrary.RInterpTo` (`self.K2_GetActorRotation` (`self.Get gun`)) (`KismetMathLibrary.SelectRotator` (`KismetMathLibrary.TransformRotation` _returnvalue (`KismetMathLibrary.MakeRotator` (.roll (`KismetMathLibrary.InverseTransformRotation` _returnvalue Angle)) (.pitch (`KismetMathLibrary.InverseTransformRotation` _returnvalue Angle)) (`KismetMathLibrary.FMax` (`KismetMathLibrary.FMin` (.yaw (`KismetMathLibrary.InverseTransformRotation` _returnvalue Angle)) _angle_lock) (* _angle_lock -1.0)))) Angle (`self.Gun Locked`)) (`GameplayStatics.GetWorldDeltaSeconds`) (`self.Rotation speed`)))
  (`SceneComponent.K2_SetWorldRotation` (`self.Gun`) _returnvalue_2 false false)
  (return _returnvalue_2 (`self.Is target out of angle lock` Angle)))

(fn `Aim on point`
  (params (Target :type "Vector Structure"))
  (returns (`Current angle` :type "Rotator Structure"))
  (bind (_current_aim_angle _angle_blocked) (`self.Aim on angle` (`self.Angle to target` Target)))
  (if (not _angle_blocked)
    (`self.Vert Aim on Location` Target))
  (return _current_aim_angle))

(fn `Angle to target`
  (params (Target :type "Vector Structure"))
  (returns (Angle :type "Rotator Structure"))
  (return (`KismetMathLibrary.MakeRotator` 0.0 0.0 (`KismetMathLibrary.RadiansToDegrees` (`KismetMathLibrary.Vector_HeadingAngle` (- Target (`self.SnipePoint Location`)))))))

(fn `Check if Clothest`
  (params (`Find out of range` :type Boolean) (`Find if not visible` :type Boolean) (Actor :type "Actor Object Reference") (`Clothest dist` :type "Float (double-precision) (by ref)"))
  (bind _asbase_character (cast `/Game/Blueprints/Chars/Abstract/Base_Character` Actor :!pure true))
  (bind _returnvalue (`KismetMathLibrary.Vector_Distance` (`self.K2_GetActorLocation`) (`self.K2_GetActorLocation` Actor)))
  (if (`|EnumInequality` (`self.Team`) (`/Game/Blueprints/Chars/Abstract/Base_Character.Team` _asbase_character))
    (if (`/Game/Blueprints/Chars/Abstract/Base_Character.Dead` _asbase_character)
      _
      (elif (or (not (`self.Is target out of angle lock` (`self.Angle to target` (`self.K2_GetActorLocation` _asbase_character)))) `Find out of range`)
        (`/Engine/EditorBlueprintResources/StandardMacros.CompareFloat` _returnvalue (`self.blind zone radius`)
          (:`>`
            (`/Engine/EditorBlueprintResources/StandardMacros.CompareFloat` _returnvalue `Clothest dist`
              (:`<`
                (bind _visible (`self.Check is target visible` (`/Game/Blueprints/Chars/Abstract/Base_Character.Pls shoot here` _asbase_character)))
                (if (or `Find if not visible` _visible)
                  (set `self.Clothest target` _asbase_character)
                  (`|VariableSetRef` `Clothest dist` _returnvalue))))))))))

(fn `Check is target visible`
  (params (`Target location` :type "Vector Structure"))
  (returns (Visible :type Boolean))
  (bind (_outhit _returnvalue) (`KismetSystemLibrary.LineTraceSingleByProfile` :`Start` (`self.K2_GetActorLocation`) :`End` `Target location` :`ProfileName` (select `/Game/Data/enums/Team` (`self.Team`) :`NewEnumerator0` "AllyTrace" :`NewEnumerator1` "EnemyTrace" :!type "Name") :`DrawDebugType` (select `bool` (`/Game/Blueprints/System/DDay_Instance.Debug Graphics` (`/Game/Blueprints/System/FunctionLibrary.Get Instanse Troops`)) :`true` "ForOneFrame" :!type "EDrawDebugTrace Enum")))
  (return (not _returnvalue)))

(fn `Draw laser pointer`
  (bind _gun (`self.Get gun`))
  (bind _location (`/Game/Blueprints/Arms/Gun.Endpoint Location` _gun))
  (`KismetSystemLibrary.LineTraceSingle` :`Start` _location :`End` (+ _location (* (`SceneComponent.GetForwardVector` (`Actor.RootComponent` _gun)) 1000.0)) :`TraceChannel` "TraceTypeQuery2" :`DrawDebugType` (select `bool` (`/Game/Blueprints/System/DDay_Instance.Debug Graphics` (cast `/Game/Blueprints/System/DDay_Instance` (`GameplayStatics.GetGameInstance`) :!pure true)) :`true` "ForOneFrame" :!type "EDrawDebugTrace Enum") :`TraceColor` (struct :`R` 1.0 :`G` 0.966577 :`A` 1.0) :`TraceHitColor` (struct :`G` 0.016429 :`B` 1.0 :`A` 1.0) :`DrawTime` 0.0))

(fn `Find clothest target in range`
  (returns (`Target found` :type Boolean) (`Target character` :type "/Game/Blueprints/Chars/Abstract/Base_Character Object Reference"))
  (locals (`Clothest dist` :type "Float (double-precision)"))
  (bind _clothest_target (`self.Clothest target`))
  (bind _overlappingactors (`self.GetOverlappingActors` (select `/Game/Data/enums/Team` (`self.Team`) :`NewEnumerator0` "/Game/Blueprints/Chars/Enemy_Character.Enemy_Character_C" :`NewEnumerator1` "/Game/Blueprints/Chars/Abstract/Ally_Character.Ally_Character_C" :`NewEnumerator3` "/Game/Blueprints/Chars/Abstract/Base_Character.Base_Character_C" :!type "Actor Class Reference")))
  (set `local.Clothest dist` (`self.potential range`))
  (set `self.Clothest target` null)
  (for _array_element _overlappingactors
    (`self.Check if Clothest` false false _array_element (`local.Clothest dist`)))
  (`/Engine/EditorBlueprintResources/StandardMacros.IsValid` _clothest_target
    (:`Is Valid`
      _)
    (:`Is Not Valid`
      (for _ _overlappingactors
        (`self.Check if Clothest` (`self.Find targets out of angle`) (`self.Find if not visible`) _array_element (`local.Clothest dist`)))
      (`/Engine/EditorBlueprintResources/StandardMacros.IsValid` (`self.Clothest target`)
        (:`Is Valid`
          _)
        (:`Is Not Valid`
          (return false null)))))
  (return true (cast `/Game/Blueprints/Chars/Abstract/Base_Character` _clothest_target :!pure true)))

(fn `Get gun`
  (returns (Gun :type "/Game/Blueprints/Arms/Gun Object Reference"))
  (return (cast `/Game/Blueprints/Arms/Gun` (`ChildActorComponent.ChildActor` (`self.Gun`)) :!pure true)))

(fn `Get Team`
  (returns (team :type "/Game/Data/enums/Team Enum"))
  (return (`self.Team`)))

(fn `Gun Shoot`
  (params (`shot info` :type "/Game/Blueprints/recording/Shot_Info Object Reference") (`100%hit` :type Boolean) (`Target location` :type "Vector Structure") (`Add owner speed` :type Boolean) (`Hit Targets` :type "Array of /Game/Blueprints/Chars/Abstract/Base_Character Object Reference (by ref)"))
  (returns (Done :type Boolean))
  (if (`self.Available`)
    (bind _done (`/Game/Blueprints/Arms/Gun.Shoot` (`self.Get gun`) (`self.Generate recoil`) `shot info` (`self.ignore cd`) `100%hit` `Target location` `Add owner speed` `Hit Targets`))
    (return _done)
    (else
      (return false))))

(fn `Has Target`
  (returns (Has :type Boolean))
  (return (`self.Found target`)))

(fn `Is player`
  (returns (Player :type Boolean))
  (return false))

(fn `Is target out of angle lock`
  (params (`Angle to target` :type "Rotator Structure"))
  (returns (Out :type Boolean))
  (return (and (`self.Gun Locked`) (> (`KismetMathLibrary.Abs` (.yaw (`KismetMathLibrary.InverseTransformRotation` (`self.GetTransform`) `Angle to target`))) (`self.Angle lock`)))))

(fn `Set gun vert angle`
  (params (angle :type "Float (double-precision)"))
  (bind _gun (`self.Get gun`))
  (bind (_upangle _downangle) (break `/Game/Data/structs/Recoil_Angles` (`self.Vert aim angle lock`)))
  (bind _returnvalue (`KismetMathLibrary.RInterpTo` (`self.Current aim`) (`KismetMathLibrary.MakeRotator` 0.0 (`KismetMathLibrary.SelectFloat` (`KismetMathLibrary.FMin` angle _upangle) (`KismetMathLibrary.FMax` angle _downangle) (> angle 0.0)) (.yaw (`self.K2_GetActorRotation` _gun))) (`GameplayStatics.GetWorldDeltaSeconds`) (`self.Vert aim Speed`)))
  (set `self.Current aim` _returnvalue)
  (`self.K2_SetActorRotation` _gun (`KismetMathLibrary.MakeRotator` 0.0 (+ (.pitch _returnvalue) (`/Game/Blueprints/Arms/Gun.current spread on angle` _gun)) (.yaw (`self.K2_GetActorRotation` _gun))) false))

(fn `SnipePoint Location`
  (returns (location :type "Vector Structure"))
  (return (`/Game/Blueprints/Arms/Gun.SnipePoint Location` (`self.Get gun`))))

(fn `Speed`
  (returns (speed :type "Vector Structure"))
  (return (`self.GetVelocity`)))

(fn `UserConstructionScript`)

(fn `Vert Aim on Location`
  (params (location :type "Vector Structure"))
  (bind _gun (`self.Get gun`))
  (bind _returnvalue (- location (`KismetMathLibrary.FindClosestPointOnLine` (`/Game/Blueprints/Arms/Gun.Rotation Point` _gun) (`/Game/Blueprints/Arms/Gun.Endpoint Location` _gun) (`/Game/Blueprints/Arms/Gun.Get Forward Unspread` _gun))))
  (bind _returnvalue_2 (`KismetMathLibrary.Conv_RotatorToVector` (`KismetMathLibrary.MakeRotator` 0.0 0.0 (`KismetMathLibrary.RadiansToDegrees` (`KismetMathLibrary.Vector_HeadingAngle` (- location (`self.SnipePoint Location`)))))))
  (bind _angle (`/Game/Blueprints/System/DDayMacroLibrary.Angle between vectors` _returnvalue _returnvalue_2))
  (if (not (`self.Vertical aim locked`))
    (`self.Set gun vert angle` (`KismetMathLibrary.SelectFloat` _angle (* _angle -1.0) (> (.z _returnvalue) (.z _returnvalue_2))))))