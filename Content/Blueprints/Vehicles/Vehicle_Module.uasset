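; Vehicle module that groups a vehicle's seats and a worker and handles characters boarding it.
; On BeginPlay it scans its child actor components, storing the Vehicle_Worker and collecting each Vehicle_Seat.
; Enter uses the given seat or tries each free one, flagging player control when the boarding character is a Player_Main.
; The crew check always returns false and Out is an empty stub.
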(event `self.ReceiveBeginPlay`
  (for _array_element (`self.GetChildrenComponents` false)
    (bind _aschild_actor_component (cast `ChildActorComponent` _array_element))
    (bind _childactor (`ChildActorComponent.ChildActor` _aschild_actor_component))
    (bind _asvehicle_worker (cast `/Game/Blueprints/Vehicles/Vehicle_Worker` _childactor)
      (:`then`
        (set `self.worker` _asvehicle_worker))
      (:`CastFailed`
        (bind _asvehicle_seat (cast `/Game/Blueprints/Vehicles/Vehicle_Seat` _childactor))
        (`KismetArrayLibrary.Array_Add` (`self.Seats`) _asvehicle_seat)))))

(fn `Enter`
  (params (Seat :type "/Game/Blueprints/Vehicles/Vehicle_Seat Object Reference") (Entrace :type "/Game/Blueprints/Vehicles/Vehicle_Entrace Object Reference") (Charcter :type "/Game/Blueprints/Chars/Abstract/Base_Character Object Reference"))
  (returns (Success :type Boolean))
  (bind (_asplayer_main _bsuccess) (cast `/Game/Blueprints/Chars/Players/Player_Main` Charcter :!pure true))
  (`/Engine/EditorBlueprintResources/StandardMacros.IsValid` Seat
    (:`Is Valid`
      (bind _success (`/Game/Blueprints/Vehicles/Vehicle_Seat.Enter` Seat Entrace Charcter))
      (if _success
        (set `self.Player controled` _bsuccess)
        (return true)
        (else
          (return false))))
    (:`Is Not Valid`
      (for _array_element (`self.Seats`)
        (if (`/Game/Blueprints/Vehicles/Vehicle_Seat.Is free` _array_element)
          (bind _success_2 (`/Game/Blueprints/Vehicles/Vehicle_Seat.Enter` _array_element Entrace Charcter))
          (if _success_2
            (set `self.Player controled` _bsuccess)
            (return true))))
      (return false))))

(fn `Has enough crew`
  (returns (has :type Boolean))
  (return false))

(fn `Has free sits`
  (returns (`Has free` :type Boolean))
  (for _array_element (`self.Seats`)
    (if (`/Game/Blueprints/Vehicles/Vehicle_Seat.Is free` _array_element)
      (return true)))
  (return false))

(fn `Out`
  (params (Character :type "/Game/Blueprints/Chars/Abstract/Base_Character Object Reference")))