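; Menu_Controller is the player controller for the menu, handling cursor input and a hidden dev mode unlock.
; On BeginPlay it shows the mouse cursor, applies game-only input, then switches to Game and UI input after a short delay.
; Each Dev trigger press increments DevRank, and reaching three sets DevMode and prints an on-screen confirmation.
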(event `self.ReceiveBeginPlay`
  (set `self.bShowMouseCursor` true)
  (`WidgetBlueprintLibrary.SetInputMode_GameOnly` self)
  (`KismetSystemLibrary.Delay` 0.2)
  (`WidgetBlueprintLibrary.SetInputMode_GameAndUIEx` self null "DoNotLock" false))

(event `InputAction|Dev trigger`
  (params (Key :type "Key Structure"))
  (:`Pressed`
    (bind _result (`/Engine/EditorBlueprintResources/StandardMacros.IncrementInt` (`self.Dev rank`))
      (:`  `
        (`/Engine/EditorBlueprintResources/StandardMacros.CompareInt` _result 3
          (:`==`
            (set `self.Dev mode` true)
            (`KismetSystemLibrary.PrintString` "Dev mode activated" true true (struct :`R` 1.0 :`A` 1.0) 4.0)))))))

(fn `UserConstructionScript`)