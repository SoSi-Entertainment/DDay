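; Ability Blueprint for a transform that lasts for a limited number of charges rather than running indefinitely.
; Start and end events toggle the transform; ending also records the game time and resets the used-charge count.
; Each ChargeUsed call increments the counter and ends the transform once it reaches ChargesCount.
; GetState keeps the parent's uses, active and cooldown values but reports active percent as the fraction of charges remaining.
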(event `self.Start Transform`
  (`self.Transform` true))

(event `End transform`
  (`self.Transform` false)
  (set `self.last end time` (`KismetSystemLibrary.GetGameTimeInSeconds`))
  (set `self.charges used` 0))

(fn `charge used`
  (bind _result (`/Engine/EditorBlueprintResources/StandardMacros.IncrementInt` (`self.charges used`))
    (:`  `
      (`/Engine/EditorBlueprintResources/StandardMacros.CompareInt` _result (`self.charges count`)
        (:`>`
          _)
        (:`==`
          _))
      (`self.End transform`))))

(fn `Get State`
  (returns (`Available uses` :type Integer) (Active :type Boolean) (`Active percent` :type "Float (double-precision)") (`Cd percent` :type "Float (double-precision)"))
  (bind (_available_uses _active _active_percent _cd_percent) (`parent.Get State`))
  (return _available_uses _active (/ (`KismetMathLibrary.Conv_IntToDouble` (- (`self.charges count`) (`self.charges used`))) (`KismetMathLibrary.Conv_IntToDouble` (`self.charges count`))) _cd_percent))