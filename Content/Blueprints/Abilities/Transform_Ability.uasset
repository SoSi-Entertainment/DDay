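; Timed transform ability that switches an active flag on for a set Duration.
; Use defers to the parent check and, on success, fires StartTransform, which sets IsActive, waits, clears it and records LastEndTime.
; TurnOff runs the parent logic and clears the flag immediately, without cancelling the pending delay or recording an end time.
; Transform only sets IsActive, with no visual or stat change here, and SetStartVars is empty.
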(event `Start Transform`
  (`self.Transform` true)
  (`KismetSystemLibrary.Delay` (`self.Duration`))
  (`self.Transform` false)
  (set `self.last end time` (`KismetSystemLibrary.GetGameTimeInSeconds`)))

(fn `Set start vars`)

(fn `Transform`
  (params (Ability :type Boolean))
  (set `self.Is active` Ability))

(fn `Turn off`
  (`parent.Turn off`)
  (`self.Transform` false))

(fn `Use`
  (returns (Success :type Boolean))
  (bind _success (`parent.Use`))
  (`|ExecutionSequence`
    (:`then_0`
      (if _success
        (`self.Start Transform`)))
    (:`then_1`
      (return _success))))