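; Shield charge ability that rams the owner along tiles in one direction until its target tile, an obstacle or an enemy.
; Transform checks the first gate to pick run, blocked or one-tile hit; each entered tile rechecks during runs.
; Enemies overlapped mid-run take damage, and HitImpact damages the end tile plus surrounding tiles.
; Player charges record case, direction and interruption in save objects, which non-player owners replay through Transform and Abort.
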(event `Parent aborted`
  (params (`Abort info` :type "/Game/Blueprints/recording/events/Ability_Info Object Reference")))

(event `enter tile`
  (params (tile :type "/Game/3D/platforms/Tile Object Reference"))
  (if (!= tile (`self.charge target tile`))
    (bind (_responce _character _target_tile _blocker) (`/Game/3D/platforms/Tile.Check Gate` tile (`self.Charge Dir`) null))
    (switch `/Game/Blueprints/Navigation/Tile_Gate_Responce` _responce
      (:`NewEnumerator0`
        (`/Game/3D/platforms/Tile.press effect` tile true :!label _label))
      (:`NewEnumerator8`
        (goto _label))
      (:`NewEnumerator2`
        (cast `/Game/Blueprints/Chars/Players/Player_Main` (`self.Owner character`) :!label _label_2)
        (`self.charge end` true tile)
        (`self.shake if wire` _responce _blocker))
      (:`NewEnumerator3`
        (cast `/Game/Blueprints/Logics/StaticTargets/BP_BarricadeSandbag` _blocker
          (:`then`
            (goto _label_2))
          (:`CastFailed`
            (cast `/Game/Blueprints/Chars/Players/Player_Main` (`self.Owner character`) :!label _label_3
              (:`then`
                (`self.charge end` false _target_tile))
              (:`CastFailed`
                (`/Game/3D/platforms/Tile.Damage Visitors` _target_tile "NewEnumerator0" (`self.Hit damage`) false (`self.Owner character`) false (0.0 0.0 0.0)))))))
      (:`NewEnumerator4`
        (goto _label))
      (:`NewEnumerator5`
        (goto _label_3))
      (:`NewEnumerator1`
        (goto _label_2))
      (:`NewEnumerator6`
        (goto _label_2))
      (:`NewEnumerator7`
        (goto _label_2)))
    (else
      (`self.charge end` true tile))))

(event `On overlap body`
  (params (OverlappedComponent :type "PrimitiveComponent Object Reference") (OtherActor :type "Actor Object Reference") (OtherComp :type "PrimitiveComponent Object Reference") (OtherBodyIndex :type Integer) (bFromSweep :type Boolean) (SweepResult :type "HitResult Structure (by ref)"))
  (bind _owner_character (`self.Owner character`))
  (bind _asenemy_character (cast `/Game/Blueprints/Chars/Abstract/Enemy_Character` OtherActor))
  (`/Game/Blueprints/Chars/Abstract/Base_Character.got radial damage` _asenemy_character 500.0 "/Game/Blueprints/Logics/Components/tile_damage.tile_damage" (`Actor.K2_GetActorLocation` _owner_character) true _owner_character)
  (`GameplayStatics.ApplyDamage` _asenemy_character 500.0 null _owner_character))

(event `charge end`
  (params (interrupted :type Boolean) (`Ended On tile` :type "/Game/3D/platforms/Tile Object Reference"))
  (`|ExecutionSequence`
    (:`then_0`
      (`KismetSystemLibrary.Delay` 0.5)
      (set `self.In charge_or small after` false)
      (remove `PrimitiveComponent.OnComponentBeginOverlap` (`/Game/Blueprints/Chars/Abstract/Base_Character.BodyCollision` (`self.Owner character`)) (delegate `On overlap body`)))
    (:`then_1`
      (set `self.In charge` false)
      (`self.hit impact` `Ended On tile`)
      (`|ExecutionSequence`
        (:`then_0`
          (bind _asplayer_main (cast `/Game/Blueprints/Chars/Players/Player_Main` (`self.Owner character`)))
          (`Controller.StopMovement` (`AIBlueprintHelperLibrary.GetAIController` _asplayer_main))
          (`/Game/Blueprints/Navigation/Player_Movement.Stop charge process` (`/Game/Blueprints/Controllers/Player_Controller.Player_Movement` (`/Game/Blueprints/System/Funtions/FunctionLibrary.Get PlayerController Troops`)))
          (bind _returnvalue (`GameplayStatics.CreateSaveGameObject` "/Game/Blueprints/recording/events/Charge/Charge_Abort_Info.Charge_Abort_Info_C"))
          (set `/Game/Blueprints/recording/events/Charge/Charge_Abort_Info.Interrupted` interrupted _returnvalue)
          (`/Game/Blueprints/Controllers/Player_Controller.Save event` (`/Game/Blueprints/System/Funtions/FunctionLibrary.Get PlayerController Troops`) "NewEnumerator1" _returnvalue)
          (`KismetSystemLibrary.Delay` 0.3)
          (`/Game/Blueprints/Controllers/Player_Controller.Block input` (`/Game/Blueprints/System/Funtions/FunctionLibrary.Get PlayerController Troops`) false false)
          (`/Game/Blueprints/Arms/Hands/Arsenal.Fixate all arms forward` (`/Game/Blueprints/Chars/Abstract/Base_Character.Get Arsenal` (`self.Owner character`)) false false))
        (:`then_1`
          (`Character.PlayAnimMontage` (`self.Owner character`) (select `bool` interrupted :`false` "/Game/Anim/Charge/Charge_End_Montage.Charge_End_Montage" :`true` "/Game/Anim/Charge/Charge_Interrupt_Montage.Charge_Interrupt_Montage" :!type "AnimMontage Object Reference") 1.0 "None")
          (remove `/Game/Blueprints/Chars/Abstract/Base_Character.enter tile` (`self.Owner character`) (`|CreateDelegate` :!event `enter tile`))
          (`self.unlock walking after charge end`))))))

(event `hit impact`
  (params (`hit tile` :type "/Game/3D/platforms/Tile Object Reference"))
  (`/Game/3D/platforms/Tile.Highlight for period` `hit tile` (struct :`R` 1.0 :`A` 1.0) 0.2 1.0 0 null false :!enabledstate Disabled)
  (`/Game/3D/platforms/Tile.Damage Visitors` `hit tile` "NewEnumerator0" (`self.Hit damage`) false (`self.Owner character`) false (0.0 0.0 0.0))
  (`/Game/3D/platforms/Tile.press effect` `hit tile` true)
  (`|SpawnActorFromClass` (`self.impact effect`) (`KismetMathLibrary.MakeTransform` (+ (`Actor.K2_GetActorLocation` `hit tile`) (0.0 0.0 20.0)) (`Actor.K2_GetActorRotation` `hit tile`)) "Undefined" "MultiplyWithRoot" null null)
  (bind _tiles (`self.Get AUE impact tiles` `hit tile` (`self.Charge Dir`)))
  (`KismetSystemLibrary.Delay` 0.2)
  (for _array_element _tiles
    (`/Game/3D/platforms/Tile.Highlight for period` _array_element (struct :`R` 1.0 :`G` 0.783 :`A` 1.0) 0.2 1.0 0 null false :!enabledstate Disabled)
    (`/Game/3D/platforms/Tile.press effect` _array_element true)
    (`/Game/3D/platforms/Tile.Damage Visitors` _array_element "NewEnumerator0" (`self.AUE damage`) false (`self.Owner character`) false (0.0 0.0 0.0))))

(event `unlock walking after charge end`
  (bind _player_movement (`/Game/Blueprints/Controllers/Player_Controller.Player_Movement` (`/Game/Blueprints/System/Funtions/FunctionLibrary.Get PlayerController Troops`)))
  (`KismetSystemLibrary.Delay` 0.3)
  (cast `/Game/Blueprints/Chars/Players/Player_Main` (`self.Owner character`))
  (`/Game/Blueprints/Navigation/Player_Movement.Update walk speed` _player_movement 1.0)
  (set `/Game/Blueprints/Navigation/Player_Movement.in charge` false _player_movement))

(fn `Abort`
  (params (`Abort info` :type "/Game/Blueprints/recording/events/Ability_Info Object Reference"))
  (bind _charge_dir (`self.Charge Dir`))
  (bind _interrupted (`/Game/Blueprints/recording/events/Charge/Charge_Abort_Info.Interrupted` (cast `/Game/Blueprints/recording/events/Charge/Charge_Abort_Info` `Abort info` :!pure true)))
  (bind _tile (`/Game/Blueprints/System/Funtions/Tile_Functions.Get Tile Under` (`Actor.K2_GetActorLocation` (`self.Owner character`))))
  (bind _tile_2 (`/Game/3D/platforms/Tile.Get Neighbour` _tile _charge_dir))
  (`self.charge end` _interrupted (select `bool` _interrupted :`false` (`/Game/3D/platforms/Tile.Get Neighbour` _tile_2 _charge_dir) :`true` _tile_2)))

(fn `Get AUE impact tiles`
  (params (`impact tile` :type "/Game/3D/platforms/Tile Object Reference") (`impact direction` :type "/Game/Data/enums/Direction Enum" :default "NewEnumerator4"))
  (returns (Tiles :type "Array of /Game/3D/platforms/Tile Object Reference"))
  (locals (`Aue tiles` :type "Array of /Game/3D/platforms/Tile Object Reference"))
  (bind _aue_tiles (`local.Aue tiles`))
  (bind _impact_direction (`local.impact direction`))
  (bind _aue_tiles_2 (`local.Aue tiles`))
  (bind (_tile _not_empty) (`/Game/3D/platforms/Tile.Get Neighbour` `impact tile` (`/Game/Blueprints/System/Funtions/FunctionLibrary.Rotate Direction` "NewEnumerator0" `impact direction`)))
  (bind (_tile_2 _not_empty_2) (`/Game/3D/platforms/Tile.Get Neighbour` `impact tile` (`/Game/Blueprints/System/Funtions/FunctionLibrary.Rotate Direction` "NewEnumerator3" `impact direction`)))
  (bind (_tile_3 _not_empty_3) (`/Game/3D/platforms/Tile.Get Neighbour` `impact tile` (`/Game/Blueprints/System/Funtions/FunctionLibrary.Rotate Direction` "NewEnumerator2" `impact direction`)))
  (bind (_tile_4 _not_empty_4) (`/Game/3D/platforms/Tile.Get Neighbour` _tile (`/Game/Blueprints/System/Funtions/FunctionLibrary.Rotate Direction` "NewEnumerator2" _impact_direction)))
  (bind (_tile_5 _not_empty_5) (`/Game/3D/platforms/Tile.Get Neighbour` _tile (`/Game/Blueprints/System/Funtions/FunctionLibrary.Rotate Direction` "NewEnumerator3" _impact_direction)))
  (`|ExecutionSequence`
    (:`then_0`
      (if _not_empty_2
        (`KismetArrayLibrary.Array_Add` _aue_tiles_2 _tile_2)))
    (:`then_1`
      (if _not_empty_3
        (`KismetArrayLibrary.Array_Add` _aue_tiles_2 _tile_3)))
    (:`then_2`
      (if _not_empty
        (`|ExecutionSequence`
          (:`then_0`
            (`KismetArrayLibrary.Array_Add` _aue_tiles_2 _tile))
          (:`then_1`
            (if _not_empty_5
              (`KismetArrayLibrary.Array_Add` _aue_tiles _tile_5)))
          (:`then_2`
            (if _not_empty_4
              (`KismetArrayLibrary.Array_Add` _aue_tiles _tile_4))))))
    (:`then_5`
      (return (`local.Aue tiles`)))))

(fn `shake if wire`
  (params (`block reason` :type "/Game/Blueprints/Navigation/Tile_Gate_Responce Enum" :default "NewEnumerator0") (blocker :type "Object Object Reference"))
  (if (`|EnumEquality` `block reason` "NewEnumerator2")
    (bind _asstatic_mesh_actor (cast `StaticMeshActor` blocker))
    (if (== (`StaticMeshComponent.StaticMesh` (`StaticMeshActor.StaticMeshComponent` _asstatic_mesh_actor)) "/Game/3D/Artificial/wire/Wire/SM_wire.SM_wire")
      (`/Game/Blueprints/Navigation/Player_Movement.Shake wire` (`/Game/Blueprints/Controllers/Player_Controller.Player_Movement` (`/Game/Blueprints/System/Funtions/FunctionLibrary.Get PlayerController Troops`)) _asstatic_mesh_actor))))

(fn `Transform`
  (params (Ability :type Boolean) (`Ability info in` :type "/Game/Blueprints/recording/events/Ability_Info Object Reference"))
  (returns (`Ability info out` :type "/Game/Blueprints/recording/events/Ability_Info Object Reference"))
  (locals (`Charge info` :type "/Game/Blueprints/recording/events/Charge/Charge_Info Object Reference"))
  (bind _owner_character (`self.Owner character`))
  (bind _arsenal (`/Game/Blueprints/Chars/Abstract/Base_Character.Get Arsenal` (`self.Owner character`)))
  (bind _returnvalue (`Actor.K2_GetActorLocation` (`self.Owner character`)))
  (bind _ascharge_info (cast `/Game/Blueprints/recording/events/Charge/Charge_Info` (`local.Ability info in`) :!pure true))
  (bind _charge_direction (`/Game/Blueprints/recording/events/Charge/Charge_Info.Charge direction` _ascharge_info))
  (`|ExecutionSequence`
    (:`then_0`
      (if Ability
        (cast `/Game/Blueprints/Chars/Players/Player_Main` (`self.Owner character`)
          (:`then`
            (bind _output_get (set `self.Charge Dir` (`/Game/Blueprints/Navigation/Player_Movement.Get dir for charge` (`/Game/Blueprints/Controllers/Player_Controller.Player_Movement` (`/Game/Blueprints/System/Funtions/FunctionLibrary.Get PlayerController Troops`)))))
            (bind _tile (`/Game/Blueprints/System/Funtions/Tile_Functions.Get Tile Under` (+ (`Actor.K2_GetActorLocation` (`self.Owner character`)) (* (`/Game/Blueprints/System/Funtions/FunctionLibrary.Vector from direction` _output_get) 20.0))))
            (bind (_responce _character _target_tile _blocker) (`/Game/3D/platforms/Tile.Check Gate` _tile _output_get null))
            (switch `/Game/Blueprints/Navigation/Tile_Gate_Responce` _responce
              (:`NewEnumerator0`
                (add `/Game/Blueprints/Chars/Abstract/Base_Character.enter tile` _owner_character (`|CreateDelegate` :!event `enter tile`) :!label _label)
                (`Character.PlayAnimMontage` _owner_character "/Game/Anim/Charge/Charge_Montage.Charge_Montage" 1.0 "None")
                (set `self.In charge` true)
                (set `self.In charge_or small after` true)
                (add `PrimitiveComponent.OnComponentBeginOverlap` (`/Game/Blueprints/Chars/Abstract/Base_Character.BodyCollision` (`self.Owner character`)) (`|CreateDelegate` :!event `On overlap body`))
                (cast `/Game/Blueprints/Chars/Players/Player_Main` (`self.Owner character`)
                  (:`then`
                    (bind (_target_tile_2 _charge_dir) (`/Game/Blueprints/Navigation/Player_Movement.Start charge` (`/Game/Blueprints/Controllers/Player_Controller.Player_Movement` (`/Game/Blueprints/System/Funtions/FunctionLibrary.Get PlayerController Troops`)) (`self.Charge Lenght In Tiles`)))
                    (set `self.Charge Target Tile` _target_tile_2)
                    (bind _output_get_2 (set `self.Charge Dir` _charge_dir))
                    (bind _returnvalue_2 (`GameplayStatics.CreateSaveGameObject` "/Game/Blueprints/recording/events/Charge/Charge_Info.Charge_Info_C"))
                    (bind _output_get_3 (set `local.Charge info` _returnvalue_2))
                    (set `/Game/Blueprints/recording/events/Charge/Charge_Info.Charge direction` _output_get_2 _output_get_3)
                    (`/Game/Blueprints/Controllers/Player_Controller.Block input` (`/Game/Blueprints/System/Funtions/FunctionLibrary.Get PlayerController Troops`) true false)
                    (`/Game/Blueprints/Arms/Hands/Arsenal.Update used arms` _arsenal true true)
                    (`/Game/Blueprints/Arms/Hands/Arsenal.Fixate all arms forward` _arsenal true true))
                  (:`CastFailed`
                    (set `self.Charge Dir` (`/Game/Blueprints/recording/events/Charge/Charge_Info.Charge direction` (cast `/Game/Blueprints/recording/events/Charge/Charge_Info` (`local.Ability info in`) :!pure true))))))
              (:`NewEnumerator8`
                (goto _label))
              (:`NewEnumerator2`
                (`self.shake if wire` _responce _blocker :!label _label_2)
                (`/Game/Blueprints/Chars/Abstract/Base_Character.Shake body in dir` (`self.Owner character`) (`self.Charge Dir`))
                (`self.hit impact` null)
                (bind _returnvalue_3 (`GameplayStatics.CreateSaveGameObject` "/Game/Blueprints/recording/events/Charge/Charge_Info.Charge_Info_C"))
                (bind _output_get_4 (set `local.Charge info` _returnvalue_3))
                (set `/Game/Blueprints/recording/events/Charge/Charge_Info.Charge case` "NewEnumerator1" _output_get_4)
                (set `/Game/Blueprints/recording/events/Charge/Charge_Info.Charge direction` (`self.Charge Dir`) _output_get_4)
                (`/Game/Blueprints/Arms/Hands/Arsenal.Update used arms` (`/Game/Blueprints/Chars/Abstract/Base_Character.Get Arsenal` (`self.Owner character`)) true true))
              (:`NewEnumerator3`
                (cast `/Game/Blueprints/Logics/StaticTargets/BP_BarricadeSandbag` _blocker
                  (:`then`
                    (goto _label_2))
                  (:`CastFailed`
                    (set `/Game/Blueprints/Navigation/Player_Movement.in charge` true (`/Game/Blueprints/Controllers/Player_Controller.Player_Movement` (`/Game/Blueprints/System/Funtions/FunctionLibrary.Get PlayerController Troops`)) :!label _label_3)
                    (`Character.PlayAnimMontage` (`self.Owner character`) "/Game/Anim/Charge/Charge_1_Tile_Montage.Charge_1_Tile_Montage" 1.0 "None")
                    (`self.hit impact` _target_tile)
                    (bind _returnvalue_4 (`GameplayStatics.CreateSaveGameObject` "/Game/Blueprints/recording/events/Charge/Charge_Info.Charge_Info_C"))
                    (bind _output_get_5 (set `local.Charge info` _returnvalue_4))
                    (set `/Game/Blueprints/recording/events/Charge/Charge_Info.Charge case` "NewEnumerator2" _output_get_5)
                    (set `/Game/Blueprints/recording/events/Charge/Charge_Info.Charge direction` (`self.Charge Dir`) _output_get_5)
                    (`self.unlock walking after charge end`)
                    (`/Game/Blueprints/Arms/Hands/Arsenal.Update used arms` (`/Game/Blueprints/Chars/Abstract/Base_Character.Get Arsenal` (`self.Owner character`)) true true))))
              (:`NewEnumerator4`
                (goto _label))
              (:`NewEnumerator5`
                (goto _label_3))
              (:`NewEnumerator1`
                (goto _label_2))
              (:`NewEnumerator6`
                (goto _label_2))
              (:`NewEnumerator7`
                (goto _label_2))))
          (:`CastFailed`
            (`/Game/Blueprints/Arms/Hands/Arsenal.Update used arms` (`/Game/Blueprints/Chars/Abstract/Base_Character.Get Arsenal` (`self.Owner character`)) true true)
            (switch `/Game/Blueprints/recording/events/Charge/Charge_Case` (`/Game/Blueprints/recording/events/Charge/Charge_Info.Charge case` _ascharge_info)
              (:`NewEnumerator0`
                (goto _label))
              (:`NewEnumerator1`
                (set `self.Charge Dir` _charge_direction)
                (bind _tile_2 (`/Game/Blueprints/System/Funtions/Tile_Functions.Get Tile Under` _returnvalue))
                (`self.hit impact` _tile_2))
              (:`NewEnumerator2`
                (bind _output_get_6 (set `self.Charge Dir` _charge_direction))
                (`Character.PlayAnimMontage` (`self.Owner character`) "/Game/Anim/Charge/Charge_1_Tile_Montage.Charge_1_Tile_Montage" 1.0 "None")
                (bind _tile_3 (`/Game/Blueprints/System/Funtions/Tile_Functions.Get Tile Under` _returnvalue))
                (`self.hit impact` (`/Game/3D/platforms/Tile.Get Neighbour` _tile_3 _output_get_6))))))
        (else
          (`/Game/Blueprints/Arms/Hands/Arsenal.Update used arms` (`/Game/Blueprints/Chars/Abstract/Base_Character.Get Arsenal` (`self.Owner character`)) true false))))
    (:`then_1`
      (`parent.Transform` Ability `Ability info in`)
      (return (`local.Charge info`)))))