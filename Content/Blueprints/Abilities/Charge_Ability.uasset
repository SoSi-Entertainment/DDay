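; Charge ability that plays a charge montage on its owning character and starts a charge movement for the player.
; It overrides Use and acts only when the parent Use succeeds, then returns that parent result.
; The movement step runs only for a Player_Main owner, calling StartCharge on the PlayerMovement obtained through GetPlayerControllerTroops.
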(fn `Use`
  (returns (Success :type Boolean))
  (bind _owner_character (`self.Owner character`))
  (bind _success (`parent.Use`))
  (`|ExecutionSequence`
    (:`then_0`
      (if _success
        (`Character.PlayAnimMontage` _owner_character "/Game/Anim/Charge/Charge_Montage.Charge_Montage" 1.0 "None")
        (cast `/Game/Blueprints/Chars/Players/Player_Main` _owner_character)
        (`/Game/Blueprints/Navigation/Player_Movement.Start charge` (`/Game/Blueprints/Controllers/Player_Controller.Player_Movement` (`/Game/Blueprints/System/Funtions/FunctionLibrary.Get PlayerController Troops`)))))
    (:`then_1`
      (return _success))))