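; Shield ability that switches on or off through an overridden Transform function on its owning character.
; Switching off while active saves an event on the player controller, but only for player-owned characters.
; It then runs the parent transform, updates arsenal arm usage (right always, middle while shielding) and locks vertical aim while the shield is up.
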(fn `Transform`
  (params (Ability :type Boolean))
  (bind _asbase_character (cast `/Game/Blueprints/Chars/Abstract/Base_Character` (`self.GetOwner`) :!pure true))
  (`|ExecutionSequence`
    (:`then_0`
      (if Ability
        _
        (elif (`self.Is active`)
          (cast `/Game/Blueprints/Chars/Players/Player_Main` _asbase_character)
          (`/Game/Blueprints/Controllers/DDay_Player_Controller.Save event` (`/Game/Blueprints/System/FunctionLibrary.Get PlayerController Troops`) "NewEnumerator1"))))
    (:`then_1`
      (`parent.Transform` Ability)
      (`/Game/Blueprints/Arms/Hands/Arsenal.Update used arms` (`/Game/Blueprints/Chars/Abstract/Base_Character.Get Arsenal` _asbase_character) true Ability)
      (set `/Game/Blueprints/Chars/Abstract/Base_Character.Vertical aim locked` Ability _asbase_character))))