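; Time slow ability that slows the world while active and keeps its owning Base_Character at normal speed.
; Transform sets global time dilation to the inverse of SlowCoef, offsets it with the owner's CustomTimeDilation, and swaps in a scaled gun cooldown, restoring all three when off.
; SetupStats caches original and scaled cooldown and walk speed values.
; The walk speed, shot sound and shell swaps are disconnected and never run.
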(event `self.ReceiveBeginPlay`
  (`parent.ReceiveBeginPlay`))

(fn `Setup stats`
  (params (params :type "/Game/Data/structs/Ability_Params Structure"))
  (bind _asbase_character (cast `/Game/Blueprints/Chars/Abstract/Base_Character` (`self.GetOwner`) :!pure true))
  (bind _cd_length (`/Game/Blueprints/Arms/Gun.cd length` (`/Game/Blueprints/Chars/Abstract/Base_Character.Get gun` _asbase_character)))
  (`parent.Setup stats` params)
  (set `self.original gun cd` _cd_length)
  (set `self.fast gun cd` (/ _cd_length (`self.slow coef`)))
  (bind _output_get (set `self.original speed` (`CharacterMovementComponent.MaxWalkSpeed` (`Character.CharacterMovement` _asbase_character))))
  (set `self.fast speed` (* _output_get (`self.slow coef`))))

(fn `Transform`
  (params (Ability :type Boolean) (`Ability info in` :type "/Game/Blueprints/recording/events/Ability_Info Object Reference"))
  (bind _ability (`local.Ability`))
  (bind _asbase_character (cast `/Game/Blueprints/Chars/Abstract/Base_Character` (`self.GetOwner`) :!pure true))
  (`parent.Transform` Ability null)
  (set `/Game/Blueprints/Arms/Gun.cd length` (`KismetMathLibrary.SelectFloat` (`self.fast gun cd`) (`self.original gun cd`) Ability) (`/Game/Blueprints/Chars/Abstract/Base_Character.Get gun` _asbase_character))
  (`GameplayStatics.SetGlobalTimeDilation` (`KismetMathLibrary.SelectFloat` (/ 1.0 (`self.slow coef`)) 1.0 _ability))
  (set `Actor.CustomTimeDilation` (`KismetMathLibrary.SelectFloat` (`self.slow coef`) 1.0 _ability) _asbase_character))