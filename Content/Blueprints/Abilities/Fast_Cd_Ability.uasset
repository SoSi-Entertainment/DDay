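; Ability component that temporarily turns the owning character's gun into a faster-firing one by shortening its shot cooldown.
; SetupStats caches the gun's original cooldown and derives the fast one by dividing it by a coefficient from the ability parameters.
; Transform extends the parent's toggle, switching the gun's cooldown, shot sound and shell type between ability and normal versions.
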(event `self.ReceiveBeginPlay`
  (`parent.ReceiveBeginPlay`))

(fn `Setup stats`
  (params (params :type "/Game/Data/structs/Ability_Params Structure"))
  (bind _cd_length (`/Game/Blueprints/Arms/Gun.cd length` (`/Game/Blueprints/Chars/Abstract/Base_Character.Get gun` (cast `/Game/Blueprints/Chars/Abstract/Base_Character` (`self.GetOwner`) :!pure true))))
  (`parent.Setup stats` params)
  (set `self.Fast coef` (`KismetStringLibrary.Conv_StringToDouble` (`|GetArrayItem` (`.Abilityparams_11_E8D4A37B491C7A9543C0D3A6F050EB2D` (break `/Game/Data/structs/Ability_Params` params)))))
  (set `self.original gun cd` _cd_length)
  (set `self.fast gun cd` (/ _cd_length (`self.Fast coef`))))

(fn `Transform`
  (params (Ability :type Boolean) (`Ability info in` :type "/Game/Blueprints/recording/events/Ability_Info Object Reference"))
  (bind _gun (`/Game/Blueprints/Chars/Abstract/Base_Character.Get gun` (cast `/Game/Blueprints/Chars/Abstract/Base_Character` (`self.GetOwner`) :!pure true)))
  (`parent.Transform` Ability null)
  (set `/Game/Blueprints/Arms/Gun.cd length` (`KismetMathLibrary.SelectFloat` (`self.fast gun cd`) (`self.original gun cd`) Ability) _gun)
  (set `/Game/Blueprints/Arms/Gun.Shot Sound` (select `bool` Ability :`false` "/Game/Sounds/Shoting_Cue/Tommy_Cue.Tommy_Cue" :`true` "/Game/Sounds/Shoting_Cue/MachineGun_Cue.MachineGun_Cue" :!type "SoundCue Object Reference") _gun)
  (set `/Game/Blueprints/Arms/Gun.shell type` (select `bool` Ability :`false` "/Game/Blueprints/Arms/Shells/Shell.Shell_C" :`true` "/Game/Blueprints/Arms/Shells/Ability_Shell.Ability_Shell_C" :!type "/Game/Blueprints/Arms/Shells/Shell Class Reference") _gun))