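; Grenade ability that lets a character throw a damaging grenade toward its aim location.
; Use defers to the parent ability and, on success, spawns a Grenade actor at the owning Base_Character's left hand.
; The grenade receives damage, radius, normalized hand-to-aim direction and the owner's speed at spawn.
; SetupStats extends the parent setup, reading damage and radius from the ability parameters.
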(fn `Setup stats`
  (params (params :type "/Game/Data/structs/Ability_Params Structure"))
  (bind (_abilitycount _abilitycd _abilityduration _abilityparams) (break `/Game/Data/structs/Ability_Params` params))
  (`parent.Setup stats` params)
  (set `self.Damage` (`KismetStringLibrary.Conv_StringToDouble` (`|GetArrayItem` _abilityparams)))
  (set `self.Radius` (`KismetStringLibrary.Conv_StringToDouble` (`|GetArrayItem` _abilityparams 1))))

(fn `Use`
  (params (`Ability info in` :type "/Game/Blueprints/recording/events/Ability_Info Object Reference"))
  (returns (Success :type Boolean) (`Ability info out` :type "/Game/Blueprints/recording/events/Ability_Info Object Reference"))
  (bind _returnvalue (`self.GetOwner`))
  (bind _asbase_character (cast `/Game/Blueprints/Chars/Abstract/Base_Character` _returnvalue :!pure true))
  (bind _location (`/Game/Blueprints/Chars/Abstract/Base_Character.Left hand location` _asbase_character))
  (bind _returnvalue_2 (- (`/Game/Blueprints/Chars/Abstract/Base_Character.Aim location` _asbase_character) _location))
  (bind _success (`parent.Use` `Ability info in`))
  (`|ExecutionSequence`
    (:`then_0`
      (if _success
        (`|SpawnActorFromClass` "/Game/Blueprints/Abilities/Grenade.Grenade_C" (`KismetMathLibrary.MakeTransform` _location (`KismetMathLibrary.MakeRotator` 45.0 45.0 (.yaw (`KismetMathLibrary.MakeRotFromX` _returnvalue_2)))) "Undefined" "MultiplyWithRoot" _returnvalue (`self.Damage`) (`self.Radius`) (`KismetMathLibrary.Normal` _returnvalue_2) (`/Game/Blueprints/Chars/Abstract/Base_Character.Get speed` _asbase_character) null)))
    (:`then_1`
      (return _success null))))