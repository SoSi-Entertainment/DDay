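; Thrown grenade actor that explodes after a fuse or when it overlaps an enemy character.
; On BeginPlay it launches its cube along the throw direction with a vertical impulse, half the owner's speed and added spin.
; The first hit starts the fuse delay, while overlapping an enemy of the owner detonates it immediately.
; Explode spawns an actor carrying damage, radius and sound, then destroys the grenade.
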(event `self.ReceiveBeginPlay`
  (`PrimitiveComponent.SetPhysicsLinearVelocity` (`self.Cube`) (+ (`KismetMathLibrary.Conv_Vector2DToVector` (* (`KismetMathLibrary.Conv_VectorToVector2D` (`self.throw direction`)) 400.0) (`self.vertical impulse`)) (/ (`self.Owner speed`) 2.0)) false "None")
  (`PrimitiveComponent.SetPhysicsAngularVelocityInDegrees` (`self.Cube`) (-200.0 200.0 0.0) false "None")
  (`PrimitiveComponent.SetPhysicsAngularVelocityInDegrees` (`self.Cube`) (-200.0 200.0 0.0) false "None"))

(event `self.ReceiveHit`
  (params (MyComp :type "PrimitiveComponent Object Reference") (Other :type "Actor Object Reference") (OtherComp :type "PrimitiveComponent Object Reference") (bSelfMoved :type Boolean) (HitLocation :type "Vector Structure") (HitNormal :type "Vector Structure") (NormalImpulse :type "Vector Structure") (Hit :type "HitResult Structure (by ref)"))
  (`/Engine/EditorBlueprintResources/StandardMacros.DoOnce` false
    (:`Completed`
      (`KismetSystemLibrary.Delay` (`self.Timer`))
      (`self.Explode`))))

(event `self.ReceiveActorBeginOverlap`
  (params (OtherActor :type "Actor Object Reference"))
  (bind _asbase_character (cast `/Game/Blueprints/Chars/Abstract/Base_Character` OtherActor))
  (if (`/Game/Blueprints/System/FunctionLibrary.Are enemies` (cast `/Game/Blueprints/Chars/Abstract/Base_Character` (`self.GetOwner`) :!pure true) _asbase_character)
    (`self.Explode`)))

(fn `Explode`
  (`|SpawnActorFromClass` "/Game/Blueprints/Logics/Components/Vibooh_grenade.Vibooh_grenade_C" (`KismetMathLibrary.MakeTransform` (`self.K2_GetActorLocation`)) "Undefined" "MultiplyWithRoot" (`self.GetOwner`) (`self.Damage`) (`self.Radius`) "/Game/Sounds/Shoting_Cue/Grenade_norm.Grenade_norm" null)
  (`self.K2_DestroyActor`))

(fn `UserConstructionScript`)