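; Base ability component on a Clone_Main owner that gates uses by active state, a use limit and a cooldown.
; Use records the count and time, then calls SetStartVars to stamp LastEndTime, from which the cooldown runs.
; Owners flagged as Repeater bypass every check and bookkeeping step.
; GetState reports remaining uses, active state, duration and cooldown progress, while TurnOff is an empty stub.
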(event `self.ReceiveBeginPlay`
  (set `self.last use time` (* (`self.cd`) -1.0))
  (bind _asclone_main (cast `/Game/Blueprints/Chars/Clones/Clone_Main` (`self.GetOwner`)))
  (set `self.ignore rules` (`/Game/Blueprints/Chars/Clones/Clone_Main.Repeater` _asclone_main)))

(fn `Get State`
  (returns (`Available uses` :type Integer) (Active :type Boolean) (`Active percent` :type "Float (double-precision)") (`Cd percent` :type "Float (double-precision)"))
  (bind _returnvalue (- (`self.Count`) (`self.Used`)))
  (return _returnvalue (`self.Is active`) (- 1.0 (/ (- (`KismetSystemLibrary.GetGameTimeInSeconds`) (`self.last use time`)) (`self.Duration`))) (`KismetMathLibrary.SelectFloat` (/ (- (`KismetSystemLibrary.GetGameTimeInSeconds`) (`self.last end time`)) (`self.cd`)) 0.0 (> _returnvalue 0))))

(fn `Set start vars`
  (set `self.last end time` (`KismetSystemLibrary.GetGameTimeInSeconds`)))

(fn `Turn off`)

(fn `Use`
  (returns (Success :type Boolean))
  (bind _returnvalue (`KismetSystemLibrary.GetGameTimeInSeconds`))
  (if (`self.ignore rules`)
    (return true)
    (elif (not (`self.Is active`))
      (`/Engine/EditorBlueprintResources/StandardMacros.CompareInt` (`self.Used`) (`self.Count`)
        (:`<`
          (`/Engine/EditorBlueprintResources/StandardMacros.CompareFloat` _returnvalue (+ (`self.last end time`) (`self.cd`))
            (:`>`
              _)
            (:`==`
              _))
          (`/Engine/EditorBlueprintResources/StandardMacros.IncrementInt` (`self.Used`)
            (:`  `
              (set `self.last use time` _returnvalue)
              (`self.Set start vars`)
              (return true))))))))