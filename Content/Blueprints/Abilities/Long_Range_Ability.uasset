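; Long-range ability that temporarily turns the owning character's gun into a precise long-range weapon.
; SetupStats caches the gun's original spread and shell settings, then builds boosted shell params and camera offset from ability parameters.
; Transform toggles spread, shell type and params, refreshes aim spread, and adjusts camera height for Player_Main owners.
; While active, it binds to the gun's shoot event so shots consume charges; deactivation unbinds all that event's listeners.
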(event `self.ReceiveBeginPlay`
  (`parent.ReceiveBeginPlay`))

(fn `On gun shoot`
  (`self.charge used`))

(fn `Setup stats`
  (params (params :type "/Game/Data/structs/Ability_Params Structure"))
  (bind (_abilitycount _abilitycd _abilityduration _abilityparams) (break `/Game/Data/structs/Ability_Params` params))
  (bind _gun (`/Game/Blueprints/Chars/Abstract/Base_Character.Get gun` (cast `/Game/Blueprints/Chars/Abstract/Base_Character` (`self.GetOwner`) :!pure true)))
  (`parent.Setup stats` params)
  (set `self.Original Spread Angles` (`/Game/Blueprints/Arms/Gun.Default Spread angles` _gun))
  (set `self.Original Shell Params` (`/Game/Blueprints/Arms/Gun.Shell params` _gun))
  (set `self.Original Spread Coef` (`/Game/Blueprints/Arms/Gun.Gun spread coef` _gun))
  (set `self.Range` (`KismetStringLibrary.Conv_StringToDouble` (`|GetArrayItem` _abilityparams)))
  (set `self.Cam offset` (`KismetStringLibrary.Conv_StringToDouble` (`|GetArrayItem` _abilityparams 1)))
  (set `self.Speed up coef` (`KismetStringLibrary.Conv_StringToDouble` (`|GetArrayItem` _abilityparams 2)))
  (set `self.damage` (`KismetStringLibrary.Conv_StringToDouble` (`|GetArrayItem` _abilityparams 3)))
  (set `self.Ability Shell Params` (make `/Game/Data/structs/Shell_params` (* (`.Speed_2_80B58CFE496243D9076773A44D02D811` (break `/Game/Data/structs/Shell_params` (`self.Original Shell Params`))) (`self.Speed up coef`)) (`self.damage`) (`self.Range`))))

(fn `Transform`
  (params (Ability :type Boolean))
  (bind _asbase_character (cast `/Game/Blueprints/Chars/Abstract/Base_Character` (`self.GetOwner`) :!pure true))
  (bind _gun (`/Game/Blueprints/Chars/Abstract/Base_Character.Get gun` _asbase_character))
  (`parent.Transform` Ability)
  (set `/Game/Blueprints/Arms/Gun.Gun spread coef` (select `bool` Ability :`false` (`self.Original Spread Coef`)) _gun)
  (set `/Game/Blueprints/Arms/Gun.shell type` (select `bool` Ability :`false` "/Game/Blueprints/Arms/Shells/Rifle_Shell.Rifle_Shell_C" :`true` "/Game/Blueprints/Arms/Shells/Long_Range_Shell.Long_Range_Shell_C" :!type "/Game/Blueprints/Arms/Shells/Shell Class Reference") _gun)
  (set `/Game/Blueprints/Arms/Gun.Default Spread angles` (select `bool` Ability :`false` (`self.Original Spread Angles`) :`true` (make `/Game/Data/structs/Spread_Angles` 1.0 -1.0)) _gun)
  (set `/Game/Blueprints/Arms/Gun.Shell params` (select `bool` Ability :`false` (`self.Original Shell Params`) :`true` (`self.Ability Shell Params`)) _gun)
  (`/Game/Blueprints/Arms/Gun.Update Spread` _gun null (`/Game/Blueprints/Chars/Abstract/Base_Character.Aim location` _asbase_character))
  (if Ability
    (add `/Game/Blueprints/Arms/Gun.Shoot event` _gun (`|CreateDelegate` :!event `On gun shoot`))
    (bind _asplayer_main (cast `/Game/Blueprints/Chars/Players/Player_Main` _asbase_character))
    (`/Game/Blueprints/Chars/Players/Player_Main.Set cam height offset` _asplayer_main (`self.Cam offset`))
    (else
      (clear `/Game/Blueprints/Arms/Gun.Shoot event` _gun)
      (bind _asplayer_main_2 (cast `/Game/Blueprints/Chars/Players/Player_Main` _asbase_character))
      (`/Game/Blueprints/Chars/Players/Player_Main.Set cam height offset` _asplayer_main_2 0.0))))