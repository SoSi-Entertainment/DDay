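; Shield actor for an ability, which caches its parent Base_Character on BeginPlay and can remove itself along with its parent component.
; ShieldAngle derives a yaw from the gun's spread-free forward and 2D aim distance, flagging close aim as unstable so gun yaw can substitute.
; The interpolated rotation logic using that angle is disconnected, and Tick is empty, so this graph never rotates the shield.
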(event `self.ReceiveBeginPlay`
  (bind _asbase_character (cast `/Game/Blueprints/Chars/Abstract/Base_Character` (`self.GetParentActor`)))
  (set `self.body` _asbase_character))

(event `self.ReceiveTick`
  (params (DeltaSeconds :type "Float (single-precision)")))

(fn `remove`
  (`ActorComponent.K2_DestroyComponent` (`self.GetParentComponent`))
  (`self.K2_DestroyActor`))

(fn `Shield angle`
  (returns (`shield angle` :type "Float (double-precision)") (`close unstable` :type Boolean) (`gun angle` :type "Float (double-precision)"))
  (locals (`dist to gun` :type "Float (double-precision)" :default 10.0) (`dist to aim` :type "Float (double-precision)" :default 3.0) (`gun to aim angle` :type "Float (double-precision)" :default 0.0))
  (bind _body (`self.body`))
  (bind _output_get (set `local.dist to aim` (`KismetMathLibrary.Vector_Distance2D` (`self.K2_GetActorLocation` _body) (`/Game/Blueprints/Chars/Abstract/Base_Character.Aim location` _body))))
  (set `local.dist to gun` 65.0)
  (bind _output_get_2 (set `local.gun to aim angle` (.yaw (`KismetMathLibrary.MakeRotFromX` (`/Game/Blueprints/Arms/Gun.Get Forward Unspread` (`/Game/Blueprints/Chars/Abstract/Base_Character.Get gun` (`self.body`)))))))
  (return (- 90.0 (- 180.0 (`KismetMathLibrary.DegAtan2` (`local.dist to gun`) (`local.dist to aim`)) (`local.gun to aim angle`))) (< _output_get 150.0) _output_get_2))

(fn `UserConstructionScript`)