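; Enemy shieldbearer character that pushes and damages allied characters with its shield instead of shooting, as its gun shot override always returns false.
; An ally entering the shield attack area starts a gated loop that calls Push on the Shield_Device, waits out the cooldown and retargets the first overlapping ally until none remain.
; Damage and cooldown come from the parent's unit stats, and tier upgrades shorten the cooldown.
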(event `self.Shiel atatk area.OnComponentBeginOverlap`
  (params (OverlappedComponent :type "PrimitiveComponent Object Reference") (OtherActor :type "Actor Object Reference") (OtherComp :type "PrimitiveComponent Object Reference") (OtherBodyIndex :type Integer) (bFromSweep :type Boolean) (SweepResult :type "HitResult Structure (by ref)"))
  (bind _overlappingactors (`PrimitiveComponent.GetOverlappingActors` (`self.Shiel atatk area`) "/Game/Blueprints/Chars/Abstract/Ally_Character.Ally_Character_C"))
  (bind _asally_character (cast `/Game/Blueprints/Chars/Abstract/Ally_Character` OtherActor))
  (set `self.push target` _asally_character)
  (`/Engine/EditorBlueprintResources/StandardMacros.DoOnce` false :!label _label
    (:`Completed`
      (bind _asshield_device (cast `/Game/Blueprints/Arms/Devices/Shield_Device` (`self.Get Device`)))
      (`/Game/Blueprints/Arms/Devices/Shield_Device.Push` _asshield_device (`self.push target`) (`self.Damage`) :!label _label_2)
      (`KismetSystemLibrary.Delay` (`self.Cd`))
      (if (`KismetArrayLibrary.Array_IsNotEmpty` _overlappingactors)
        (set `self.push target` (cast `/Game/Blueprints/Chars/Abstract/Ally_Character` (`|GetArrayItem` _overlappingactors) :!pure true))
        (goto _label_2)
        (else
          (goto _label :!via `Reset`))))))

(event `self.Up tier`
  (set `self.Cd` (/ (`self.Cd`) (`self.fast cd coef`)))
  (`parent.Up tier`))

(fn `Gun Shoot`
  (params (`shot info` :type "/Game/Blueprints/recording/Shot_Info Object Reference") (`100%hit` :type Boolean) (`Target location` :type "Vector Structure") (`Add owner speed` :type Boolean) (`Hit Targets` :type "Array of /Game/Blueprints/System/Interfaces/Aimable Interface (by ref)"))
  (returns (Done :type Boolean))
  (return false))

(fn `Set unit stats`
  (returns (Stats :type "/Game/Data/structs/Balance_State Structure"))
  (bind _stats (`parent.Set unit stats`))
  (bind ((`Cd_36_46CB7EC3440A0CD2C90916B2276E198F` _cd) (`Bulletdamage_45_88F44442451551AD29B50195A02FD64C` _bulletdamage)) (break `/Game/Data/structs/Balance_State` _stats))
  (set `self.Cd` _cd)
  (set `self.Damage` _bulletdamage)
  (return _stats))

(fn `UserConstructionScript`
  (`parent.UserConstructionScript`))