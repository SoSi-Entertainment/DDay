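; Enemy cannon Blueprint that customizes the hit and death effects of its parent class, with no active event graph logic.
; Die spawns a scaled-up Vibooh with a shell explosion sound and a larger Hit1 just above the platform under it, runs the parent death, then destroys the actor.
; Hit blood spawns a Hit1 oriented to the hit normal and attaches it to the Gun, keeping world transform.
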(fn `Die`
  (params (causer :type "Actor Object Reference") (`Death impulse` :type "Vector Structure") (`Hit location` :type "Vector Structure"))
  (bind _location (`self.Get platform under`))
  (bind _returnvalue (+ _location (0.0 0.0 30.0)))
  (`|SpawnActorFromClass` "/Game/Blueprints/Logics/Components/Vibooh.Vibooh_C" (`KismetMathLibrary.MakeTransform` _returnvalue (struct) (2.0 2.0 2.0)) "Undefined" "MultiplyWithRoot" null 0.0 0.0 "/Game/Sounds/Shoting_Cue/ShellExplosion_Cue.ShellExplosion_Cue" null)
  (`|SpawnActorFromClass` "/Game/Effects/Hit1.Hit1_C" (`KismetMathLibrary.MakeTransform` _returnvalue (struct) (5.0 5.0 5.0)) "Undefined" "MultiplyWithRoot" null null)
  (`parent.Die` causer `Death impulse` `Hit location`)
  (`self.K2_DestroyActor`))

(fn `Hit blood`
  (params (`Hit location` :type "Vector Structure") (`Hit normal` :type "Vector Structure"))
  (bind _returnvalue (`|SpawnActorFromClass` "/Game/Effects/Hit1.Hit1_C" (`KismetMathLibrary.MakeTransform` `Hit location` (`/Game/Blueprints/System/FunctionLibrary.Normal to Rotation` `Hit normal`)) "Undefined" "MultiplyWithRoot" null null))
  (`self.K2_AttachToComponent` _returnvalue (`self.Gun`) "None" "KeepWorld" "KeepWorld" "KeepWorld" false))

(fn `UserConstructionScript`
  (`parent.UserConstructionScript`))