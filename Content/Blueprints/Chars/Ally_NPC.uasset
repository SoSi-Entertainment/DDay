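; Allied soldier NPC character, layering ally-specific behavior over its parent's death, shooting and outline logic.
; Capsule overlap with the player sets an overlapped state and notifies the player, clearing on a short timer that suggests a transparency effect.
; An empty name is generated from the run's stream on first actor overlap, not at BeginPlay.
; Death notifies its NPC_Controller, successful shots play a body animation, and on-screen-based movement tick throttling is left unwired.
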(event `self.ReceiveActorBeginOverlap`
  (params (OtherActor :type "Actor Object Reference"))
  (`parent.ReceiveActorBeginOverlap` OtherActor)
  (if (`KismetStringLibrary.IsEmpty` (`self.Name`))
    (bind _name (`/Game/Blueprints/System/Funtions/FunctionLibrary.Generate Soldier Name from stream` (`self.Get current run stream`)))
    (set `self.Name` _name)))

(event `self.CapsuleComponent.OnComponentBeginOverlap`
  (params (OverlappedComponent :type "PrimitiveComponent Object Reference") (OtherActor :type "Actor Object Reference") (OtherComp :type "PrimitiveComponent Object Reference") (OtherBodyIndex :type Integer) (bFromSweep :type Boolean) (SweepResult :type "HitResult Structure (by ref)"))
  (bind _asplayer_main (cast `/Game/Blueprints/Chars/Players/Player_Main` OtherActor))
  (`KismetSystemLibrary.K2_ClearAndInvalidateTimerHandle` (`self.Transperancy timer`))
  (`self.Set Overlaped` true)
  (`/Game/Blueprints/Chars/Players/Player_Main.New overlapping` _asplayer_main true self))

(event `self.CapsuleComponent.OnComponentEndOverlap`
  (params (OverlappedComponent :type "PrimitiveComponent Object Reference") (OtherActor :type "Actor Object Reference") (OtherComp :type "PrimitiveComponent Object Reference") (OtherBodyIndex :type Integer))
  (cast `/Game/Blueprints/Chars/Players/Player_Main` OtherActor)
  (bind _returnvalue (`KismetSystemLibrary.K2_SetTimerDelegate` (delegate `remove transperancy`) 0.2))
  (set `self.Transperancy timer` _returnvalue))

(event `remove transperancy`
  (`self.Set Overlaped` false)
  (`/Game/Blueprints/Chars/Players/Player_Main.New overlapping` (`/Game/Blueprints/System/Funtions/FunctionLibrary.Get Player Body`) false self))

(event `self.ReceiveTick`
  (params (DeltaSeconds :type "Float (single-precision)")))

(fn `Die`
  (params (causer :type "Actor Object Reference") (`On start` :type Boolean) (`Death impulse local` :type "Vector Structure") (`Hit location local` :type "Vector Structure") (`Death impulse common local` :type "Vector Structure") (suicide :type Boolean) (`killer character` :type "/Game/Blueprints/Chars/Abstract/Base_Character Object Reference"))
  (`parent.Die` causer `On start` `Death impulse local` `Hit location local` `Death impulse common local` suicide `killer character`)
  (`self.Set Overlaped` false)
  (bind _asnpc_controller (cast `/Game/Blueprints/Controllers/NPC_Controller` (`self.GetController`)))
  (`/Game/Blueprints/Controllers/NPC_Controller.Body dead` _asnpc_controller))

(fn `Get gun`
  (returns (Gun :type "/Game/Blueprints/Arms/Gun Object Reference"))
  (return (`parent.Get gun`)))

(fn `Get path`
  (returns (Path :type "/Game/Blueprints/Navigation/Path_holder Object Reference"))
  (return (`self.Path`)))

(fn `Get shooting radius`
  (returns (Radius :type "Float (double-precision)"))
  (return (`self.Attack radius`)))

(fn `Gun Shoot`
  (params (`shot info` :type "/Game/Blueprints/recording/Shot_Info Object Reference") (`100%hit` :type Boolean) (`Target location` :type "Vector Structure") (`Add owner speed` :type Boolean) (`Hit Targets` :type "Array of /Game/Blueprints/System/Interfaces/Aimable Interface (by ref)"))
  (returns (Done :type Boolean))
  (bind _done (`parent.Gun Shoot` `shot info` `100%hit` `Target location` `Add owner speed` `Hit Targets`))
  (if _done
    (`self.Play shoot body anim`))
  (return _done))

(fn `Is on screen`
  (returns (True :type Boolean))
  (locals (offset :type "Float (double-precision)" :default 200.0))
  (bind _offset (`local.offset`))
  (bind _offset_2 (`local.offset`))
  (bind (_x _y) (`KismetMathLibrary.BreakVector2D` (`WidgetLayoutLibrary.GetViewportSize`)))
  (bind (_x_2 _y_2) (`KismetMathLibrary.BreakVector2D` (`PlayerController.ProjectWorldLocationToScreen` (`GameplayStatics.GetPlayerController` 0) (`self.K2_GetActorLocation`) false)))
  (return (and (> _x_2 (- 0.0 _offset_2)) (> _y_2 (- 100.0 _offset_2)) (< _x_2 (+ _x _offset)) (< _y_2 (+ _y _offset)))))

(fn `Set outline`
  (params (Outlined :type Boolean))
  (`parent.Set outline` (and Outlined (`self.Could be aimed global`))))

(fn `UserConstructionScript`
  (`parent.UserConstructionScript`)
  (`SceneComponent.SetVisibility` (`self.Field`) (`self.Show range sphere`) false)
  (`SphereComponent.SetSphereRadius` (`self.Field`) (/ (`self.View radius`) 13.34) true))