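; Enemy machine gunner character whose child-actor Gun turns independently of the body to aim.
; AimOnAngle interpolates the gun toward the requested rotation at BodyRotationSpeed and returns its resulting world rotation.
; When GunLocked, yaw is clamped to AngleLock either side of the actor's forward using a signed dot-product angle; a zero target pitch keeps the current pitch.
; Die detaches GunLegs and Gun in place before running the parent death logic.
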(event `self.ReceiveBeginPlay`
  (`parent.ReceiveBeginPlay`))

(fn `Aim on angle`
  (params (Angle :type "Rotator Structure"))
  (returns (`Current aim angle` :type "Rotator Structure"))
  (`self.Rotate gun on angle` Angle)
  (return (`SceneComponent.K2_GetComponentRotation` (`Actor.RootComponent` (`ChildActorComponent.ChildActor` (`self.Gun`))))))

(fn `Die`
  (params (causer :type "Actor Object Reference") (`On start` :type Boolean) (`Death impulse` :type "Vector Structure") (`Hit location` :type "Vector Structure"))
  (`SceneComponent.K2_DetachFromComponent` (`self.Gun Legs`) "KeepWorld" "KeepWorld" "KeepWorld" true)
  (`SceneComponent.K2_DetachFromComponent` (`self.Gun`) "KeepWorld" "KeepWorld" "KeepWorld" true)
  (`parent.Die` causer false `Death impulse` `Hit location`))

(fn `Rotate gun on angle`
  (params (Rotation :type "Rotator Structure"))
  (bind _pitch (.pitch Rotation))
  (bind _returnvalue (`KismetMathLibrary.Normal` (`KismetMathLibrary.GetForwardVector` Rotation)))
  (bind _returnvalue_2 (`KismetMathLibrary.DegAcos` (`KismetMathLibrary.Dot_VectorVector` (`KismetMathLibrary.Normal` (`self.GetActorForwardVector`)) _returnvalue)))
  (bind _returnvalue_3 (`SceneComponent.K2_GetComponentRotation` (`Actor.RootComponent` (`ChildActorComponent.ChildActor` (`self.Gun`)))))
  (bind _returnvalue_4 (select `bool` (< (`KismetMathLibrary.Dot_VectorVector` (`KismetMathLibrary.Normal` (`self.GetActorRightVector`)) _returnvalue) 0.0) :`false` _returnvalue_2 :`true` (* _returnvalue_2 -1.0)))
  (set `SceneComponent.bAbsoluteRotation` true (`self.Gun`))
  (`SceneComponent.K2_SetWorldRotation` (`Actor.RootComponent` (`ChildActorComponent.ChildActor` (`self.Gun`))) (`KismetMathLibrary.RInterpTo` _returnvalue_3 (`KismetMathLibrary.MakeRotator` (.roll _returnvalue_3) (`KismetMathLibrary.SelectFloat` _pitch (.pitch _returnvalue_3) (!= _pitch 0.0)) (select `bool` (and (`self.Gun Locked`) (> (`KismetMathLibrary.Abs` _returnvalue_4) (`self.Angle lock`))) :`false` (.yaw Rotation) :`true` (+ (.yaw (`self.K2_GetActorRotation`)) (* (`self.Angle lock`) (`KismetMathLibrary.SignOfFloat` _returnvalue_4))) :!type "Float (single-precision)")) (`GameplayStatics.GetWorldDeltaSeconds`) (`self.Body rotation speed`)) false false))

(fn `UserConstructionScript`
  (`parent.UserConstructionScript`))