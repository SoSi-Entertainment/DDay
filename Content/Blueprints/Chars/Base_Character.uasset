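; Base character class that handles health, death and a child-actor gun.
; BeginPlay scales Health by a coefficient; AnyDamage debug-prints through DDay_Instance and subtracts Health until Die hides the gun and calls CallDeath.
; Aiming sets the gun's absolute world yaw, clamped to AngleLock around the actor's facing when GunLocked, using signed dot-product angles.
; Shoot and the endpoint and snipe-point queries forward to the Gun actor, with firing blocked once Dead.
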(event `self.ReceiveBeginPlay`
  (`self.Apply hp coef` (`self.start hp coef`)))

(event `self.ReceiveAnyDamage`
  (params (Damage :type "Float (single-precision)") (DamageType :type "DamageType Object Reference") (InstigatedBy :type "Controller Object Reference") (DamageCauser :type "Actor Object Reference"))
  (bind _asdday_instance (cast `/Game/Blueprints/System/DDay_Instance` (`GameplayStatics.GetGameInstance`)))
  (`/Game/Blueprints/System/DDay_Instance.Debug Print` _asdday_instance (`KismetStringLibrary.Conv_DoubleToString` Damage) (struct :`G` 0.658824 :`B` 1.0 :`A` 1.0) 2.0)
  (if (not (`self.Dead`))
    (bind _output_get (set `self.Health` (- (`self.Health`) Damage)))
    (if (<= _output_get 0.0)
      (`self.Die`))))

(fn `Apply hp coef`
  (params (coef :type "Float (double-precision)"))
  (set `self.Health` (* coef (`self.Health`))))

(fn `Die`
  (set `self.Dead` true)
  (`SceneComponent.SetVisibility` (`self.Gun`) false false)
  (`self.Death` self))

(fn `Endpoint Location`
  (returns (Location :type "Vector Structure"))
  (return (`/Game/Blueprints/Arms/Gun.Endpoint Location` (cast `/Game/Blueprints/Arms/Gun` (`ChildActorComponent.ChildActor` (`self.Gun`)) :!pure true))))

(fn `Set gun angle`
  (params (Rotaion :type "Rotator Structure"))
  (returns (Rotation :type "Rotator Structure"))
  (bind _returnvalue (`KismetMathLibrary.Normal` (`KismetMathLibrary.GetForwardVector` Rotaion)))
  (bind _returnvalue_2 (`KismetMathLibrary.DegAcos` (`KismetMathLibrary.Dot_VectorVector` (`KismetMathLibrary.Normal` (`self.GetActorForwardVector`)) _returnvalue)))
  (bind _returnvalue_3 (select `bool` (< (`KismetMathLibrary.Dot_VectorVector` (`KismetMathLibrary.Normal` (`self.GetActorRightVector`)) _returnvalue) 0.0) :`false` _returnvalue_2 :`true` (* _returnvalue_2 -1.0)))
  (bind _returnvalue_4 (`KismetMathLibrary.MakeRotator` (.roll (`SceneComponent.K2_GetComponentRotation` (`Actor.RootComponent` (`ChildActorComponent.ChildActor` (`self.Gun`))))) (.pitch (`SceneComponent.K2_GetComponentRotation` (`Actor.RootComponent` (`ChildActorComponent.ChildActor` (`self.Gun`))))) (select `bool` (and (`self.Gun Locked`) (> (`KismetMathLibrary.Abs` _returnvalue_3) (`self.Angle lock`))) :`false` (.yaw Rotaion) :`true` (+ (.yaw (`self.K2_GetActorRotation`)) (* (`self.Angle lock`) (`KismetMathLibrary.SignOfFloat` _returnvalue_3))) :!type "Float (single-precision)")))
  (set `SceneComponent.bAbsoluteRotation` true (`self.Gun`))
  (`SceneComponent.K2_SetWorldRotation` (`Actor.RootComponent` (`ChildActorComponent.ChildActor` (`self.Gun`))) _returnvalue_4 false false)
  (return _returnvalue_4))

(fn `Set gun forward`
  (bind _gun (`self.Gun`))
  (if (`SceneComponent.bAbsoluteRotation` _gun)
    (set `SceneComponent.bAbsoluteRotation` false _gun)
    (`SceneComponent.K2_SetRelativeRotation` :`self` _gun)))

(fn `Shoot`
  (params (Target :type "Vector Structure"))
  (returns (Done :type Boolean))
  (if (`self.Dead`)
    (return false)
    (else
      (bind _done (`/Game/Blueprints/Arms/Gun.Fire` (cast `/Game/Blueprints/Arms/Gun` (`ChildActorComponent.ChildActor` (`self.Gun`)) :!pure true) Target (`self.Generate recoil`)))
      (return _done))))

(fn `SnipePoint Location`
  (returns (location :type "Vector Structure"))
  (bind _location (`/Game/Blueprints/Arms/Gun.SnipePoint Location` (cast `/Game/Blueprints/Arms/Gun` (`ChildActorComponent.ChildActor` (`self.Gun`)) :!pure true)))
  (return _location))

(fn `UserConstructionScript`)