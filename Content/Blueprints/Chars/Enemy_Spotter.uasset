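; Enemy spotter (radioman) character that calls in artillery through its radio device instead of firing a gun.
; GunShoot is gated by CanCallAttack, which it clears before telling the Radio_Device to call an Artillery attack; nothing here re-arms the flag.
; The call also triggers the radioman montage and activates lightning and speak effects.
; ClearMarkers runs the parent logic, then hides both effects.
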(event `Play call artellery anim`
  (`|PlayMontage` (`self.Mesh`) "/Game/3D/Enemy/enemy/Radioman/Radioman_ready_Anim_Montage.Radioman_ready_Anim_Montage"))

(fn `Clear markers`
  (`parent.Clear markers`)
  (`SceneComponent.SetVisibility` (`self.NS_SpotterRadiomanAttack_Speak`) false false)
  (`SceneComponent.SetVisibility` (`self.NS_SpotterRadiomanAttack_Lightning`) false false))

(fn `Gun Shoot`
  (params (`shot info` :type "/Game/Blueprints/recording/Shot_Info Object Reference") (`100%hit` :type Boolean) (`Target location` :type "Vector Structure") (`Add owner speed` :type Boolean) (`Hit Targets` :type "Array of /Game/Blueprints/System/Interfaces/Aimable Interface (by ref)"))
  (returns (Done :type Boolean))
  (if (`self.can call attack`)
    (set `self.can call attack` false)
    (bind _asradio_device (cast `/Game/Blueprints/Arms/Devices/Radio_Device` (`self.Get Device`)))
    (`/Game/Blueprints/Arms/Devices/Radio_Device.call for attack` _asradio_device (`self.Artillery`))
    (`self.Play call artellery anim`)
    (`ActorComponent.Activate` (`self.NS_SpotterRadiomanAttack_Lightning`) true)
    (`ActorComponent.Activate` (`self.NS_SpotterRadiomanAttack_Speak`) true)))

(fn `UserConstructionScript`
  (`parent.UserConstructionScript`))