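; Grenadier enemy character that replaces the inherited gun shot with a throw aimed at a target character.
; The Gun Shoot function casts its current device to Throwble_Device, calls ThrowToCharacter on the first hit target and returns the result.
; Shot info, target location and the other shot inputs go unused, while BeginPlay and the construction script only call the parent.
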(event `self.ReceiveBeginPlay`
  (`parent.ReceiveBeginPlay`))

(fn `Gun Shoot`
  (params (`shot info` :type "/Game/Blueprints/recording/Shot_Info Object Reference") (`100%hit` :type Boolean) (`Target location` :type "Vector Structure") (`Add owner speed` :type Boolean) (`Hit Targets` :type "Array of /Game/Blueprints/System/Interfaces/Aimable Interface (by ref)"))
  (returns (Done :type Boolean))
  (bind _asthrowble_device (cast `/Game/Blueprints/Arms/Devices/Throwble_Device` (`self.Get Device`)))
  (bind _done (`/Game/Blueprints/Arms/Devices/Throwble_Device.Throw to character` _asthrowble_device (`|GetArrayItem` `Hit Targets`)))
  (return _done))

(fn `UserConstructionScript`
  (`parent.UserConstructionScript`))