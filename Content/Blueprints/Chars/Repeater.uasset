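; Repeater is a character Blueprint that mostly defers to its parent class for setup, shooting and death.
; Any damage lowers Health, floored at zero, and refreshes the health texture.
; Body rotation sets the whole actor's yaw to the given angle.
; Shoot returns the parent's result, leaving a debug shot counter with on-screen print disconnected and unreachable.
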(event `self.ReceiveBeginPlay`
  (`parent.ReceiveBeginPlay`))

(event `self.ReceiveAnyDamage`
  (params (Damage :type "Float (single-precision)") (DamageType :type "DamageType Object Reference") (InstigatedBy :type "Controller Object Reference") (DamageCauser :type "Actor Object Reference"))
  (bind _returnvalue (- (`self.Health`) Damage))
  (set `self.Health` (select `bool` (< _returnvalue 0.0) :`false` _returnvalue))
  (`self.Update Health texture`))

(fn `Die`
  (params (causer :type "Actor Object Reference"))
  (`parent.Die` causer))

(fn `Rotate body_0`
  (params (`Body angle` :type "Float (double-precision)"))
  (`self.K2_SetActorRotation` (`KismetMathLibrary.MakeRotator` 0.0 0.0 `Body angle`)))

(fn `Shoot`
  (params (Target :type "Vector Structure") (`shot info` :type "/Game/Blueprints/recording/Shot_Info Object Reference"))
  (returns (Done :type Boolean))
  (bind _done (`parent.Shoot` Target `shot info`))
  (return _done))

(fn `UserConstructionScript`
  (`parent.UserConstructionScript`))