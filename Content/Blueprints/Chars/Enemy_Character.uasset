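; Enemy character for a D-Day game, extending a parent character with notice and attack ranges, a patrol path and a kill bounty.
; A NoticeField sphere is sized from ViewRadius, with debug visibility driven by ShowRangeSphere and game settings, which can also disable enemy shooting.
; Point damage from player AI controllers notifies the game mode, and death pays Price when the causer's owner is a Main_Character or Repeater.
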(event `self.ReceiveBeginPlay`
  (`parent.ReceiveBeginPlay`)
  (`SceneComponent.SetHiddenInGame` (`self.Notice Field`) (not (`.Visiblezones_11_B9DDDC4740327F135A98A59E294A1857` (break `/Game/Data/structs/Dev_Settings` (`/Game/Blueprints/System/DDay_Instance.Game Settings` (cast `/Game/Blueprints/System/DDay_Instance` (`GameplayStatics.GetGameInstance`) :!pure true))))) false))

(event `self.ReceiveAnyDamage`
  (params (Damage :type "Float (single-precision)") (DamageType :type "DamageType Object Reference") (InstigatedBy :type "Controller Object Reference") (DamageCauser :type "Actor Object Reference"))
  (`parent.ReceiveAnyDamage` Damage DamageType InstigatedBy DamageCauser))

(event `self.ReceivePointDamage`
  (params (Damage :type "Float (single-precision)") (DamageType :type "DamageType Object Reference") (HitLocation :type "Vector Structure") (HitNormal :type "Vector Structure") (HitComponent :type "PrimitiveComponent Object Reference") (BoneName :type Name) (ShotFromDirection :type "Vector Structure") (InstigatedBy :type "Controller Object Reference") (DamageCauser :type "Actor Object Reference") (HitInfo :type "HitResult Structure (by ref)"))
  (`parent.ReceivePointDamage` Damage DamageType HitLocation HitNormal HitComponent BoneName ShotFromDirection InstigatedBy DamageCauser HitInfo)
  (cast `/Game/Blueprints/Controllers/Player_AI_Controller` InstigatedBy)
  (`/Game/Blueprints/System/DDay_GameMode.Hit Event` (cast `/Game/Blueprints/System/DDay_GameMode` (`GameplayStatics.GetGameMode`) :!pure true) self))

(fn `Clear`
  (set `self.Dead on start` true)
  (`self.Die` null)
  (return))

(fn `Die`
  (params (causer :type "Actor Object Reference") (`Death impulse` :type "Vector Structure") (`Hit location` :type "Vector Structure"))
  (bind _returnvalue (`self.GetOwner` causer))
  (`/Engine/EditorBlueprintResources/StandardMacros.IsValid` causer
    (:`Is Valid`
      (cast `/Game/Blueprints/Chars/Players/Main_Character` _returnvalue
        (:`then`
          (`/Game/Blueprints/System/DDay_GameMode.Add enemy money` (cast `/Game/Blueprints/System/DDay_GameMode` (`GameplayStatics.GetGameMode`) :!pure true) (`self.Price`) :!label _label))
        (:`CastFailed`
          (cast `/Game/Blueprints/Chars/Clones/Repeater` _returnvalue
            (:`then`
              (goto _label))
            (:`CastFailed`
              _)))))
    (:`Is Not Valid`
      _))
  (`parent.Die` causer `Death impulse` `Hit location`))

(fn `Get notice radius`
  (returns (`Has collision sphere` :type Boolean) (`Sphere radius` :type "Float (double-precision)"))
  (return true (`SphereComponent.SphereRadius` (`self.Notice Field`))))

(fn `Get path`
  (returns (Path :type "/Game/Blueprints/Navigation/Path_holder Object Reference"))
  (return (`self.Path_holder`)))

(fn `Get shooting radius`
  (returns (Radius :type "Float (double-precision)"))
  (return (`self.Attack radius`)))

(fn `Gun Shoot`
  (params (`shot info` :type "/Game/Blueprints/recording/Shot_Info Object Reference") (`100%hit` :type Boolean) (`Target location` :type "Vector Structure") (`Add owner speed` :type Boolean) (`Hit Targets` :type "Array of /Game/Blueprints/Chars/Abstract/Base_Character Object Reference (by ref)"))
  (returns (Done :type Boolean))
  (if (`.Enemiesdontshoot_16_D156372D4F9CFC442C3B258E6129A7BD` (break `/Game/Data/structs/Dev_Settings` (`/Game/Blueprints/System/DDay_Instance.Game Settings` (cast `/Game/Blueprints/System/DDay_Instance` (`GameplayStatics.GetGameInstance`) :!pure true))))
    (return false)
    (else
      (bind _done (`parent.Gun Shoot` `shot info` `100%hit` `Target location` false `Hit Targets`))
      (return _done))))

(fn `UserConstructionScript`
  (`parent.UserConstructionScript`)
  (`SceneComponent.SetVisibility` (`self.Notice Field`) (`self.Show range sphere`) false)
  (`SphereComponent.SetSphereRadius` (`self.Notice Field`) (/ (`self.View radius`) 13.34) true))