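; Ally NPC Devicer is a child ally character Blueprint for a unit that carries a device.
; Its SetUnitStats override runs the parent logic, then passes the resulting stats to the device to initialize its settings.
; GetRange reads attack range from the balanced stats for its unit type and variation.
; SetGunDown is empty, and the event graph holds only disabled placeholder events.
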(fn `Get range`
  (returns (range :type "Float (double-precision)"))
  (bind _stats (`/Game/Blueprints/System/Funtions/FunctionLibrary.Get Balanced stats` (`self.Unit type`) (`self.Unit Variation`)))
  (return (`KismetMathLibrary.Conv_IntToDouble` (`.Attackrange_49_DB0D27BC40A3BAD165D3429F8E8D3ED8` (break `/Game/Data/structs/Balance_State` _stats)))))

(fn `Set gun down`
  (params (down :type Boolean)))

(fn `Set unit stats`
  (returns (Stats :type "/Game/Data/structs/Balance_State Structure"))
  (bind _stats (`parent.Set unit stats`))
  (`/Game/Blueprints/Arms/Devices/Base_Device.Init settings` (`self.Get Device`) _stats)
  (return _stats))

(fn `UserConstructionScript`
  (`parent.UserConstructionScript`))