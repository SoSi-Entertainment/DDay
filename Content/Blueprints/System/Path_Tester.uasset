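; Editor path-authoring actor that previews a route of points with debug lines, linking each point to the platform under it.
; Its construction script, skipped when a game state exists, offsets newly added points from the previous one and converts points to world space.
; It persists point count and root location in a data asset keyed by object path, detecting edits and shifting points opposite to root movement.
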(fn `Add new point offset`
  (locals (`New point offset` :type "Vector Structure" :default (0.0 100.0 0.0)))
  (bind _points (`self.points`))
  (bind _returnvalue (`KismetArrayLibrary.Array_LastIndex` _points))
  (`KismetArrayLibrary.Array_Set` _points _returnvalue (+ (`|GetArrayItem` _points (- _returnvalue 1)) (`local.New point offset`))))

(fn `Check for new point`
  (`/Engine/EditorBlueprintResources/StandardMacros.CompareInt` (`KismetArrayLibrary.Array_Length` (`self.points`)) (`.Prevpointscount_7_8CF67DD043849308A6852F8507B87860` (break `/Game/Data/structs/Spawner_Data` (`BlueprintMapLibrary.Map_Find` (`/Game/Blueprints/System/EditorAsset.spawners info` (`self.data asset`)) (`/Game/Blueprints/System/FunctionLibrary.Get object path string` self))))
    (:`>`
      (`self.Add new point offset`))))

(fn `Check for root move`
  (bind _returnvalue (- (`.Prevrootlocation_6_665D68604F47D84A51D4B299CE1012D2` (break `/Game/Data/structs/Spawner_Data` (`BlueprintMapLibrary.Map_Find` (`/Game/Blueprints/System/EditorAsset.spawners info` (`self.data asset`)) (`/Game/Blueprints/System/FunctionLibrary.Get object path string` self)))) (`self.K2_GetActorLocation`)))
  (`/Engine/EditorBlueprintResources/StandardMacros.CompareFloat` (`KismetMathLibrary.VSize` _returnvalue)
    (:`>`
      (set `self.delta` _returnvalue))))

(fn `Draw`
  (bind _world_points (`self.world points`))
  (for (_array_element _array_index) _world_points
    (bind (_surface_location _platform) (`/Game/Blueprints/System/FunctionLibrary.Get platform under` _array_element))
    (`KismetSystemLibrary.DrawDebugLine` _array_element (`self.K2_GetActorLocation` _platform) (struct :`R` 1.0 :`B` 0.900965 :`A` 1.0) 90.0 5.0)
    (if (not (== _array_index (`KismetArrayLibrary.Array_LastIndex` _world_points)))
      (`KismetSystemLibrary.DrawDebugLine` _array_element (`|GetArrayItem` _world_points (+ _array_index 1)) (struct :`R` 1.0 :`B` 0.900965 :`A` 1.0) 90.0 5.0))))

(fn `Hide path`
  (`KismetSystemLibrary.FlushPersistentDebugLines`))

(fn `Is Inited`
  (returns (`Is inited` :type Boolean))
  (return (`.ReturnValue` (`BlueprintMapLibrary.Map_Find` (`/Game/Blueprints/System/EditorAsset.spawners info` (`self.data asset`)) (`/Game/Blueprints/System/FunctionLibrary.Get object path string` self)))))

(fn `main`
  (`KismetSystemLibrary.FlushPersistentDebugLines`)
  (if (`self.Is Inited`)
    (`self.Check for new point`)
    (`self.Check for root move`)
    (`self.Save data to asset`)
    (`self.Setup Points`)
    (`self.Draw`)
    (else
      (`self.Save data to asset`))))

(fn `Save data to asset`
  (`BlueprintMapLibrary.Map_Add` (`/Game/Blueprints/System/EditorAsset.spawners info` (`self.data asset`)) (`/Game/Blueprints/System/FunctionLibrary.Get object path string` self) (make `/Game/Data/structs/Spawner_Data` (`KismetArrayLibrary.Array_Length` (`self.points`)) (`self.K2_GetActorLocation`))))

(fn `Setup Points`
  (bind _points (`self.points`))
  (for (_array_element _array_index) _points
    (`KismetArrayLibrary.Array_Set` _points _array_index (+ (`self.delta`) _array_element))
    (`KismetArrayLibrary.Array_Set` (`self.world points`) _array_index (`KismetMathLibrary.TransformLocation` (`self.GetTransform`) _array_element) true)))

(fn `Show path`
  (`self.main`))

(fn `UserConstructionScript`
  (`/Engine/EditorBlueprintResources/StandardMacros.IsValid` (`GameplayStatics.GetGameState`)
    (:`Is Not Valid`
      (`self.main`))))