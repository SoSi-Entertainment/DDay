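; Web module that connects the game to VK Play for player profiles and achievements when the target platform is Vk.
; Init takes the user ID from the sz_pers_id command-line option, or a dev-settings override, then requests the profile.
; VaRest calls are signed with MD5 of parameters plus the game secret.
; Nick and avatar are stored, with Responced broadcast after the avatar downloads; achievement responses are only printed.
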(event `Get VK User Info`
  (params (uid :type String))
  (bind _returnvalue (`MD5Calculator.CalculateMD5` (`KismetStringLibrary.Concat_StrStr` "uid=" uid (`self.game secret`))))
  (`VaRestSubsystem.CallURL` (subsystem `VaRestSubsystem`) (`KismetStringLibrary.Concat_StrStr` (`KismetStringLibrary.Concat_StrStr` "https://vkplay.ru/app/" (`self.game id`) "/user/profile") "?uid=" uid "&sign=" _returnvalue) "GET" "x_www_form_urlencoded_url" null (delegate `CustomEvent`)))

(event `CustomEvent`
  (params (Request :type "VaRestRequestJSON Object Reference"))
  (bind _returnvalue (`VaRestRequestJSON.GetResponseContentAsString` Request true))
  (bind _outjsonobject (`JsonBlueprintFunctionLibrary.FromString` _returnvalue))
  (bind _outvalue (`|GetJsonField` _outjsonobject "nick"))
  (set `self.nick` _outvalue)
  (bind _outvalue_2 (`|GetJsonField` _outjsonobject "avatar"))
  (bind _texture (`AsyncTaskDownloadImage.DownloadImage` _outvalue_2)
    (:`OnSuccess`
      (set `self.avatar` _texture)
      (set `self.user data received` true)
      (`self.responced`))))

(event `Add vk achievement`
  (params (`achivement vk id` :type Integer))
  (bind _returnvalue (`KismetStringLibrary.Conv_IntToString` `achivement vk id`))
  (bind _returnvalue_2 (subsystem `VaRestSubsystem`))
  (bind _returnvalue_3 (`MD5Calculator.CalculateMD5` (`KismetStringLibrary.Concat_StrStr` "ach_id=" _returnvalue "uid=" (`self.uid`) (`self.game secret`))))
  (bind _returnvalue_4 (`VaRestSubsystem.DecodeJsonObject` _returnvalue_2 (`KismetStringLibrary.Concat_StrStr` "{" "\"ach_id\":\"" _returnvalue "\",\"uid\":\"" (`self.uid`) "\",\"sign\":\"" _returnvalue_3 "\"}")))
  (`VaRestSubsystem.CallURL` _returnvalue_2 (`KismetStringLibrary.Concat_StrStr` "https://vkplay.ru/app/" (`self.game id`) "/achievement/set") "POST" "x_www_form_urlencoded_body" _returnvalue_4 (delegate `achivement responce`)))

(event `achivement responce`
  (params (Request :type "VaRestRequestJSON Object Reference"))
  (bind _returnvalue (`VaRestRequestJSON.GetResponseContentAsString` Request false))
  (`KismetSystemLibrary.PrintString` _returnvalue true true (struct :`G` 0.66 :`B` 1.0 :`A` 1.0) 10.0))

(fn `Add Achievement`
  (params (Achievement :type "/Game/Achievements/_System/Achievement_Data_Asset Object Reference"))
  (switch `/Game/Data/enums/Target_platform` (`self.Platform`)
    (:`NewEnumerator1`
      (`KismetSystemLibrary.PrintString` (`KismetSystemLibrary.GetDisplayName` Achievement) true true (struct :`R` 1.0 :`G` 0.628237 :`A` 1.0) 10.0)
      (`self.Add vk achievement` (`/Game/Achievements/_System/Achievement_Data_Asset.vk id` Achievement)))))

(fn `Get Cmd Option Value`
  (params (`Option name` :type String))
  (returns (`Option value` :type String))
  (bind _returnvalue (`KismetSystemLibrary.GetCommandLine`))
  (for _array_element (`KismetStringLibrary.ParseIntoArray` _returnvalue)
    (if (>= (`KismetStringLibrary.FindSubstring` _array_element `Option name`) 0)
      (return (`|GetArrayItem` (`KismetStringLibrary.ParseIntoArray` _array_element "=") 1)))))

(fn `Init`
  (bind (_devmode _debuggraphics _titanmode _fastrun _cameramovement _visiblezones _enemiesdontshoot _1shot1kill _cutscenesoff _moneymoney _invisibleinterface _alllevelsunlocked _loadstatsfromfile _loadstatsoutput _playopening _targetplatform _emeluateuid) (break `/Game/Data/structs/Dev_Settings` (`/Game/Blueprints/System/DDay_Instance.Dev Settings` (`self.instance`))))
  (bind _output_get (set `self.Platform` _targetplatform))
  (switch `/Game/Data/enums/Target_platform` _output_get
    (:`NewEnumerator1`
      (bind _option_value (`self.Get Cmd Option Value` "sz_pers_id"))
      (bind _output_get_2 (set `self.uid` (select `bool` (`KismetStringLibrary.IsEmpty` _emeluateuid) :`false` _emeluateuid :`true` _option_value)))
      (`self.Get VK User Info` _output_get_2))))