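; Blueprint function library of shared helpers for units, aiming, platforms and object references.
; It converts direction enums and surface normals to vectors and rotations, and maps each unit class variant to its type from the Units_Links table.
; Shot leading projects the target along its movement at max walk speed over the shell's flight time.
; Other helpers line-trace down for the platform underneath and convert objects to and from path strings.
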(fn `Calculate Preemption`
  (params (Target :type "/Game/Blueprints/Chars/Abstract/Base_Character Object Reference") (Shooter :type "/Game/Blueprints/Chars/Abstract/Base_Character Object Reference"))
  (returns (`Target expected location` :type "Vector Structure"))
  (bind _returnvalue (`Actor.K2_GetActorLocation` Target))
  (bind _charactermovement (`Character.CharacterMovement` Target))
  (return (+ (* (* (`KismetMathLibrary.Normal` (`MovementComponent.Velocity` _charactermovement)) (`CharacterMovementComponent.MaxWalkSpeed` _charactermovement)) (/ (`KismetMathLibrary.Vector_Distance` _returnvalue (`/Game/Blueprints/Chars/Abstract/Base_Character.SnipePoint Location` Shooter)) (`/Game/Blueprints/Chars/Abstract/Base_Character.Get shell speed` Shooter))) _returnvalue)))

(fn `Find object by string`
  (params (`Object path` :type String))
  (returns (Object :type "Object Object Reference"))
  (return (`|ConvertAsset` (`KismetSystemLibrary.Conv_SoftObjPathToSoftObjRef` (`KismetSystemLibrary.MakeSoftClassPath` `Object path`)))))

(fn `Get object path string`
  (params (Object :type "Object Object Reference"))
  (returns (`Object path` :type String))
  (return (`KismetSystemLibrary.BreakSoftObjectPath` (`KismetSystemLibrary.GetSoftObjectPath` Object))))

(fn `Get platform under`
  (params (Location :type "Vector Structure") (`From sky` :type Boolean))
  (returns (`Surface location` :type "Vector Structure") (Platform :type "/Game/3D/platforms/Default_Platform_bp Object Reference"))
  (locals (`trace types` :type "Array of EObjectTypeQuery Enum"))
  (bind _outhit (`KismetSystemLibrary.LineTraceSingleForObjects` null (+ Location (`KismetMathLibrary.SelectVector` (0.0 0.0 500.0) (0.0 0.0 0.0) `From sky`)) (- Location (0.0 0.0 1000.0)) (`local.trace types`)))
  (bind (_bblockinghit _binitialoverlap _time _distance _location _impactpoint _normal _impactnormal _physmat _hitactor) (`GameplayStatics.BreakHitResult` _outhit))
  (bind _asdefault_platform_bp (cast `/Game/3D/platforms/Default_Platform_bp` _hitactor))
  (return _location _asdefault_platform_bp))

(fn `Make character class type map`
  (returns (`Character Class Type` :type "Map of /Game/Blueprints/Chars/Abstract/Base_Character Class Reference to /Game/Data/enums/Unit_Types Enum"))
  (locals (Table :type "Map of /Game/Blueprints/Chars/Abstract/Base_Character Class Reference to /Game/Data/enums/Unit_Types Enum"))
  (bind _table (`local.Table`))
  (bind _outrownames (`DataTableFunctionLibrary.GetDataTableRowNames` "/Game/Data/Units_Links.Units_Links"))
  (for _array_element _outrownames
    (bind _returnvalue (`|GetDataTableRow` "/Game/Data/Units_Links.Units_Links" _array_element)
      (:`then`
        (bind (_type _enemyunit _playerunit _cloneunit _allyunit) (break `/Game/Data/structs/Units_Link` _returnvalue))
        (`BlueprintMapLibrary.Map_Add` _table _enemyunit _type)
        (`BlueprintMapLibrary.Map_Add` _table _playerunit _type)
        (`BlueprintMapLibrary.Map_Add` _table _cloneunit _type)
        (`BlueprintMapLibrary.Map_Add` _table _allyunit _type))))
  (return (`local.Table`)))

(fn `Normal to Rotation`
  (params (normal :type "Vector Structure (by ref)"))
  (returns (Rotation :type "Rotator Structure"))
  (return (`KismetMathLibrary.MakeRotator` (+ (.roll (`KismetMathLibrary.MakeRotFromZ` normal)) 180.0) 0.0 (.yaw (`KismetMathLibrary.MakeRotFromZ` normal)))))

(fn `Vector from direction`
  (params (Direction :type "/Game/Data/enums/Dirrection Enum" :default "NewEnumerator4"))
  (returns (`Normal vector` :type "Vector Structure"))
  (return (select `/Game/Data/enums/Dirrection` Direction :`NewEnumerator0` (1.0 0.0 0.0) :`NewEnumerator1` (-1.0 0.0 0.0) :`NewEnumerator2` (0.0 1.0 0.0) :`NewEnumerator3` (0.0 -1.0 0.0) :!type "Vector Structure")))