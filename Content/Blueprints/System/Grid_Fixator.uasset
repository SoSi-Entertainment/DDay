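; Grid_Fixator is a component that snaps its owning actor to the grid tile of the platform beneath it.
; Fixate finds the platform under the owner's location, reads its tile's grid coordinates and scales them to world units.
; It then moves the owner to that X and Y without sweeping, keeping its current height.
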(fn `Fixate`
  (bind _returnvalue (`self.GetOwner`))
  (bind _returnvalue_2 (`Actor.K2_GetActorLocation` _returnvalue))
  (bind (_surface_location _platform) (`/Game/Blueprints/System/Funtions/FunctionLibrary.Get platform under` _returnvalue_2))
  (bind (_x _y) (`/Game/3D/platforms/Tile.Get grid location` (`/Game/3D/platforms/Default_Platform_bp.Get tile` _platform)))
  (`Actor.K2_SetActorLocation` _returnvalue (* (`KismetMathLibrary.MakeVector` (`KismetMathLibrary.Conv_IntToDouble` _x) (`KismetMathLibrary.Conv_IntToDouble` _y) (.z _returnvalue_2)) (100.0 100.0 1.0)) false false))