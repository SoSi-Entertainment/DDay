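; Level State blueprint that tracks how long the player has spent on a level, in whole minutes.
; Start and end times are stamped from Now, and GetTimeOnLevel refreshes the end time before measuring, while GetCurrentTimeOnLevel measures against Now without storing it.
; Both subtract timespans built from day-of-month and clock fields, then return hours times 60 plus minutes, dropping whole days and seconds.
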(fn `Get current time on level`
  (returns (Minutes :type Integer))
  (bind (_year _month _day _hour _minute _second _millisecond) (`KismetMathLibrary.BreakDateTime` (`KismetMathLibrary.Now`)))
  (bind (_year_2 _month_2 _day_2 _hour_2 _minute_2 _second_2 _millisecond_2) (`KismetMathLibrary.BreakDateTime` (`self.Start time`)))
  (bind (_days _hours _minutes) (`KismetMathLibrary.BreakTimespan` (- (`KismetMathLibrary.MakeTimespan` _day _hour _minute _second _millisecond) (`KismetMathLibrary.MakeTimespan` _day_2 _hour_2 _minute_2 _second_2 _millisecond_2))))
  (return (+ (* _hours 60) _minutes)))

(fn `Get time on level`
  (returns (minutes :type Integer))
  (bind (_year _month _day _hour _minute _second _millisecond) (`KismetMathLibrary.BreakDateTime` (`self.End time`)))
  (bind (_year_2 _month_2 _day_2 _hour_2 _minute_2 _second_2 _millisecond_2) (`KismetMathLibrary.BreakDateTime` (`self.Start time`)))
  (bind (_days _hours _minutes) (`KismetMathLibrary.BreakTimespan` (- (`KismetMathLibrary.MakeTimespan` _day _hour _minute _second _millisecond) (`KismetMathLibrary.MakeTimespan` _day_2 _hour_2 _minute_2 _second_2 _millisecond_2))))
  (`self.Set end time`)
  (return (+ (* _hours 60) _minutes)))

(fn `Set end time`
  (set `self.End time` (`KismetMathLibrary.Now`)))

(fn `Set start time`
  (set `self.Start time` (`KismetMathLibrary.Now`)))