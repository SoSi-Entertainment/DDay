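; Dialog component that queues timed dialog lines with optional voice audio and end actions, exposing the front entry as the current dialog.
; AddDialog filters lines by Between_Lifes_Sceen money check and level-reload state, then starts timers if the queue was empty.
; Display time follows voice duration, or text length without voice.
; RemoveDialog fires the end action and starts the next line; ClearDialogs cancels timer, queue and sound.
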(fn `Add dialog`
  (params (Dialog :type Text) (type :type "/Game/Data/enums/Dialog_Type Enum" :default "NewEnumerator0") (`End Action` :type "/Game/Blueprints/Logics/Action_Group Object Reference"))
  (bind _foundwidgets (`WidgetBlueprintLibrary.GetAllWidgetsOfClass` "/Game/UI/Widgets/Game/Game_Menus/Between_Lifes_Sceen.Between_Lifes_Sceen_C"))
  (bind _output (`|GetArrayItem` _foundwidgets))
  (`/Engine/EditorBlueprintResources/StandardMacros.IsValid` _output
    (:`Is Valid`
      (if (`/Game/UI/Widgets/Game/Game_Menus/Between_Lifes_Sceen.Is Enough Money` _output "NewEnumerator2")
        (`/Game/UI/Widgets/Game/Game_Menus/Between_Lifes_Sceen.Move buttons down` _output)
        (bind _voice (`self.Find Voice` Dialog :!label _label))
        (if (not (and (`|EnumEquality` type "NewEnumerator1") (`/Game/Blueprints/System/DDay_GameMode.Lvl Reloading started` (cast `/Game/Blueprints/System/DDay_GameMode` (`GameplayStatics.GetGameMode`) :!pure true))))
          (bind _returnvalue (`KismetArrayLibrary.Array_Add` (`self.Dialog queue`) (make `/Game/Data/structs/Dialog_info` Dialog type _voice `End Action`)))
          (`/Engine/EditorBlueprintResources/StandardMacros.CompareInt` _returnvalue
            (:`==`
              (`self.Start Remove Timer`))))))
    (:`Is Not Valid`
      (goto _label))))

(fn `Clear dialogs`
  (bind _current_sound (`self.Current sound`))
  (`KismetSystemLibrary.K2_ClearAndInvalidateTimerHandle` (`self.Current timer`))
  (`KismetArrayLibrary.Array_Clear` (`self.Dialog queue`))
  (`/Engine/EditorBlueprintResources/StandardMacros.IsValid` _current_sound
    (:`Is Valid`
      (`self.SetActive` _current_sound false false))))

(fn `Find Voice`
  (params (`Dialog text` :type Text))
  (returns (Voice :type "SoundWave Object Reference"))
  (bind _returnvalue (`|GetDataTableRow` "/Game/Data/dialogs/Voices_Table.Voices_Table" (`KismetStringLibrary.Conv_StringToName` (`.FilenamePart` (`BlueprintPathsLibrary.Split` (`KismetStringLibrary.Conv_NameToString` (`KismetTextLibrary.StringTableIdAndKeyFromText` `Dialog text`))))))
    (:`then`
      (return null))))

(fn `Get dialog`
  (returns (`Has conternt` :type Boolean) (`Current dialog` :type Text) (Type :type "/Game/Data/enums/Dialog_Type Enum") (Voice :type "SoundWave Object Reference"))
  (bind _dialog_queue (`self.Dialog queue`))
  (bind (_dialog _type _voice) (break `/Game/Data/structs/Dialog_info` (`|GetArrayItem` _dialog_queue)))
  (`/Engine/EditorBlueprintResources/StandardMacros.CompareInt` (`KismetArrayLibrary.Array_Length` _dialog_queue)
    (:`>`
      (return true _dialog _type _voice))
    (:`==`
      (return false "" "NewEnumerator0" null))))

(fn `Get dialog time`
  (returns (Time :type "Float (double-precision)"))
  (bind (_has_conternt _current_dialog _type _voice) (`self.Get dialog`))
  (`/Engine/EditorBlueprintResources/StandardMacros.IsValid` _voice
    (:`Is Valid`
      (return (+ (`self.Text delay after voice`) (`SoundBase.Duration` _voice))))
    (:`Is Not Valid`
      (return (+ (`self.Get Text time` _current_dialog) (`self.Take attention time`))))))

(fn `Get Text time`
  (params (Dialog :type Text))
  (returns (Time :type "Float (double-precision)"))
  (return (* (`KismetMathLibrary.Conv_IntToDouble` (`KismetStringLibrary.Len` (`KismetTextLibrary.Conv_TextToString` Dialog))) (`self.Seconds per char`))))

(fn `Play Voice`
  (bind (_has_conternt _current_dialog _type _voice) (`self.Get dialog`))
  (`/Engine/EditorBlueprintResources/StandardMacros.IsValid` _voice
    (:`Is Valid`
      (bind _returnvalue (`GameplayStatics.SpawnSound2D` _voice 1.0 1.0 0.0 null))
      (set `self.Current sound` _returnvalue))))

(fn `Remove dialog`
  (bind _dialog_queue (`self.Dialog queue`))
  (bind (_dialog _type _voice _endaction) (break `/Game/Data/structs/Dialog_info` (`|GetArrayItem` _dialog_queue)))
  (set `self.Current sound` null)
  (`/Engine/EditorBlueprintResources/StandardMacros.IsValid` _endaction
    (:`Is Valid`
      (`/Game/Blueprints/Logics/Components/Action_Starter.Start` (`/Game/Blueprints/Logics/Components/Actioner.Action_Starter` _endaction) "None"))
    (:`Is Not Valid`
      _))
  (`KismetArrayLibrary.Array_Remove` _dialog_queue)
  (`/Engine/EditorBlueprintResources/StandardMacros.CompareInt` (`KismetArrayLibrary.Array_Length` _dialog_queue)
    (:`>`
      (`self.Start Remove Timer`))))

(fn `Start Remove Timer`
  (`GameplayStatics.PlaySound2D` (`self.Dialog start Sound`) 1.0 1.0 0.0 null null)
  (`KismetSystemLibrary.K2_SetTimerDelegate` (`|CreateDelegate` :!event `Play Voice`) 0.1)
  (bind _returnvalue (`KismetSystemLibrary.K2_SetTimerDelegate` (`|CreateDelegate` :!event `Remove dialog`) (`self.Get dialog time`)))
  (set `self.Current timer` _returnvalue))