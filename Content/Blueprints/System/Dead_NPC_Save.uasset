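; Save container for an NPC, going by the asset name, with a function that records the state of its path.
; SavePath copies the looped and stop-to-shoot flags from the given path.
; Unless a non-looped path has reached its end, it also stores the iterator and appends each point as a path name string rather than a reference.
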(fn `Save path`
  (params (Path :type "/Game/Blueprints/Navigation/Path_holder Object Reference"))
  (bind _looped (`/Game/Blueprints/Navigation/Path_holder.Looped` Path))
  (bind _iterator (`/Game/Blueprints/Navigation/Path_holder.iterator` Path))
  (bind _points (`/Game/Blueprints/Navigation/Path_holder.Points` Path))
  (set `self.Path looped` _looped)
  (set `self.Path stop to shoot` (`/Game/Blueprints/Navigation/Path_holder.Stop to shoot` Path))
  (if (not (and (not _looped) (== _iterator (`KismetArrayLibrary.Array_Length` _points))))
    (set `self.Path iterator` _iterator)
    (for _array_element _points
      (`KismetArrayLibrary.Array_Add` (`self.Path points`) (`KismetSystemLibrary.GetPathName` _array_element)))))