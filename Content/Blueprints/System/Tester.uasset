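; Tester is an editor-time debug actor that visualizes a point path and the platform under each point.
; Its Construction Script runs only without a valid GameState, flushing persistent debug lines and saving the point count to a data asset.
; MoveNewToLast places the last point at a fixed offset from its predecessor.
; Show converts points to world space, drawing lines between neighbors and to each platform found by GetPlatformUnder.
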(fn `UserConstructionScript`
  (bind _points (`self.points`))
  (bind _world_points (`self.world points`))
  (bind _returnvalue (`KismetArrayLibrary.Array_LastIndex` _points))
  (`/Engine/EditorBlueprintResources/StandardMacros.IsValid` (`GameplayStatics.GetGameState`)
    (:`Is Not Valid`
      (`KismetSystemLibrary.FlushPersistentDebugLines`)
      (set `/Game/Blueprints/System/EditorAsset.old len` (`KismetArrayLibrary.Array_Length` (`self.points`)) (`self.data asset`))
      (if (`self.Move New to last`)
        (`KismetArrayLibrary.Array_Set` _points _returnvalue (+ (`|GetArrayItem` _points (- _returnvalue 1)) (0.0 100.0 0.0))))
      (if (`self.Show`)
        (for (_array_element _array_index) (`self.points`)
          (`KismetArrayLibrary.Array_Set` (`self.world points`) _array_index (`KismetMathLibrary.TransformLocation` (`self.GetTransform`) _array_element) true))
        (for (_array_element_2 _array_index_2) _world_points
          (bind (_surface_location _platform) (`/Game/Blueprints/System/FunctionLibrary.Get platform under` _array_element_2))
          (`KismetSystemLibrary.DrawDebugLine` _array_element_2 (`self.K2_GetActorLocation` _platform) (struct :`R` 1.0 :`B` 0.900965 :`A` 1.0) 90.0 5.0)
          (if (not (== _array_index_2 (`KismetArrayLibrary.Array_LastIndex` _world_points)))
            (`KismetSystemLibrary.DrawDebugLine` _array_element_2 (`|GetArrayItem` _world_points (+ _array_index_2 1)) (struct :`R` 1.0 :`B` 0.900965 :`A` 1.0) 90.0 5.0)))))))