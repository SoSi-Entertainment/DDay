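; Artillery actor that drops timed shell barrages onto platform tiles.
; Startfiring walks the Targets list with per-entry delays and replays it RepeatCount times, hitting a random TargetField tile when that field is valid, otherwise the listed tile.
; Fire spawns Art_Shell offset from the tile surface by SpawnDistance along the actor's rotated up axis.
; Clear, if ClearAfterCheckpoint is set, blocks later Startfiring calls but does not interrupt a running barrage.
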(event `Start firing`
  (bind _targets (`self.Targets`))
  (bind _target_field (`self.Target Field`))
  (bind (_time _targettile) (break `/Game/Data/structs/Tile_Sequence_Chain` (`|GetArrayItem` _targets (`self.Shell counter`))))
  (if (not (`self.cleared`))
    (`/Engine/EditorBlueprintResources/StandardMacros.CompareInt` (`self.Repeat count`) :!label _label
      (:`>`
        (`/Engine/EditorBlueprintResources/StandardMacros.CompareInt` (`self.Shell counter`) (`KismetArrayLibrary.Array_Length` _targets) :!label _label_2
          (:`==`
            (`/Engine/EditorBlueprintResources/StandardMacros.DecrementInt` (`self.Repeat count`)
              (:`  `
                (set `self.Shell counter` 0)
                (goto _label))))
          (:`<`
            (`KismetSystemLibrary.Delay` _time)
            (`/Engine/EditorBlueprintResources/StandardMacros.IsValid` _target_field
              (:`Is Valid`
                (bind _platforms (`/Game/Blueprints/Logics/Artillery_Field.Get tiles` _target_field))
                (set `self.Target tile` (`/Game/3D/platforms/Default_Platform_bp.Get tile` (cast `/Game/3D/platforms/Default_Platform_bp` (`KismetArrayLibrary.Array_Random` _platforms) :!pure true))))
              (:`Is Not Valid`
                (set `self.Target tile` _targettile)))
            (`self.Fire` (`self.Target tile`))
            (`/Engine/EditorBlueprintResources/StandardMacros.IncrementInt` (`self.Shell counter`)
              (:`  `
                (goto _label_2)))))))))

(event `Fire`
  (params (`Target tile` :type "/Game/3D/platforms/Tile Object Reference"))
  (`/Engine/EditorBlueprintResources/StandardMacros.IsValid` `Target tile`
    (:`Is Valid`
      (bind _location (`/Game/3D/platforms/Tile.get surface location` `Target tile` false))
      (`|SpawnActorFromClass` :`Class` "/Game/Blueprints/Arms/Shells/Art_Shell.Art_Shell_C" :`SpawnTransform` (`KismetMathLibrary.MakeTransform` (+ _location (`KismetMathLibrary.GreaterGreater_VectorRotator` (`KismetMathLibrary.MakeVector` 0.0 0.0 (`self.Spawn distance`)) (`self.K2_GetActorRotation`))) (`KismetMathLibrary.ComposeRotators` (struct :`Yaw` 90.0 :`Roll` 90.0) (`self.K2_GetActorRotation`))) :`CollisionHandlingOverride` "Undefined" :`TransformScaleMethod` "MultiplyWithRoot" :`shot info` null :`shell params` (make `/Game/Data/structs/Shell_params` (`self.Shell speed`) 500.0 2000.0) :`Instigator` null))))

(event `/Game/Blueprints/Chars/Components/Checkpoint_Clearable.Clear`
  (if (`self.Clear after checkpoint`)
    (set `self.cleared` true)))

(fn `UserConstructionScript`)