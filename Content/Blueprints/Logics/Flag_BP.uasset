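; Flag actor that shows which team it belongs to by swapping the material in slot 1 of its Flag component.
; The construction script previews it with fixed British (Ally) or German (Enemy) materials.
; On BeginPlay it takes the team material from the troops instance's FlagStateModule, falling back to the preview materials if that instance is invalid.
; Both and None teams have no material assigned.
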(event `self.ReceiveBeginPlay`
  (`self.set flag material` (`self.Team`)))

(fn `set flag in editor`
  (params (team :type "/Game/Data/enums/Team Enum" :default "NewEnumerator0"))
  (`PrimitiveComponent.SetMaterial` (`self.Flag`) 1 (select `/Game/Data/enums/Team` team :`NewEnumerator0` "/Game/3D/flag/txtr/britain/mat_britain.mat_britain" :`NewEnumerator1` "/Game/3D/flag/txtr/german/mat_german.mat_german" :!type "MaterialInterface Object Reference")))

(fn `set flag material`
  (params (team :type "/Game/Data/enums/Team Enum" :default "NewEnumerator0"))
  (bind _troops_instance (`/Game/Blueprints/System/Funtions/FunctionLibrary.Get Instanse Troops`))
  (bind _flag_state_module (`/Game/Blueprints/System/DDay_Instance.flag state module` _troops_instance))
  (`/Engine/EditorBlueprintResources/StandardMacros.IsValid` _troops_instance
    (:`Is Valid`
      (`PrimitiveComponent.SetMaterial` (`self.Flag`) 1 (select `/Game/Data/enums/Team` team :`NewEnumerator0` (`/Game/Blueprints/System/Instance_Modules/Flags/Flag_State_Module.ally flag material` _flag_state_module) :`NewEnumerator1` (`/Game/Blueprints/System/Instance_Modules/Flags/Flag_State_Module.enemy flag material` _flag_state_module) :!type "MaterialInterface Object Reference")))
    (:`Is Not Valid`
      (`self.set flag in editor` team))))

(fn `UserConstructionScript`
  (`self.set flag in editor` (`self.Team`)))