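; Dialog component that holds a single current line of dialog, with functions to add, get and remove it.
; Adding a dialog replaces the stored one and starts a one-shot timer whose duration scales with the text's character count times a seconds-per-character value.
; Removing clears the text; the event the timer fires is not identified in the graph.
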(fn `Add dialog`
  (params (Dialog :type Text))
  (bind _output_get (set `self.Dialog` Dialog))
  (bind _time (`self.Get Dialog time` _output_get))
  (`KismetSystemLibrary.K2_SetTimerDelegate` (`|CreateDelegate` :!event `Remove dialog`) _time))

(fn `Get dialog`
  (returns (`Current dialog` :type Text))
  (return (`self.Dialog`)))

(fn `Get Dialog time`
  (params (Dialog :type Text))
  (returns (Time :type "Float (double-precision)"))
  (return (* (`KismetMathLibrary.Conv_IntToDouble` (`KismetStringLibrary.Len` (`KismetTextLibrary.Conv_TextToString` Dialog))) (`self.Seconds per char`))))

(fn `Remove dialog`
  (set `self.Dialog` ""))