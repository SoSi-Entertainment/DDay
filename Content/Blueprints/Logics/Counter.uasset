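; Counter is a zone logic actor that starts its ActionStarter when a condition selected by WhenTrigger is met.
; Conditions cover game start, counted entries or exits, live occupancy checked on Tick, the zone clearing, and deaths of visitors.
; Death modes record visitors and bind to each Base_Character's death event, firing at a count or once none remain.
; A Draw event forwards editor drawing to its action components.
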(event `self.ReceiveBeginPlay`
  (`parent.ReceiveBeginPlay`)
  (switch `/Game/Data/enums/Counter_mode` (`self.When trigger`)
    (:`NewEnumerator6`
      (`/Game/Blueprints/Logics/Components/Action_Starter.Start` (`self.Action_Starter`) "None" :!label _label))))

(event `self.ReceiveActorEndOverlap`
  (params (OtherActor :type "Actor Object Reference"))
  (if (`GameplayStatics.ObjectIsA` OtherActor (`self.Who triggers`))
    (switch `/Game/Data/enums/Counter_mode` (`self.When trigger`)
      (:`NewEnumerator0`
        ;[1 1 1] out / dead
        (bind _result (`/Engine/EditorBlueprintResources/StandardMacros.IncrementInt` (`self.c`))
          (:`  `
            (`/Engine/EditorBlueprintResources/StandardMacros.CompareInt` _result (`self.Count`)
              (:`==`
                (goto _label))))))
      (:`NewEnumerator2`
        ;[1 1 1] Clear
        (`/Engine/EditorBlueprintResources/StandardMacros.CompareInt` (`KismetArrayLibrary.Array_Length` (`self.GetOverlappingActors` (`self.Who triggers`)))
          (:`==`
            (goto _label)))))))

(event `self.ReceiveTick`
  (params (DeltaSeconds :type "Float (single-precision)"))
  (bind _returnvalue (`KismetArrayLibrary.Array_Length` (`self.GetOverlappingActors` (`self.Who triggers`))))
  ;[1 1 1] In zone at same time
  (switch `/Game/Data/enums/Counter_mode` (`self.When trigger`)
    (:`NewEnumerator3`
      (`/Engine/EditorBlueprintResources/StandardMacros.CompareInt` _returnvalue (`self.Count`)
        (:`==`
          (goto _label))))
    (:`NewEnumerator7`
      (`/Engine/EditorBlueprintResources/StandardMacros.CompareInt` _returnvalue
        (:`>`
          (goto _label))))))

(event `self.Triggered`
  (params (`Other actor` :type "Actor Object Reference"))
  ;[1 1 1] Comment
  (switch `/Game/Data/enums/Counter_mode` (`self.When trigger`)
    (:`NewEnumerator1`
      ;[1 1 1] In / spawn
      (bind _result (`/Engine/EditorBlueprintResources/StandardMacros.IncrementInt` (`self.c`))
        (:`  `
          (`/Engine/EditorBlueprintResources/StandardMacros.CompareInt` _result (`self.Count`)
            (:`==`
              (goto _label))))))
    (:`NewEnumerator5`
      (`KismetArrayLibrary.Array_AddUnique` (`self.Visitors`) `Other actor`)
      (bind _asbase_character (cast `/Game/Blueprints/Chars/Abstract/Base_Character` `Other actor`))
      (add `/Game/Blueprints/Chars/Abstract/Base_Character.Death` _asbase_character (delegate `Visitor dead counting`)))
    (:`NewEnumerator4`
      (`KismetArrayLibrary.Array_AddUnique` (`self.Visitors`) `Other actor`)
      (bind _asbase_character_2 (cast `/Game/Blueprints/Chars/Abstract/Base_Character` `Other actor`))
      (add `/Game/Blueprints/Chars/Abstract/Base_Character.Death` _asbase_character_2 (delegate `visitor dead`)))))

(event `visitor dead`
  (params (`Who died` :type "/Game/Blueprints/Chars/Abstract/Base_Character Object Reference"))
  (bind _visitors (`self.Visitors`))
  ;[1 1 1] Comment
  (`KismetArrayLibrary.Array_RemoveItem` _visitors `Who died`)
  (`/Engine/EditorBlueprintResources/StandardMacros.CompareInt` (`KismetArrayLibrary.Array_Length` _visitors)
    (:`==`
      (goto _label))))

(event `Visitor dead counting`
  (params (`Who died` :type "/Game/Blueprints/Chars/Abstract/Base_Character Object Reference"))
  (`KismetArrayLibrary.Array_RemoveItem` (`self.Visitors`) `Who died`)
  (bind _result (`/Engine/EditorBlueprintResources/StandardMacros.IncrementInt` (`self.c`))
    (:`  `
      (`/Engine/EditorBlueprintResources/StandardMacros.CompareInt` _result (`self.Count`)
        (:`==`
          (goto _label))))))

(event `/Game/Blueprints/Chars/Components/Checkpoint_Clearable.Clear`)

(event `/Game/Blueprints/Logics/Components/Editor_Drawable.Draw`
  (for _array_element (`self.K2_GetComponentsByClass` "/Game/Blueprints/Logics/Actions/Action_Component.Action_Component_C")
    (bind _aseditor_drawable (cast `/Game/Blueprints/Logics/Components/Editor_Drawable` _array_element))
    (`/Game/Blueprints/Logics/Components/Editor_Drawable.Draw` _aseditor_drawable)))

(fn `UserConstructionScript`
  (`parent.UserConstructionScript`))