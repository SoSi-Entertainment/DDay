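; Stationary destructible target that NPCs and weapons can damage, exposing aim point, radius and team through targeting functions.
; Radial damage and shell hits lower health and update an HP bar; at zero it removes its components and makes the tile beneath walkable.
; InstanceSaver stores damaged health at checkpoints and restores it on BeginPlay, re-applying destruction if zero.
; Cursor hover timers or a forced-HUD flag control name and HP bar visibility.
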(event `self.ReceiveBeginPlay`
  (set `self.health` (`self.max health`))
  (`self.Update HP bar`)
  (add `self.OnTakeRadialDamage` (delegate `Radial Damage`))
  (add `/Game/Blueprints/System/Level_Instance.Checkpoint reached` (`/Game/Blueprints/System/Funtions/FunctionLibrary.Get level instance`) (delegate `Checkpoint reached`))
  (`|ExecutionSequence`
    (:`then_0`
      (bind (_success _save) (`/Game/Blueprints/System/Components/Instance_Saver.Get save from instance` (`self.Instance_Saver`) 0 ""))
      (if _success
        (bind (_value _found) (`/Game/Blueprints/System/Saves/Instance_Save.Get field` _save "hp"))
        (if _found
          (bind _output_get (set `self.health` (`KismetStringLibrary.Conv_StringToDouble` _value)))
          (if (== _output_get 0.0)
            (`self.Destruction` true)
            (else
              (`self.Update HP bar`))))))))

(event `Checkpoint reached`
  (params (`Checkpoint number` :type Integer) (`Distance reached` :type "Float (double-precision)"))
  (if (< (`self.health`) (`self.max health`))
    (bind _random_save (`/Game/Blueprints/System/Components/Instance_Saver.Init instance save` (`self.Instance_Saver`) 0 ""))
    (`/Game/Blueprints/System/Saves/Instance_Save.Set field` _random_save "hp" (`KismetStringLibrary.Conv_DoubleToString` (`self.health`)))))

(event `Radial Damage` :!signature `self.OnTakeRadialDamage`
  (params (DamagedActor :type "Actor Object Reference") (Damage :type "Float (single-precision)") (DamageType :type "DamageType Object Reference") (Origin :type "Vector Structure") (HitInfo :type "HitResult Structure (by ref)") (InstigatedBy :type "Controller Object Reference") (DamageCauser :type "Actor Object Reference"))
  (`self.Apply damage` Damage))

(event `/Game/Blueprints/System/Interfaces/Aimable.Shell Hit`
  (params (Damage :type "Float (double-precision)") (`Silent damage` :type Boolean) (`Impact Point` :type "Vector Structure") (`Impact Normal` :type "Vector Structure") (`Impuls strength` :type "Float (double-precision)") (Shell :type "/Game/Blueprints/Arms/Shells/Shell Object Reference") (`From Character` :type "/Game/Blueprints/Chars/Abstract/Base_Character Object Reference"))
  (`self.Apply damage` Damage))

(event `/Game/Blueprints/System/Interfaces/Aimable.Set outline I`
  (params (Outlined :type Boolean))
  (bind _mesh (`self.Mesh`))
  (if (`self.Alive`)
    (`PrimitiveComponent.SetRenderCustomDepth` _mesh Outlined)
    (`PrimitiveComponent.SetCustomDepthStencilValue` _mesh 1)))

(event `/Game/Blueprints/System/Interfaces/Aimable.Under Cursor Start`
  (set `self.is hovered by cursor` true)
  (if (`self.Is name shown`)
    _
    (elif (`self.show name allowed`)
      (bind _returnvalue (`KismetSystemLibrary.K2_SetTimerDelegate` (`|CreateDelegate` :!event `Start show name`) (`self.Time under cursor to show hp`)))
      (set `self.under cursor start timer` _returnvalue))))

(event `/Game/Blueprints/System/Interfaces/Aimable.Under Cursor End`
  (set `self.is hovered by cursor` false)
  (`KismetSystemLibrary.K2_ClearAndInvalidateTimerHandle` (`self.under cursor start timer`))
  (`KismetSystemLibrary.K2_SetTimerDelegate` (`|CreateDelegate` :!event `Stop show name`) 0.5))

(event `/Game/Blueprints/System/Interfaces/Aimable.Forced Show HUD`
  (params (`Forced show` :type Boolean))
  (bind _output_get (set `self.Forced HUD` `Forced show`))
  (if _output_get
    (`self.Start show name`)
    (else
      (`self.Stop show name`))))

(fn `Allowed To Damage By Npc Of Team`
  (params (`NPC team` :type "/Game/Data/enums/Team Enum" :default "NewEnumerator0"))
  (returns (allowed :type Boolean))
  (bind _which_team_npc_can_damage (`self.Which Team NPC can damage`))
  (switch `/Game/Data/enums/Team` _which_team_npc_can_damage
    (:`NewEnumerator0`
      _)
    (:`NewEnumerator1`
      _)
    (:`NewEnumerator3`
      (return true))
    (:`NewEnumerator4`
      (return false)))
  (return (`|EnumEquality` _which_team_npc_can_damage `NPC team`)))

(fn `Apply damage`
  (params (Damage :type "Float (double-precision)"))
  (bind _output_get (set `self.health` (`KismetMathLibrary.FMax` (- (`self.health`) Damage))))
  (`self.Update HP bar`)
  (if (== _output_get 0.0)
    (if (`self.Alive`)
      (`self.Destruction` false))))

(fn `As Actor`
  (returns (Actor :type "Actor Object Reference"))
  (return self))

(fn `Destruction`
  (params (initial :type Boolean))
  (set `self.Alive` false)
  (`ActorComponent.K2_DestroyComponent` (`self.Mesh`))
  (`ActorComponent.K2_DestroyComponent` (`self.Area`))
  (`ActorComponent.K2_DestroyComponent` (`self.HP Bar`))
  (`ActorComponent.K2_DestroyComponent` (`self.Name Text`))
  (bind _tile (`/Game/Blueprints/System/Funtions/FunctionLibrary.Get Tile Under` (`self.K2_GetActorLocation`)))
  (`/Game/3D/platforms/Tile.Set walkable` _tile true))

(fn `Get Aboba Location`
  (returns (location :type "Vector Structure"))
  (return (`SceneComponent.K2_GetComponentLocation` (`self.shoot here`))))

(fn `Get Downside location`
  (returns (Location :type "Vector Structure"))
  (return (`self.K2_GetActorLocation`)))

(fn `Get Health Percent`
  (returns (Percantage :type "Float (double-precision)"))
  (return (/ (`self.Health`) (`self.Max health`))))

(fn `Get Location`
  (returns (Location :type "Vector Structure"))
  (return (`SceneComponent.K2_GetComponentLocation` (`self.shoot here`))))

(fn `Get Radius`
  (returns (Radius :type "Float (double-precision)"))
  (return (`self.Aim Radius`)))

(fn `Get Serial Info`
  (returns (Target :type String) (`Is Spawned` :type Boolean) (`Index in spawn` :type Integer))
  (return (`/Game/Blueprints/System/Funtions/FunctionLibrary.Get object path string` self) false 0))

(fn `Get Speed Smothed`
  (returns (`Speed vector` :type "Vector Structure"))
  (return (0.0 0.0 0.0)))

(fn `Get Target Location`
  (returns (Location :type "Vector Structure"))
  (return (`SceneComponent.K2_GetComponentLocation` (`self.shoot here`))))

(fn `Get Team I`
  (returns (Team :type "/Game/Data/enums/Team Enum"))
  (return "NewEnumerator3"))

(fn `Grid Fix`
  (`/Game/Blueprints/System/Components/Grid_Fixator.Fixate` (`self.Grid_Fixator`)))

(fn `Is Alive`
  (returns (Alive :type Boolean))
  (return true))

(fn `Is Forced high Interval`
  (returns (Forced :type Boolean) (`Up Point` :type "Vector Structure") (`Down Point` :type "Vector Structure"))
  (return true (`SceneComponent.K2_GetComponentLocation` (`self.Up Point`)) (`self.K2_GetActorLocation`)))

(fn `Is name shown`
  (returns (shown :type Boolean))
  (return (`SceneComponent.bVisible` (`self.Name Text`))))

(fn `Mark as future destroyed`
  (`PrimitiveComponent.SetMaterial` (`self.Mesh`) 0 "/AnimationSharing/AnimSharingGreen.AnimSharingGreen"))

(fn `Restore showing name`
  (if (or (`self.Forced HUD`) (`self.is hovered by cursor`))
    (`self.Start show name`)))

(fn `Show hp bar`
  (params (show :type Boolean))
  (if (`self.HP bar available`)
    (bind _hp_bar (`self.HP Bar`)
      (:`then`
        (`SceneComponent.SetVisibility` _hp_bar show false))
      (:`else`))))

(fn `Show name`
  (params (show :type Boolean))
  (locals (`text color` :type "Color Structure" :default (struct :`R` 255 :`A` 255)))
  (bind _name_text (`self.Name Text`))
  (bind _returnvalue (and show (`self.show name allowed`)))
  (`|ExecutionSequence`
    (:`then_0`
      (if show
        (`TextRenderComponent.K2_SetText` _name_text (`self.Text`))
        (`TextRenderComponent.SetTextRenderColor` _name_text (`local.text color`))))
    (:`then_1`
      (bind _name_text_2 (`self.Name Text`)
        (:`then`
          (`SceneComponent.SetVisibility` _name_text_2 _returnvalue false)
          (`self.Show hp bar` _returnvalue))
        (:`else`)))))

(fn `Start show name`
  (`self.Show name` true))

(fn `Stop show name`
  (if (`KismetMathLibrary.BooleanNOR` (`self.is hovered by cursor`) (`self.Forced HUD`))
    (`self.Show name` false)))

(fn `Update HP bar`
  (bind _hp_bar (`self.HP Bar`)
    (:`then`
      (`/Game/UI/Widgets/Game/World/Character_HP_Bar.Set hp percent` (cast `/Game/UI/Widgets/Game/World/Character_HP_Bar` (`WidgetComponent.GetWidget` _hp_bar) :!pure true) (`self.Get Health Percent`)))
    (:`else`)))

(fn `UserConstructionScript`)