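; Light_Rotator pitches a referenced light actor according to how far the player has advanced through the level.
; On begin play it records the light's starting rotation and finds the first and last Checkpoints by the numbers in their PlayerStartTags, storing their X positions.
; Each tick it maps the troops controller Body's X position between those bounds, keeping the last value if invalid, and feeds it through a curve into the pitch offset.
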(event `self.ReceiveBeginPlay`
  (set `self.start rotation` (`self.K2_GetActorRotation` (`self.Light to rotate`)))
  (bind (_first _last) (`self.Find first & last checpoints`))
  (set `self.progress start` (.x (`self.K2_GetActorLocation` _first)))
  (set `self.progress end` (.x (`self.K2_GetActorLocation` _last))))

(event `self.ReceiveTick`
  (params (DeltaSeconds :type "Float (single-precision)"))
  (`self.K2_SetActorRotation` (`self.Light to rotate`) (`KismetMathLibrary.ComposeRotators` (`self.start rotation`) (`KismetMathLibrary.MakeRotator` 0.0 (`CurveFloat.GetFloatValue` (`self.curve`) (`self.GetPercent`)))) false))

(fn `Find first & last checpoints`
  (returns (first :type "/Game/Blueprints/Logics/Checkpoint Object Reference") (last :type "/Game/Blueprints/Logics/Checkpoint Object Reference"))
  (locals (`first checkpoint` :type "/Game/Blueprints/Logics/Checkpoint Object Reference") (NewLocalVar :type Integer :default 0) (`biggest index` :type Integer) (`biggest num` :type Integer) (Checkpoints :type "Array of /Game/Blueprints/Logics/Checkpoint Object Reference"))
  (bind _outactors (`GameplayStatics.GetAllActorsOfClass` "/Game/Blueprints/Logics/Checkpoint.Checkpoint_C"))
  (bind _output_get (set `local.Checkpoints` _outactors))
  (for (_array_element _array_index) _output_get
    (`|ExecutionSequence`
      (:`then_0`
        (bind _returnvalue (`KismetStringLibrary.Conv_StringToInt` (`KismetStringLibrary.Conv_NameToString` (`PlayerStart.PlayerStartTag` _array_element))))
        (`/Engine/EditorBlueprintResources/StandardMacros.CompareInt` _returnvalue
          (:`==`
            (set `local.first checkpoint` _array_element))))
      (:`then_1`
        (`/Engine/EditorBlueprintResources/StandardMacros.CompareInt` _returnvalue (`local.biggest num`)
          (:`>`
            (set `local.biggest num` _returnvalue)
            (set `local.biggest index` _array_index))))))
  (return (`local.first checkpoint`) (`|GetArrayItem` _output_get (`local.biggest index`))))

(fn `GetPercent`
  (returns (ReturnValue :type "Float (single-precision)"))
  (bind _body (`/Game/Blueprints/Controllers/DDay_Player_Controller.Body` (`/Game/Blueprints/System/FunctionLibrary.Get PlayerController Troops`)))
  (`/Engine/EditorBlueprintResources/StandardMacros.IsValid` _body
    (:`Is Valid`
      (bind _output_get (set `self.last progress` (/ (- (.x (`self.K2_GetActorLocation` _body)) (`self.progress start`)) (- (`self.progress end`) (`self.progress start`))))))
    (:`Is Not Valid`
      _))
  (return _output_get))

(fn `UserConstructionScript`)