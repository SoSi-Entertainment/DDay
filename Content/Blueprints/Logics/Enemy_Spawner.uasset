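; Enemy spawner actor that spawns a configurable number of units of a given type at its location when play begins.
; A delayed loop spawns each unit slightly above the spawner, at a fixed interval.
; Each unit receives a copy of the spawner's path in its PathHolder and is possessed by a newly spawned Enemy_Ai_Controller.
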(event `self.ReceiveBeginPlay`
  (set `self.Spawn transform` (`KismetMathLibrary.MakeTransform` (+ (`self.K2_GetActorLocation`) (0.0 0.0 100.0))))
  (`/Game/Blueprints/System/DDayMacroLibrary.For loop with delay` 0 (- (`self.Spawn unit count`) 1) (`self.Delay`)
    (:`LoopBody`
      (bind _returnvalue (`|SpawnActorFromClass` (`self.Unit type`) (`self.Spawn transform`) "Undefined" "MultiplyWithRoot" null null))
      (`/Game/Blueprints/Navigation/Path_holder.Copy Data` (`/Game/Blueprints/Chars/Enemy_Character.Path_holder` _returnvalue) (`self.path`))
      (bind _returnvalue_2 (`|SpawnActorFromClass` "/Game/Blueprints/Navigation/Enemy_Ai_Controller.Enemy_Ai_Controller_C" (`self.Spawn transform`) "Undefined" "MultiplyWithRoot" null null))
      (`Controller.Possess` _returnvalue_2 _returnvalue))))

(fn `UserConstructionScript`)