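; Light manager actor that changes a controlled light's rotation and color as the game progresses.
; While active, each Tick samples a vector curve and a color curve at the percent from the troops game mode's ProgressComponent.
; It applies the results to the light and resets its specular scale to full.
; BeginPlay stores the light's starting rotation, which the graph never reads.
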(event `self.ReceiveBeginPlay`
  (set `self.start rotation` (`self.K2_GetActorRotation` (`self.Controled Light `))))

(event `self.ReceiveTick`
  (params (DeltaSeconds :type "Float (single-precision)"))
  (bind _controled_light_ (`self.Controled Light `))
  (bind _lightcomponent (`Light.LightComponent` _controled_light_))
  (if (`self.Active`)
    (`self.K2_SetActorRotation` _controled_light_ (`KismetMathLibrary.MakeRotator` (.x (`CurveVector.GetVectorValue` (`self.Light rotation`) (`self.GetPercent`))) (.y (`CurveVector.GetVectorValue` (`self.Light rotation`) (`self.GetPercent`))) (.z (`CurveVector.GetVectorValue` (`self.Light rotation`) (`self.GetPercent`)))) false)
    (`LightComponent.SetLightColor` _lightcomponent (`CurveLinearColor.GetLinearColorValue` (`self.Light color`) (`self.GetPercent`)) true)
    (`LightComponent.SetSpecularScale` _lightcomponent 1.0)))

(fn `GetPercent`
  (returns (ReturnValue :type "Float (single-precision)"))
  (return (`/Game/Blueprints/Logics/Components/Progress_Component.GetPercent` (`/Game/Blueprints/System/DDay_GameMode.Progress_Component` (`/Game/Blueprints/System/FunctionLibrary.Get GameMode Troops`)))))

(fn `UserConstructionScript`)