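; Hide_Area is an area actor that signals nearby platforms and walls to hide while the player is inside its detection volume.
; Shortly after BeginPlay it gathers wall platforms and default platform tiles overlapping PlatformsToHide, then passes itself to each through Hidable's CreateDinamicMaterial.
; Player_Main entering or leaving PlayerDetection calls the hide or unhide event.
; Helper functions return overlapping platforms and run a grid fixator.
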(event `self.ReceiveBeginPlay`
  (bind _platforms_to_hide (`self.Platforms To Hide`))
  (`KismetSystemLibrary.Delay` 0.2)
  (bind _output_get (set `self.targets` (`PrimitiveComponent.GetOverlappingActors` _platforms_to_hide "/Game/3D/platforms/Walls/Wall_Platform.Wall_Platform_C")))
  (for _array_element (`PrimitiveComponent.GetOverlappingActors` _platforms_to_hide "/Game/3D/platforms/Default_Platform_bp.Default_Platform_bp_C")
    (`KismetArrayLibrary.Array_Add` _output_get (`/Game/3D/platforms/Default_Platform_bp.Get tile` (cast `/Game/3D/platforms/Default_Platform_bp` _array_element :!pure true))))
  (for _array_element_2 (`self.targets`)
    (bind _ashidable (cast `/Game/3D/platforms/Hidable` _array_element_2))
    (`/Game/3D/platforms/Hidable.Create dinamic material` _ashidable self)))

(event `self.Player Detection.OnComponentBeginOverlap`
  (params (OverlappedComponent :type "PrimitiveComponent Object Reference") (OtherActor :type "Actor Object Reference") (OtherComp :type "PrimitiveComponent Object Reference") (OtherBodyIndex :type Integer) (bFromSweep :type Boolean) (SweepResult :type "HitResult Structure (by ref)"))
  (cast `/Game/Blueprints/Chars/Players/Player_Main` OtherActor)
  (`self.Hide event`))

(event `self.Player Detection.OnComponentEndOverlap`
  (params (OverlappedComponent :type "PrimitiveComponent Object Reference") (OtherActor :type "Actor Object Reference") (OtherComp :type "PrimitiveComponent Object Reference") (OtherBodyIndex :type Integer))
  (cast `/Game/Blueprints/Chars/Players/Player_Main` OtherActor)
  (`self.Unhide Event`))

(fn `Get tiles`
  (returns (Platforms :type "Array of Actor Object Reference"))
  (return (`PrimitiveComponent.GetOverlappingActors` (`self.Platforms To Hide`) "/Game/3D/platforms/Default_Platform_bp.Default_Platform_bp_C")))

(fn `Grid Fix`
  (`/Game/Blueprints/System/Components/Grid_Fixator.Fixate` (`self.Grid_Fixator`)))

(fn `UserConstructionScript`)