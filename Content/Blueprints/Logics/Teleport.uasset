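; Teleport is a one-way gate that moves any Base_Character overlapping GateIn toward GateOut.
; At BeginPlay it caches the offset between the gates and adds it to the character's position as an unswept teleport, preserving placement relative to the gate.
; The construction script uses TurnOn to set GateIn's in-game visibility and query collision.
; A Grid Fix function delegates to GridFixator.
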(event `self.ReceiveBeginPlay`
  (set `self.TP offset` (- (`SceneComponent.K2_GetComponentLocation` (`self.Gate Out`)) (`SceneComponent.K2_GetComponentLocation` (`self.Gate In`)))))

(event `self.Gate In.OnComponentBeginOverlap`
  (params (OverlappedComponent :type "PrimitiveComponent Object Reference") (OtherActor :type "Actor Object Reference") (OtherComp :type "PrimitiveComponent Object Reference") (OtherBodyIndex :type Integer) (bFromSweep :type Boolean) (SweepResult :type "HitResult Structure (by ref)"))
  (bind _asbase_character (cast `/Game/Blueprints/Chars/Abstract/Base_Character` OtherActor))
  (`self.K2_AddActorWorldOffset` _asbase_character (`self.TP offset`) false true))

(fn `Grid Fix`
  (`/Game/Blueprints/System/Grid_Fixator.Fixate` (`self.Grid_Fixator`)))

(fn `UserConstructionScript`
  (bind _turn_on (`self.Turn on`))
  (bind _gate_in (`self.Gate In`))
  (`SceneComponent.SetHiddenInGame` _gate_in (not _turn_on) false)
  (`PrimitiveComponent.SetCollisionEnabled` _gate_in (select `bool` _turn_on :`false` "NoCollision" :`true` "QueryOnly" :!type "ECollisionEnabled Enum")))