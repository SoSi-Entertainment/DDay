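; NPC target area volume that gathers walkable tiles from overlapping platforms, or trenches only, and hands them out as targets.
; On BeginPlay, after a short delay, it caches the tiles and loads or creates an instance save.
; Each pick replays the saved tile path by iterator index or records a new random one, then leaves the pool.
; It also reports player overlap and exposes grid snapping via GridFixator.
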(event `self.ReceiveBeginPlay`
  (bind _instance_saver (`self.Instance_Saver`))
  (`KismetSystemLibrary.Delay` 0.2)
  (bind _tiles (`self.Get tiles`))
  (set `self.Tiles` _tiles)
  (bind (_success _save) (`/Game/Blueprints/System/Components/Instance_Saver.Get save from instance` _instance_saver 0 ""))
  (if _success
    (set `self.Instance Save` _save)
    (else
      (bind _instance_save (`/Game/Blueprints/System/Components/Instance_Saver.Create save in instance` _instance_saver 0 false ""))
      (set `self.Instance Save` _instance_save))))

(fn `Choose tile`
  (params (Tiles :type "Array of /Game/3D/platforms/Tile Object Reference (by ref)"))
  (returns (OutItem :type "/Game/3D/platforms/Tile Object Reference"))
  (locals (`selected tile` :type "/Game/3D/platforms/Tile Object Reference"))
  (bind _intatce_iterator (`self.Intatce iterator`))
  (bind _data (`/Game/Blueprints/System/Saves/Instance_Save.Data` (`self.Instance Save`)))
  (`/Engine/EditorBlueprintResources/StandardMacros.CompareInt` _intatce_iterator (`KismetArrayLibrary.Array_LastIndex` _data)
    (:`>`
      (bind _output_get (set `local.selected tile` (`KismetArrayLibrary.Array_Random` Tiles)))
      (`KismetArrayLibrary.Array_Add` _data (`/Game/Blueprints/System/Funtions/FunctionLibrary.Get object path string` _output_get)))
    (:`==`
      (set `local.selected tile` (cast `/Game/3D/platforms/Tile` (`/Game/Blueprints/System/Funtions/FunctionLibrary.Find object by string` (`|GetArrayItem` _data _intatce_iterator)) :!pure true) :!label _label))
    (:`<`
      (goto _label)))
  (`/Engine/EditorBlueprintResources/StandardMacros.IncrementInt` (`self.Intatce iterator`)
    (:`  `
      (return (`local.selected tile`)))))

(fn `Get random tile`
  (returns (Tile :type "/Game/3D/platforms/Tile Object Reference"))
  (locals (`target tile` :type "/Game/3D/platforms/Tile Object Reference"))
  (bind _tiles (`self.Tiles`))
  (bind _outitem (`self.Choose tile` _tiles))
  (bind _output_get (set `local.target tile` _outitem))
  (`KismetArrayLibrary.Array_RemoveItem` _tiles _output_get)
  (return _output_get))

(fn `Get tiles`
  (returns (Tiles :type "Array of /Game/3D/platforms/Tile Object Reference"))
  (locals (`Target tiles` :type "Array of /Game/3D/platforms/Tile Object Reference"))
  (bind _target_tiles (`local.Target tiles`))
  (for _array_element (`self.GetOverlappingActors` (select `bool` (`self.Only in trench`) :`false` "/Game/3D/platforms/Default_Platform_bp.Default_Platform_bp_C" :`true` "/Game/3D/platforms/Tile_2/Trench/Trench.Trench_C" :!type "Actor Class Reference"))
    (bind _tile (`/Game/3D/platforms/Default_Platform_bp.Get tile` (cast `/Game/3D/platforms/Default_Platform_bp` _array_element :!pure true)))
    (bind _walkable (`/Game/3D/platforms/Tile.Is walkable` _tile))
    (if _walkable
      (`KismetArrayLibrary.Array_Add` _target_tiles _tile)))
  (return _target_tiles))

(fn `Grid Fix`
  (`/Game/Blueprints/System/Components/Grid_Fixator.Fixate` (`self.Grid_Fixator`)))

(fn `Is Player Inside`
  (returns (inside :type Boolean))
  (return (> (`KismetArrayLibrary.Array_Length` (`self.GetOverlappingActors` "/Game/Blueprints/Chars/Players/Player_Main.Player_Main_C")) 0)))

(fn `UserConstructionScript`)