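; Capturable flag base that changes hands between Ally and Enemy based on which side has more characters overlapping it, within a checkpoint range.
; Tick lowers the flag, switches side at the bottom, then raises it to complete capture and fire ActionStarter; AutoCapting forces Ally capture.
; A dynamic material colors the zone and flickers during movement, while tick interval switches between idle and active rates.
; Clear can reset the base to Ally.
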(event `self.ReceiveTick`
  (params (DeltaSeconds :type "Float (single-precision)"))
  (bind _action_starter (`self.Action_Starter`))
  (bind _auto_capting (`self.auto capting`))
  (`|ExecutionSequence`
    (:`then_0`
      (bind (_capturing _team) (`self.who capture`))
      (`|ExecutionSequence`
        (:`then_0`
          (if (or (and _capturing (`self.Is available`)) _auto_capting)
            (`|ExecutionSequence`
              (:`then_0`
                (`/Engine/EditorBlueprintResources/StandardMacros.DoOnce` false :!label _label
                  (:`Completed`
                    (`self.SetActorTickInterval` 0.0))))
              (:`then_1`
                (bind _returnvalue (select `bool` _auto_capting :`false` _team :`true` "NewEnumerator0"))
                (if (`|EnumEquality` (`self.Flag side`) _returnvalue)
                  (bind (_upped _moving) (`self.move up` DeltaSeconds))
                  (if (and _upped _moving)
                    (bind _team_changed (`self.Capture`))
                    (if _team_changed
                      (`|ExecutionSequence`
                        (:`then_0`
                          (switch `/Game/Data/enums/Team` _returnvalue
                            (:`NewEnumerator0`
                              (`/Game/Blueprints/Logics/Components/Action_Starter.Start` _action_starter "ally"))
                            (:`NewEnumerator1`
                              (`/Game/Blueprints/Logics/Components/Action_Starter.Start` _action_starter "None"))))
                        (:`then_1`
                          (set `self.auto capting` false)))))
                  (else
                    (bind _downed (`self.move down` DeltaSeconds))
                    (if _downed
                      (`self.switch side`)))))
              (:`then_2`
                (goto _label_2 :!via `Reset`)))
            (else
              (`|ExecutionSequence`
                (:`then_0`
                  (`/Engine/EditorBlueprintResources/StandardMacros.DoOnce` false :!label _label_2
                    (:`Completed`
                      (`self.SetActorTickInterval` 0.1))))
                (:`then_1`
                  (set `self.moving` false))
                (:`then_2`
                  (goto _label :!via `Reset`))))))
        (:`then_1`
          (`self.Update Zone` (`self.moving`) (`self.Is available`)))))
    (:`then_1`
      (`/Engine/EditorBlueprintResources/StandardMacros.CompareFloat` (`self.height`)
        (:`>`
          (set `self.height` 0.0))))))

(event `/Game/Blueprints/Logics/Components/Editor_Drawable.Draw`
  (for _array_element (`self.K2_GetComponentsByClass` "/Game/Blueprints/Logics/Actions/Action_Component.Action_Component_C")
    (bind _aseditor_drawable (cast `/Game/Blueprints/Logics/Components/Editor_Drawable` _array_element))
    (`/Game/Blueprints/Logics/Components/Editor_Drawable.Draw` _aseditor_drawable)))

(event `self.ReceiveBeginPlay`
  (`self.set flag material` (`self.Flag side`)))

(fn `Capture`
  (returns (`team changed` :type Boolean))
  (if (`|EnumInequality` (`self.Flag side`) (`self.Team`))
    (set `self.Team` (`self.Flag side`))
    (return true)
    (else
      (return false))))

(fn `Clear`
  (if (`self.Clear after checkpoint`)
    (`self.Set team` "NewEnumerator0")
    (set `self.Flag side` "NewEnumerator0")
    (set `self.Team` "NewEnumerator0")
    (if (`self.trigger ally if cleared`)
      (`/Game/Blueprints/Logics/Components/Action_Starter.Start` (`self.Action_Starter`) "ally"))
    (return)))

(fn `Is available`
  (returns (available :type Boolean))
  (bind _checkpoint_number (`/Game/Blueprints/System/Funtions/FunctionLibrary.Get Current Checkpoint num`))
  (bind (_always _from _to) (break `/Game/Data/structs/Checkpoint_Interval` (`self.Available on checkpoints`)))
  (return (or (and (>= _checkpoint_number _from) (<= _checkpoint_number _to)) _always)))

(fn `move down`
  (params (delta :type "Float (double-precision)"))
  (returns (downed :type Boolean))
  (set `self.Upped` false)
  (if (`self.Downed`)
    (set `self.moving` false)
    (return true)
    (else
      (bind _output_get (set `self.height` (- (`self.height`) (* delta (`KismetMathLibrary.SelectFloat` (`self.AutoCap speed`) (`self.Capture Speed`) (`self.auto capting`))))))
      (bind _output_get_2 (set `self.Downed` (<= _output_get (`self.down limit`))))
      (set `self.moving` (not _output_get_2))
      (return _output_get_2))))

(fn `move up`
  (params (delta :type "Float (double-precision)"))
  (returns (upped :type Boolean) (moving :type Boolean))
  (set `self.Downed` false)
  (if (`self.Upped`)
    (set `self.moving` false)
    (return true false)
    (else
      (bind _output_get (set `self.height` (+ (`self.height`) (* delta (`KismetMathLibrary.SelectFloat` (`self.AutoCap speed`) (`self.Capture Speed`) (`self.auto capting`))))))
      (bind _output_get_2 (set `self.Upped` (>= _output_get 0.0)))
      (set `self.moving` (not _output_get_2))
      (return _output_get_2 true))))

(fn `set flag material`
  (params (team :type "/Game/Data/enums/Team Enum" :default "NewEnumerator0"))
  (bind _troops_instance (`/Game/Blueprints/System/Funtions/FunctionLibrary.Get Instanse Troops`))
  (bind _flag (`self.Flag`))
  (bind _flag_state_module (`/Game/Blueprints/System/DDay_Instance.flag state module` _troops_instance))
  (`/Engine/EditorBlueprintResources/StandardMacros.IsValid` _troops_instance
    (:`Is Valid`
      (`PrimitiveComponent.SetMaterial` _flag 1 (select `/Game/Data/enums/Team` team :`NewEnumerator0` (`/Game/Blueprints/System/Instance_Modules/Flags/Flag_State_Module.ally flag material` _flag_state_module) :`NewEnumerator1` (`/Game/Blueprints/System/Instance_Modules/Flags/Flag_State_Module.enemy flag material` _flag_state_module) :!type "MaterialInterface Object Reference")))
    (:`Is Not Valid`
      (`PrimitiveComponent.SetMaterial` _flag 1 (select `/Game/Data/enums/Team` team :`NewEnumerator0` "/Game/3D/flag/txtr/britain/mat_britain.mat_britain" :`NewEnumerator1` "/Game/3D/flag/txtr/german/mat_german.mat_german" :!type "MaterialInterface Object Reference")))))

(fn `Set team`
  (params (Team :type "/Game/Data/enums/Team Enum" :default "NewEnumerator0"))
  (`self.set flag material` Team)
  (`MaterialInstanceDynamic.SetVectorParameterValue` (`self.zone material`) "color" (select `/Game/Data/enums/Team` Team :`NewEnumerator0` (struct :`G` 1.0 :`B` 0.002151 :`A` 1.0) :`NewEnumerator1` (struct :`R` 1.0 :`A` 1.0) :`NewEnumerator3` (struct :`R` 1.0 :`G` 1.0 :`B` 1.0 :`A` 1.0) :`NewEnumerator4` (struct :`R` 1.0 :`G` 1.0 :`B` 1.0 :`A` 1.0) :!type "LinearColor Structure")))

(fn `switch side`
  (switch `/Game/Data/enums/Team` (`self.Flag side`)
    (:`NewEnumerator0`
      (bind _output_get (set `self.Flag side` "NewEnumerator1"))
      (`self.Set team` _output_get))
    (:`NewEnumerator1`
      (bind _output_get_2 (set `self.Flag side` "NewEnumerator0"))
      (`self.Set team` _output_get_2))))

(fn `Update Zone`
  (params (moving :type Boolean) (Available :type Boolean))
  (`SceneComponent.SetVisibility` (`self.zone indicator`) Available false)
  (`MaterialInstanceDynamic.SetScalarParameterValue` (`self.zone material`) "flicking" (`KismetMathLibrary.SelectFloat` 0.25 0.0 moving)))

(fn `UserConstructionScript`
  (bind _flag_side (`self.Flag side`))
  (bind _returnvalue (`PrimitiveComponent.CreateDynamicMaterialInstance` (`self.zone indicator`) 0 "/Game/other/Materials/Base_zone/base_zone_inst.base_zone_inst" "None"))
  (set `self.zone material` _returnvalue)
  (`self.Set team` _flag_side)
  (set `self.Team` _flag_side))

(fn `who capture`
  (returns (Capturing :type Boolean) (Team :type "/Game/Data/enums/Team Enum"))
  (locals (`ally count` :type Integer) (`enemy count` :type Integer))
  (for _array_element (`self.GetOverlappingActors` (`self.Who triggers`))
    (cast `/Game/Blueprints/Chars/Abstract/Enemy_Character` _array_element
      (:`then`
        (`/Engine/EditorBlueprintResources/StandardMacros.IncrementInt` (`local.enemy count`)))
      (:`CastFailed`
        (cast `/Game/Blueprints/Chars/Abstract/Ally_Character` _array_element)
        (`/Engine/EditorBlueprintResources/StandardMacros.IncrementInt` (`local.ally count`)))))
  (return (!= (`local.ally count`) (`local.enemy count`)) (select `bool` (> (`local.ally count`) (`local.enemy count`)) :`false` "NewEnumerator1" :`true` "NewEnumerator0" :!type "/Game/Data/enums/Team Enum")))