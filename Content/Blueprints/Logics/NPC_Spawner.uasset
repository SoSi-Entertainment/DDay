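; NPC_Spawner is a one-shot spawner that creates a wave of NPC units when triggered.
; Each trigger starts its ActionStarter, but only the first, gated by the Virgin flag, spawns units after an initial delay, using a delayed loop.
; Units appear slightly above SpawnPoint with an HP coefficient applied.
; Ai_Character units also receive a copy of the spawner's Path and a newly spawned NPC_Ai_Controller that possesses them.
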(event `self.ReceiveBeginPlay`
  (set `self.Spawn transform` (`KismetMathLibrary.MakeTransform` (+ (`SceneComponent.K2_GetComponentLocation` (`self.Spawn point`)) (0.0 0.0 80.0)))))

(event `self.Triggered`
  (params (`Other actor` :type "Actor Object Reference"))
  (`/Game/Blueprints/Logics/Components/Action_Starter.Start` (`self.Action_Starter`))
  (if (`self.Virgin`)
    (set `self.Virgin` false)
    (`KismetSystemLibrary.Delay` (`self.Trigger delay`))
    (`/Game/Blueprints/System/DDayMacroLibrary.For loop with delay` 0 (- (`self.Spawn unit count`) 1) (`self.Delay`)
      (:`LoopBody`
        (bind _returnvalue (`|SpawnActorFromClass` (`self.Unit type`) (`self.Spawn transform`) "Undefined" "MultiplyWithRoot" null null))
        (`/Game/Blueprints/Chars/Base_Character.Apply hp coef` _returnvalue (`self.Unit hp coef`))
        (bind _asai_character (cast `/Game/Blueprints/Chars/Components/Ai_Character` _returnvalue))
        (bind _path (`/Game/Blueprints/Chars/Components/Ai_Character.Get path` _asai_character))
        (`/Game/Blueprints/Navigation/Path_holder.Copy Data` _path (`self.path`))
        (bind _returnvalue_2 (`|SpawnActorFromClass` "/Game/Blueprints/Controllers/NPC_Ai_Controller.NPC_Ai_Controller_C" (`self.Spawn transform`) "Undefined" "MultiplyWithRoot" null null))
        (`Controller.Possess` _returnvalue_2 _returnvalue)))))

(fn `UserConstructionScript`)