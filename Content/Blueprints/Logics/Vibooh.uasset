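; Vibooh is a one-shot explosion actor that does all its work on BeginPlay, then destroys itself.
; It applies radial damage with falloff that spares its owner.
; A vertical line trace finds any Flat platform at its location and calls AddExplosion on that platform's tile.
; It then plays a sound and spawns two Blast_bp effects at different rotations and scales.
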(event `self.ReceiveBeginPlay`
  (`GameplayStatics.ApplyRadialDamageWithFalloff` (`self.Damage`) 0.0 (`self.K2_GetActorLocation`) 0.0 (`self.Radius`) 2.0 null (`|MakeArray` (`self.GetOwner`)) self null "ECC_Pawn")
  (`self.Add explosion on platform`)
  (`self.Add effects`)
  (`self.K2_DestroyActor`))

(fn `Add effects`
  (bind _returnvalue (`self.K2_GetActorLocation`))
  (bind _returnvalue_2 (+ _returnvalue (0.0 0.0 0.0)))
  (`GameplayStatics.PlaySoundAtLocation` (`self.Sound`) _returnvalue (struct) 1.0 1.0 0.0 null null null null)
  (`|SpawnActorFromClass` "/Game/Effects/blast_bp.blast_bp_C" (`KismetMathLibrary.MakeTransform` _returnvalue_2) "Undefined" "MultiplyWithRoot" null null)
  (`|SpawnActorFromClass` "/Game/Effects/blast_bp.blast_bp_C" (`KismetMathLibrary.MakeTransform` _returnvalue_2 (struct :`Yaw` 60.0) (1.5 1.5 1.5)) "Undefined" "MultiplyWithRoot" null null))

(fn `Add explosion on platform`
  (bind _platform (`self.Get Platform under`))
  (`/Engine/EditorBlueprintResources/StandardMacros.IsValid` _platform
    (:`Is Valid`
      (`/Game/3D/platforms/Tile.Add explosion` (`/Game/3D/platforms/Default_Platform_bp.Get tile` _platform)))))

(fn `Get Platform under`
  (returns (platform :type "/Game/3D/platforms/Tile_2/Flat/Flat Object Reference"))
  (locals (`trace types` :type "Array of EObjectTypeQuery Enum"))
  (bind _returnvalue (`self.K2_GetActorLocation`))
  (bind _outhit (`KismetSystemLibrary.LineTraceSingleForObjects` (+ _returnvalue (0.0 0.0 100.0)) (- _returnvalue (0.0 0.0 100.0)) (`local.trace types`)))
  (bind _asflat (cast `/Game/3D/platforms/Tile_2/Flat/Flat` (`.HitActor` (`GameplayStatics.BreakHitResult` _outhit))))
  (return _asflat))

(fn `UserConstructionScript`)