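; NPC spawner actor that creates units of a configured type just above its location when Spawn is called while TurnOn is set.
; Each unit gets an HP coefficient, a copy of the spawner's path, a new NPC_Ai_Controller and an incremental ID, and joins the Spawned list.
; The construction script sets the marker material by enemy or ally type.
; GridFix and Rotate180 delegate to helpers for grid fixing and rotation.
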(event `self.ReceiveBeginPlay`
  (set `self.Spawn transform` (`KismetMathLibrary.MakeTransform` (+ (`self.K2_GetActorLocation`) (0.0 0.0 100.0)) (`self.K2_GetActorRotation`))))

(fn `Get spawned`
  (returns (spawned :type "Array of /Game/Blueprints/Chars/Abstract/Base_Character Object Reference"))
  (return (`self.Spawned`)))

(fn `Grid Fix`
  (`/Game/Blueprints/System/Grid_Fixator.Fixate` (`self.Grid_Fixator`)))

(fn `Rotate 180`
  (`/Game/Blueprints/System/180_Rotator.Rotate` (`self.180_Rotator`)))

(fn `Spawn`
  (bind _unit_id (`self.Unit id`))
  (if (`self.Turn on`)
    (bind _returnvalue (`|SpawnActorFromClass` (`self.Unit type`) (`self.Spawn transform`) "Undefined" "MultiplyWithRoot" self null))
    (`/Game/Blueprints/Chars/Abstract/Base_Character.Apply hp coef` _returnvalue (`self.Unit hp coef`))
    (bind _asai_character (cast `/Game/Blueprints/Chars/Components/Ai_Character` _returnvalue))
    (bind _path (`/Game/Blueprints/Chars/Components/Ai_Character.Get path` _asai_character))
    (`/Game/Blueprints/Navigation/Path_holder.Copy Data` _path (`self.Path`))
    (bind _returnvalue_2 (`|SpawnActorFromClass` "/Game/Blueprints/Controllers/NPC_Ai_Controller.NPC_Ai_Controller_C" (`self.Spawn transform`) "Undefined" "MultiplyWithRoot" null null))
    (`Controller.Possess` _returnvalue_2 _returnvalue)
    (set `/Game/Blueprints/Chars/Abstract/Base_Character.Id in spawner` _unit_id _returnvalue)
    (`/Engine/EditorBlueprintResources/StandardMacros.IncrementInt` _unit_id
      (:`  `
        (`KismetArrayLibrary.Array_Add` (`self.Spawned`) _returnvalue)))))

(fn `UserConstructionScript`
  (bind _unit_type (`self.Unit type`))
  (bind _spawn_point (`self.Spawn point`))
  (if (`self.Turn on`)
    (castclass `/Game/Blueprints/Chars/Enemy_Character` _unit_type
      (:`then`
        (`PrimitiveComponent.SetMaterial` _spawn_point 0 "/Engine/MapTemplates/Materials/BasicAsset01.BasicAsset01"))
      (:`CastFailed`
        (castclass `/Game/Blueprints/Chars/Ally_NPC` _unit_type)
        (`PrimitiveComponent.SetMaterial` _spawn_point 0 "/Engine/MapTemplates/Materials/BasicAsset03.BasicAsset03")))))