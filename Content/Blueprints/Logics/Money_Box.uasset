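; Money box Blueprint that adds its MoneyCount to the level instance's money when destroyed.
; It overrides Destruction, using InstanceSaver to check for a saved "was_desroyed" field, so the reward is granted only if that field is absent.
; After paying out it writes the field with an empty value as a presence flag, and the parent Destruction runs afterwards in every case.
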(fn `Destruction`
  (params (initial :type Boolean))
  (`|ExecutionSequence`
    (:`then_0`
      (bind _instance_save (`/Game/Blueprints/System/Components/Instance_Saver.Init instance save` (`self.Instance_Saver`) 0 ""))
      (if (not (`.found` (`/Game/Blueprints/System/Saves/Instance_Save.Get field` _instance_save "was_desroyed")))
        (`/Game/Blueprints/System/Instance_Modules/Level_Instance.Add money` (`/Game/Blueprints/System/Funtions/FunctionLibrary.Get level instance`) (`self.Money Count`))
        (`/Game/Blueprints/System/Saves/Instance_Save.Set field` _instance_save "was_desroyed" "")))
    (:`then_1`
      (`parent.Destruction` initial))))

(fn `UserConstructionScript`
  (`parent.UserConstructionScript`))