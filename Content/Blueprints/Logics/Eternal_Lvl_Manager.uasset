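; Level manager for an eternal mode that spawns endless waves, growing the unit count and adjusting the interval after each one.
; After an initial delay, each wave sends one preset to one spawn zone, both picked from run-seeded random streams keyed by wave number.
; A one-time check two seconds after BeginPlay calls WinLevel if the level lacks 70 money.
; SpawnWave, a weighted split across all zones, is never called.
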(event `self.ReceiveBeginPlay`
  (`|ExecutionSequence`
    (:`then_0`
      (`KismetSystemLibrary.Delay` (`self.Delay before first wave`))
      (`self.Spawn wave one flang` :!label _label)
      (`self.New wave` (`self.Wave number`))
      (`KismetSystemLibrary.Delay` (`self.Waves interval`))
      (set `self.Waves interval` (+ (`self.Waves interval`) (`self.Every wave add interval`)))
      (set `self.wave units count` (+ (`self.wave units count`) (`self.Every wave add units count`)))
      (`/Engine/EditorBlueprintResources/StandardMacros.IncrementInt` (`self.Wave number`)
        (:`  `
          (goto _label))))
    (:`then_1`
      (`KismetSystemLibrary.Delay` 2.0)
      (if (not (`/Game/Blueprints/System/Instance_Modules/Level_Instance.Is enough money` (`/Game/Blueprints/System/Funtions/FunctionLibrary.Get level instance`) 70))
        (`/Game/Blueprints/System/DDay_GameMode.Win Level` (`/Game/Blueprints/System/Funtions/FunctionLibrary.Get GameMode Troops`))))))

(fn `Spawn wave`
  (locals (`spawn zones weights` :type "Array of Float (single-precision)") (`spawn zones weight sum` :type "Float (single-precision)") (`current weight` :type "Float (single-precision)" :default 0.0) (`spawn zone counts` :type "Array of Float (single-precision)"))
  (for (_ _array_index) (`self.Spawn zones`)
    (bind _output_get (set `local.current weight` (`KismetMathLibrary.RandomFloatFromStream` (`/Game/Blueprints/System/Funtions/FunctionLibrary.Get Current Run Random Stream` self (`KismetStringLibrary.Concat_StrStr` (`KismetStringLibrary.Conv_IntToString` (`self.Wave number`)) "zone" (`KismetStringLibrary.Conv_IntToString` _array_index))))))
    (`KismetArrayLibrary.Array_Add` (`local.spawn zones weights`) _output_get)
    (set `local.spawn zones weight sum` (+ (`local.spawn zones weight sum`) _output_get)))
  (bind _outcounts (`CppFunctionLibrary.SpawnWeightedCount` (`local.spawn zones weights`) (`self.wave units count`)))
  (for (_array_element _array_index_2) _outcounts
    (`/Game/Blueprints/Logics/Path/Spawn_Zone.Spawn wave` (`|GetArrayItem` (`self.Spawn zones`) _array_index_2) (`KismetArrayLibrary.Array_RandomFromStream` (`self.Units Presets`) (`/Game/Blueprints/System/Funtions/FunctionLibrary.Get Current Run Random Stream` self (`KismetStringLibrary.Concat_StrStr` (`KismetStringLibrary.Conv_IntToString` (`self.Wave number`)) "preset" (`KismetStringLibrary.Conv_IntToString` _array_index_2)))) _array_element)))

(fn `Spawn wave one flang`
  (locals (`spawn zones weights` :type "Array of Float (single-precision)") (`spawn zones weight sum` :type "Float (single-precision)") (`current weight` :type "Float (single-precision)" :default 0.0) (`spawn zone counts` :type "Array of Float (single-precision)"))
  (`/Game/Blueprints/Logics/Path/Spawn_Zone.Spawn wave` (`KismetArrayLibrary.Array_RandomFromStream` (`self.Spawn zones`) (`/Game/Blueprints/System/Funtions/FunctionLibrary.Get Current Run Random Stream` self (`KismetStringLibrary.Concat_StrStr` (`KismetStringLibrary.Conv_IntToString` (`self.Wave number`)) "zone"))) (`KismetArrayLibrary.Array_RandomFromStream` (`self.Units Presets`) (`/Game/Blueprints/System/Funtions/FunctionLibrary.Get Current Run Random Stream` self (`KismetStringLibrary.Concat_StrStr` (`KismetStringLibrary.Conv_IntToString` (`self.Wave number`)) "preset"))) (`self.wave units count`)))

(fn `UserConstructionScript`)