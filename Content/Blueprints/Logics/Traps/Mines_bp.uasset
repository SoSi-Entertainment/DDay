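; Mine trap that detonates after a timer when an opposing or dead character, or optionally any character, overlaps its sphere.
; Detonation spawns a Vibooh explosion actor with damage and radius, logs an event for players, and removes the mine.
; Sufficient radial damage or any tile damage also detonates it after a chain delay.
; Exploded state saves at checkpoints for Clear to restore, and an optional nav modifier marks live mines as a separate area.
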(event `self.ReceiveBeginPlay`
  (add `/Game/Blueprints/System/Instance_Modules/Level_Instance.Checkpoint reached` (`/Game/Blueprints/System/Funtions/FunctionLibrary.Get level instance`) (delegate `Checkpoint reached`)))

(event `Checkpoint reached`
  (params (`Checkpoint number` :type Integer) (`Distance reached` :type "Float (double-precision)"))
  (if (`self.Exploded`)
    (`/Game/Blueprints/System/Components/Instance_Saver.Create save in instance` (`self.Instance_Saver`) 0 false "")))

(event `self.Sphere.OnComponentBeginOverlap`
  (params (OverlappedComponent :type "PrimitiveComponent Object Reference") (OtherActor :type "Actor Object Reference") (OtherComp :type "PrimitiveComponent Object Reference") (OtherBodyIndex :type Integer) (bFromSweep :type Boolean) (SweepResult :type "HitResult Structure (by ref)"))
  (bind _asbase_character (cast `/Game/Blueprints/Chars/Abstract/Base_Character` OtherActor))
  (if (or (`|EnumInequality` (`/Game/Blueprints/Chars/Abstract/Base_Character.Team` _asbase_character) (`self.Team`)) (`self.Both team trigger`) (`/Game/Blueprints/Chars/Abstract/Base_Character.Dead` _asbase_character))
    (`KismetSystemLibrary.Delay` (`self.Timer`))
    (if (not (`self.Exploded`)) :!label _label
      (`|ExecutionSequence`
        (:`then_0`
          (cast `/Game/Blueprints/Chars/Players/Player_Main` _asbase_character)
          (`/Game/Blueprints/Controllers/Player_Controller.Save event` (`/Game/Blueprints/System/Funtions/FunctionLibrary.Get PlayerController Troops`) "NewEnumerator2" null))
        (:`then_1`
          (`self.Spawn vibooh`)
          (`self.Die`))))))

(event `self.ReceiveRadialDamage`
  (params (DamageReceived :type "Float (single-precision)") (DamageType :type "DamageType Object Reference") (Origin :type "Vector Structure") (HitInfo :type "HitResult Structure (by ref)") (InstigatedBy :type "Controller Object Reference") (DamageCauser :type "Actor Object Reference"))
  (`/Engine/EditorBlueprintResources/StandardMacros.CompareFloat` DamageReceived (`self.Chain Start Damage`)
    (:`>`
      (`KismetSystemLibrary.Delay` (`self.Chain delay`) :!label _label_2)
      (goto _label))))

(event `Tile damage`
  (params (Damage :type "Float (double-precision)"))
  (goto _label_2))

(fn `Add explosion on platform`
  (bind _tile (`/Game/Blueprints/System/Funtions/Tile_Functions.Get Tile Under` (`self.K2_GetActorLocation`) 100.0))
  (`/Engine/EditorBlueprintResources/StandardMacros.IsValid` _tile
    (:`Is Valid`
      (`/Game/3D/platforms/Tile.Add explosion` _tile false))))

(fn `Clear`
  (bind _success (`/Game/Blueprints/System/Components/Instance_Saver.Get save from instance` (`self.Instance_Saver`) 0 ""))
  (if _success
    (`self.Die`)
    (return)))

(fn `Die`
  (`ActorComponent.K2_DestroyComponent` (`self.Sphere`))
  (`ActorComponent.K2_DestroyComponent` (`self.mesh`))
  (set `self.Exploded` true)
  (if (`self.High navigation price`)
    (`NavModifierComponent.SetAreaClass` (`self.NavModifier`) null)))

(fn `Explode`
  (bind _returnvalue (`self.K2_GetActorLocation`))
  (bind _returnvalue_2 (+ _returnvalue (0.0 0.0 0.0)))
  (`GameplayStatics.PlaySoundAtLocation` "/Game/Sounds/Shoting_Cue/MineExplosion_Cue.MineExplosion_Cue" _returnvalue (struct) 1.0 1.0 0.0 null null null null)
  (`|SpawnActorFromClass` "/Game/Effects/blast_bp.blast_bp_C" (`KismetMathLibrary.MakeTransform` _returnvalue_2) "Undefined" "MultiplyWithRoot" null null)
  (`|SpawnActorFromClass` "/Game/Effects/blast_bp.blast_bp_C" (`KismetMathLibrary.MakeTransform` _returnvalue_2 (struct :`Yaw` 60.0) (1.5 1.5 1.5)) "Undefined" "MultiplyWithRoot" null null)
  (`|SpawnActorFromClass` "/Game/Effects/Hit/blood_bp.blood_bp_C" (`KismetMathLibrary.MakeTransform` _returnvalue (struct) (3.0 3.0 0.01)) "Undefined" "MultiplyWithRoot" null null))

(fn `Grid Fix`
  (`/Game/Blueprints/System/Components/Grid_Fixator.Fixate` (`self.Grid_Fixator`)))

(fn `Spawn vibooh`
  (`|SpawnActorFromClass` "/Game/Blueprints/Logics/Components/Vibooh.Vibooh_C" (`KismetMathLibrary.MakeTransform` (`self.K2_GetActorLocation`)) "Undefined" "MultiplyWithRoot" self (`self.Damage`) (`self.Radius`) "/Game/Sounds/Shoting_Cue/MineExplosion_Cue.MineExplosion_Cue" null))

(fn `UserConstructionScript`
  (`NavModifierComponent.SetAreaClass` (`self.NavModifier`) (select `bool` (`self.High navigation price`) :`true` "/Game/Blueprints/Navigation/nav_mesh/Mine_Area.Mine_Area_C" :!type "NavArea Class Reference")))