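; Kill zone actor that kills characters of a configurable type when they overlap it.
; With artillery enabled, it spawns a high-damage shell at a randomly tilted offset from the victim, plays an incoming sound and calls Die after a delay.
; Otherwise it calls Die after a shorter delay.
; A Clear event destroys the zone when flagged to clear after a checkpoint, and GridFix calls GridFixator to fixate it.
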(event `self.ReceiveActorBeginOverlap`
  (params (OtherActor :type "Actor Object Reference"))
  (bind _returnvalue (`KismetMathLibrary.RandomFloatInRange` -20.0 20.0))
  (bind _returnvalue_2 (`KismetMathLibrary.MakeRotator` _returnvalue _returnvalue _returnvalue))
  (bind _asbase_character (cast `/Game/Blueprints/Chars/Abstract/Base_Character` OtherActor))
  (if (`GameplayStatics.ObjectIsA` OtherActor (`self.Kill character type`))
    (if (`self.Use artellery`)
      (bind _returnvalue_3 (`self.K2_GetActorLocation` _asbase_character))
      (`/Game/Blueprints/System/Funtions/FunctionLibrary.Get platform under` _returnvalue_3)
      (`|SpawnActorFromClass` :`Class` "/Game/Blueprints/Arms/Shells/Art_Shell.Art_Shell_C" :`SpawnTransform` (`KismetMathLibrary.MakeTransform` (+ _returnvalue_3 (`KismetMathLibrary.GreaterGreater_VectorRotator` (`KismetMathLibrary.MakeVector` 0.0 0.0 (`self.Spawn distance`)) _returnvalue_2)) (`KismetMathLibrary.ComposeRotators` (struct :`Yaw` 90.0 :`Roll` 90.0) _returnvalue_2)) :`CollisionHandlingOverride` "Undefined" :`TransformScaleMethod` "MultiplyWithRoot" :`Target tile` null :`Team` "NewEnumerator3" :`shot info` null :`shell params` (make `/Game/Data/structs/Shell_params` (`self.Shell speed`) 2000.0 2000.0) :`Instigator` null)
      (`GameplayStatics.SpawnSoundAtLocation` "/Game/Sounds/Artellery/Artelley_Incoming.Artelley_Incoming" _returnvalue_3 (struct) 1.0 2.0 0.5 null null)
      (`KismetSystemLibrary.Delay` 1.0)
      (`/Game/Blueprints/Chars/Abstract/Base_Character.Die` _asbase_character null false (0.0 0.0 0.0) (0.0 0.0 0.0) (0.0 0.0 0.0) false null)
      (else
        (`KismetSystemLibrary.Delay` 0.5)
        (`/Game/Blueprints/Chars/Abstract/Base_Character.Die` _asbase_character null false (0.0 0.0 0.0) (0.0 0.0 0.0) (0.0 0.0 0.0) false null)))))

(event `/Game/Blueprints/Chars/Components/Checkpoint_Clearable.Clear`
  (if (`self.Clear after checkpoint`)
    (`self.K2_DestroyActor`)))

(fn `Grid Fix`
  (`/Game/Blueprints/System/Components/Grid_Fixator.Fixate` (`self.Grid_Fixator`)))

(fn `UserConstructionScript`)