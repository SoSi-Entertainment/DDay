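; Sensor is a trigger volume that adds dialog text when the player's Main_Character walks into it.
; The Box overlap event calls DoAction, which passes the Text variable to the DialogComponent on DDay_GameMode.
; With TriggersOnce set, the Virigin flag limits it to the first overlap; otherwise every overlap adds the dialog again.
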(event `self.Box.OnComponentBeginOverlap`
  (params (OverlappedComponent :type "PrimitiveComponent Object Reference") (OtherActor :type "Actor Object Reference") (OtherComp :type "PrimitiveComponent Object Reference") (OtherBodyIndex :type Integer) (bFromSweep :type Boolean) (SweepResult :type "HitResult Structure (by ref)"))
  (cast `/Game/Blueprints/Chars/Main_Character` OtherActor)
  (`self.Do action`))

(fn `Do action`
  (if (`self.Triggers once`)
    (if (`self.Virigin`)
      (bind _asdday_game_mode (cast `/Game/Blueprints/System/DDay_GameMode` (`GameplayStatics.GetGameMode`) :!label _label))
      (`/Game/Blueprints/Logics/Dialog_component.Add dialog` (`/Game/Blueprints/System/DDay_GameMode.Dialog_component` _asdday_game_mode) (`self.Text`))
      (set `self.Virigin` false))
    (else
      (goto _label))))

(fn `UserConstructionScript`)