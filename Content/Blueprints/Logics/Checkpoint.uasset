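; Numbered player-start checkpoint that saves level progress through the level instance when the player overlaps its trigger.
; Its number comes from PlayerStartTag; unless hidden, reaching it plays a sound and spawns an animated radio.
; On load, passed checkpoints respawn their radios, and the current one clears Checkpoint_Clearable actors behind its rotated clear line.
; In editor, it snaps above the platform below and draws debug links.
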(event `self.ReceiveBeginPlay`
  (bind _number (`self.Number`))
  (bind _returnvalue (`KismetStringLibrary.Conv_NameToString` (`self.PlayerStartTag`)))
  (bind _checkpoint_number (`/Game/Blueprints/System/Instance_Modules/Level_Instance.Checkpoint Number` (`/Game/Blueprints/System/Funtions/FunctionLibrary.Get level instance`)))
  (add `self.OnActorBeginOverlap` (`ChildActorComponent.ChildActor` (`self.Trigger`)) (delegate `TriggerEvent`))
  ;[1 1 1] Check tag
  (if (`KismetStringLibrary.IsNumeric` _returnvalue)
    (set `self.Number` (`KismetStringLibrary.Conv_StringToInt` _returnvalue))
    (`|ExecutionSequence`
      (:`then_0`
        ;[1 1 1] check if checkpoint is old
        (set `self.Triggered` (> _checkpoint_number _number))
        (if (== _checkpoint_number _number)
          (`self.Clear Before`)))
      (:`then_1`
        (if (<= (`self.Number`) (`/Game/Blueprints/System/Instance_Modules/Level_Instance.Checkpoint Number` (`/Game/Blueprints/System/Funtions/FunctionLibrary.Get level instance`)))
          (`self.Spawn radio` false))))
    (else
      (`KismetSystemLibrary.PrintString` "Wrong checkpoint name" true true (struct :`R` 1.0 :`A` 1.0) 5.0))))

(event `TriggerEvent` :!signature `self.OnActorBeginOverlap`
  (params (OverlappedActor :type "Actor Object Reference") (OtherActor :type "Actor Object Reference"))
  (cast `/Game/Blueprints/Chars/Players/Player_Main` OtherActor)
  (if (`self.Own zone trigger`)
    (`self.Set point checked`)))

(event `Player spawned`
  (`/Game/Blueprints/Logics/Components/Action_Starter.Start` (`self.Action_Starter`) "None"))

(event `/Game/Blueprints/Logics/Components/Editor_Drawable.Draw`
  (bind _npc_target_area (`self.NPC Target Area`))
  (bind _world (`self.Local to world` (`self.Clear Line`)))
  (bind _returnvalue (`KismetMathLibrary.MakeVector` 0.0 (`self.Clear Line Lengh`)))
  ;[1 1 1] Draw action links
  (for _array_element (`self.K2_GetComponentsByClass` "/Game/Blueprints/Logics/Actions/Action_Component.Action_Component_C")
    (bind _aseditor_drawable (cast `/Game/Blueprints/Logics/Components/Editor_Drawable` _array_element))
    (`/Game/Blueprints/Logics/Components/Editor_Drawable.Draw` _aseditor_drawable))
  (`KismetSystemLibrary.DrawDebugLine` (- _world _returnvalue) (+ _world _returnvalue) (struct :`G` 1.0 :`B` 0.99346 :`A` 1.0) 10.0 10.0)
  (`/Engine/EditorBlueprintResources/StandardMacros.IsValid` _npc_target_area
    (:`Is Valid`
      (`KismetSystemLibrary.DrawDebugLine` (+ (`self.K2_GetActorLocation`) (0.0 0.0 100.0)) (+ (`self.K2_GetActorLocation` _npc_target_area) (0.0 0.0 100.0)) (struct :`R` 0.029834 :`G` 0.666667 :`B` 0.166529 :`A` 1.0) 10.0 7.0))))

(fn `Clear Before`
  (bind _outactors (`GameplayStatics.GetAllActorsWithInterface` "/Game/Blueprints/Chars/Components/Checkpoint_Clearable.Checkpoint_Clearable_C"))
  (for _array_element _outactors
    (bind _before (`self.Is Actor Before CheckPoint` _array_element))
    (if _before
      (`/Game/Blueprints/Chars/Components/Checkpoint_Clearable.Clear` (cast `/Game/Blueprints/Chars/Components/Checkpoint_Clearable` _array_element :!pure true)))))

(fn `Force Clear before`
  (bind _outactors (`GameplayStatics.GetAllActorsOfClass` "/Game/Blueprints/Chars/Abstract/Enemy_Character.Enemy_Character_C"))
  (for _array_element _outactors
    (bind _before (`self.Is Actor Before CheckPoint` _array_element))
    (if _before
      (bind _asbase_character (cast `/Game/Blueprints/Chars/Abstract/Base_Character` _array_element))
      (`/Game/Blueprints/Chars/Abstract/Base_Character.Die on start` :`self` _asbase_character :`Cleared` true))))

(fn `Get checkpoint line`
  (returns (`X Coord` :type "Float (double-precision)"))
  (return (.x (`self.Local to world` (`self.Clear Line`)))))

(fn `Get time progress`
  (returns (progress :type "Float (double-precision)"))
  (return (+ (`/Game/Blueprints/System/Funtions/FunctionLibrary.Get progress` self) (`self.Time offset (light)`))))

(fn `Is Actor Before CheckPoint`
  (params (Actor :type "Actor Object Reference"))
  (returns (Before :type Boolean))
  (bind _returnvalue (`self.K2_GetActorLocation` Actor))
  (bind _returnvalue_2 (`self.K2_GetActorRotation`))
  (return (> (.x (`KismetMathLibrary.GreaterGreater_VectorRotator` (- (`KismetMathLibrary.FindClosestPointOnLine` _returnvalue (`self.Local to world` (`self.Clear Line`)) (`KismetMathLibrary.GreaterGreater_VectorRotator` (0.0 -1.0 0.0) _returnvalue_2)) _returnvalue) (`KismetMathLibrary.NegateRotator` _returnvalue_2))) 0.0)))

(fn `Local to world`
  (params (Local :type "Vector Structure"))
  (returns (World :type "Vector Structure"))
  (return (`KismetMathLibrary.TransformLocation` (`self.GetTransform`) Local)))

(fn `Set point checked`
  (if (not (`self.Triggered`))
    (bind _success (`/Game/Blueprints/System/Instance_Modules/Level_Instance.Set Check Point` (`/Game/Blueprints/System/Funtions/FunctionLibrary.Get level instance`) (`self.Number`) (`self.Get checkpoint line`)))
    (if _success
      (set `self.Triggered` true)
      (if (not (`self.Hidden checkpoint`))
        (`GameplayStatics.PlaySound2D` (`self.Reach sound`) 1.0 1.0 0.0 null null)
        (`self.Spawn radio` true)))))

(fn `set trigger forward position`
  (bind _trigger (`self.Trigger`))
  (`SceneComponent.K2_SetRelativeLocation` _trigger (140.0 0.0 -90.0) false false)
  (`SceneComponent.SetRelativeScale3D` _trigger (0.2 20.0 1.0)))

(fn `Spawn radio`
  (params (`With animation` :type Boolean))
  (bind _radio_point (`self.Radio point`))
  (`/Engine/EditorBlueprintResources/StandardMacros.IsValid` _radio_point
    (:`Is Valid`
      (`|SpawnActorFromClass` "/Game/3D/Artificial/Walkie_Talkie/Fbx/ally/Radio.Radio_C" (`self.GetTransform` _radio_point) "Undefined" "MultiplyWithRoot" null `With animation` null))))

(fn `Update visibility`
  (params (`New visible` :type Boolean))
  (bind _output_get (set `self.Visible` `New visible`))
  (`SceneComponent.SetVisibility` (`self.Trigger`) (and _output_get (`self.Own zone trigger`)) false))

(fn `UserConstructionScript`
  (`/Engine/EditorBlueprintResources/StandardMacros.IsValid` (`GameplayStatics.GetGameState`)
    (:`Is Not Valid`
      (set `self.Clear Line` (`KismetMathLibrary.MakeVector` (.x (`self.Clear Line`))))
      (`SceneComponent.SetVisibility` (`self.Trigger`) (and (`self.Visible`) (`self.Own zone trigger`)) false)
      (bind _surface_location (`/Game/Blueprints/System/Funtions/FunctionLibrary.Get platform under` (`self.K2_GetActorLocation`)))
      (`self.K2_SetActorLocation` (`KismetMathLibrary.MakeVector` (.x (`self.K2_GetActorLocation`)) (.y (`self.K2_GetActorLocation`)) (+ (.z _surface_location) (`self.Height above tile`) 0.0)))
      (if (`self.Forward Line trigger`)
        (`self.set trigger forward position`)))))