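; Action group actor, named for level opening, that holds Action_Component actions and exposes a Start function to launch them through ActionStarter.
; The construction script labels it with its optional name and action count, or "Empty" when it has none.
; Text scale derives from LineLengh and the longest candidate line, including an "on start" suffix that is hard-wired off.
; The file shows no level-open trigger, and its Draw event is empty.
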(event `/Game/Blueprints/Logics/Components/Editor_Drawable.Draw`)

(fn `start`
  (`/Game/Blueprints/Logics/Components/Action_Starter.Start` (`self.Action_Starter`) "None"))

(fn `UserConstructionScript`
  (bind _name (`self.Name`))
  (bind _textrender (`self.TextRender`))
  (bind _returnvalue (`KismetArrayLibrary.Array_Length` (`self.K2_GetComponentsByClass` "/Game/Blueprints/Logics/Actions/Action_Component.Action_Component_C")))
  (bind _returnvalue_2 (`KismetMathLibrary.SelectString` "Empty" (`KismetStringLibrary.Concat_StrStr` (`KismetStringLibrary.Conv_IntToString` _returnvalue) " " "Actions") (== _returnvalue 0)))
  (bind _returnvalue_3 (`KismetMathLibrary.SelectString` _returnvalue_2 (`KismetStringLibrary.Concat_StrStr` _name "<br>" _returnvalue_2) (`KismetStringLibrary.IsEmpty` _name)))
  (`TextRenderComponent.K2_SetText` _textrender (`KismetTextLibrary.Conv_StringToText` (`KismetMathLibrary.SelectString` (`KismetStringLibrary.Concat_StrStr` _returnvalue_3 "<br>" "on start") _returnvalue_3)))
  (`SceneComponent.SetRelativeScale3D` _textrender (`KismetMathLibrary.Conv_DoubleToVector` (/ (`self.line lengh`) (`KismetMathLibrary.Max` (`KismetStringLibrary.Len` _returnvalue_2) (`KismetStringLibrary.Len` _name) (`KismetStringLibrary.Len` "on start"))))))