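; Team-based proximity mine that detonates after a timer when a character enters its sphere.
; Enemy or dead characters trigger it, as does anyone when BothTeamTrigger is set; it then spawns a Vibooh explosion actor carrying damage, radius and sound, and destroys itself.
; A separate Clear function adds an explosion to the nearest overlapping Flat platform before destroying the mine.
; The Explode effects function is not called here, and the body-throw impulse is disconnected.
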(event `self.ReceiveBeginPlay`)

(event `self.ReceiveActorBeginOverlap`
  (params (OtherActor :type "Actor Object Reference")))

(event `self.Sphere.OnComponentBeginOverlap`
  (params (OverlappedComponent :type "PrimitiveComponent Object Reference") (OtherActor :type "Actor Object Reference") (OtherComp :type "PrimitiveComponent Object Reference") (OtherBodyIndex :type Integer) (bFromSweep :type Boolean) (SweepResult :type "HitResult Structure (by ref)"))
  (bind _asbase_character (cast `/Game/Blueprints/Chars/Abstract/Base_Character` OtherActor))
  (if (or (`|EnumInequality` (`/Game/Blueprints/Chars/Abstract/Base_Character.Team` _asbase_character) (`self.Team`)) (`self.Both team trigger`) (`/Game/Blueprints/Chars/Abstract/Base_Character.Dead` _asbase_character))
    (`KismetSystemLibrary.Delay` (`self.Timer`))
    (`|SpawnActorFromClass` "/Game/Blueprints/Logics/Vibooh.Vibooh_C" (`KismetMathLibrary.MakeTransform` (`self.K2_GetActorLocation`)) "Undefined" "MultiplyWithRoot" self (`self.Damage`) (`self.Radius`) "/Game/Sounds/Shoting_Cue/MineExplosion_Cue.MineExplosion_Cue" null)
    (`self.Die`)))

(fn `Add explosion on platform`
  (bind _platform (`self.Get Platform under`))
  (`/Engine/EditorBlueprintResources/StandardMacros.IsValid` _platform
    (:`Is Valid`
      (`/Game/3D/platforms/Tile_2/Flat/Flat.Add explosion` _platform))))

(fn `Clear`
  (`self.Add explosion on platform`)
  (`self.K2_DestroyActor`)
  (return))

(fn `Die`
  (`self.K2_DestroyActor`))

(fn `Explode`
  (bind _returnvalue (`self.K2_GetActorLocation`))
  (bind _returnvalue_2 (+ _returnvalue (0.0 0.0 0.0)))
  (`GameplayStatics.PlaySoundAtLocation` "/Game/Sounds/Shoting_Cue/MineExplosion_Cue.MineExplosion_Cue" _returnvalue (struct) 1.0 1.0 0.0 null null null null)
  (`|SpawnActorFromClass` "/Game/Effects/blast_bp.blast_bp_C" (`KismetMathLibrary.MakeTransform` _returnvalue_2) "Undefined" "MultiplyWithRoot" null null)
  (`|SpawnActorFromClass` "/Game/Effects/blast_bp.blast_bp_C" (`KismetMathLibrary.MakeTransform` _returnvalue_2 (struct :`Yaw` 60.0) (1.5 1.5 1.5)) "Undefined" "MultiplyWithRoot" null null)
  (`|SpawnActorFromClass` "/Game/Effects/blood_bp.blood_bp_C" (`KismetMathLibrary.MakeTransform` _returnvalue (struct) (3.0 3.0 0.01)) "Undefined" "MultiplyWithRoot" null null))

(fn `Get Platform under`
  (returns (platform :type "/Game/3D/platforms/Tile_2/Flat/Flat Object Reference"))
  (locals (`Clothest distance` :type "Float (double-precision)" :default 1000.0) (`clothest platform` :type "/Game/3D/platforms/Tile_2/Flat/Flat Object Reference"))
  (for _array_element (`PrimitiveComponent.GetOverlappingActors` (`self.Sphere`) "/Game/3D/platforms/Tile_2/Flat/Flat.Flat_C")
    (bind _returnvalue (`KismetMathLibrary.Vector_Distance` (`self.K2_GetActorLocation` _array_element) (`self.K2_GetActorLocation`)))
    (`/Engine/EditorBlueprintResources/StandardMacros.CompareFloat` _returnvalue (`local.Clothest distance`)
      (:`<`
        (set `local.Clothest distance` _returnvalue)
        (set `local.clothest platform` (cast `/Game/3D/platforms/Tile_2/Flat/Flat` _array_element :!pure true)))))
  (return (`local.clothest platform`)))

(fn `UserConstructionScript`)