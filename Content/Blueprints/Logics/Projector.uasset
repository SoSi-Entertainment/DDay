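; Movie projector actor that plays a video with timed subtitles on a widget screen, along with reel animation, Niagara effect, sound and music.
; Activate initializes the Projector_Screen widget and fades the screen via a timeline.
; Video-end callbacks replay until the loop count is reached, then deactivate it.
; Subtitles run from a copied buffer, with chained one-shot timers showing, clearing and removing each entry by its time interval.
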(event `Deactivate`
  (`SkeletalMeshComponent.Stop` (`self.Projector Mesh`))
  (`SceneComponent.SetHiddenInGame` (`self.Screen`) true false)
  (`SceneComponent.SetHiddenInGame` (`self.NS_Projector`) true false)
  (`AudioComponent.Stop` (`self.ProjectorSound_Cue`))
  (`AudioComponent.Stop` (`self.Music`)))

(event `Activate`
  (bind _projector_screen (`self.Get screen widget`))
  (set `self.loop count` 0)
  (`AudioComponent.Play` (`self.ProjectorSound_Cue`) 0.0)
  (`AudioComponent.Play` (`self.Music`) 0.0)
  (`SkeletalMeshComponent.PlayAnimation` (`self.Projector Mesh`) "/Game/3D/Artificial/MovieProjector/AS_MovieProjector.AS_MovieProjector" true)
  (add `/Game/UI/Widgets/Game/World/Projector/Projector_Screen.Video end` _projector_screen (delegate `on video end`))
  (`/Game/UI/Widgets/Game/World/Projector/Projector_Screen.Init` _projector_screen (`self.Video`) :!label _label)
  (`self.play subtitles`)
  (`KismetSystemLibrary.Delay` 0.1)
  (`SceneComponent.SetHiddenInGame` (`self.Screen`) false false)
  (`SceneComponent.SetHiddenInGame` (`self.NS_Projector`) false false)
  (bind (_direction _opacity) (`Timeline|Timeline`)
    (:`Update`
      (`WidgetComponent.SetTintColorAndOpacity` (`self.Screen`) (`KismetMathLibrary.MakeColor` 1.0 1.0 1.0 _opacity)))))

(event `on video end`
  (bind _result (`/Engine/EditorBlueprintResources/StandardMacros.IncrementInt` (`self.loop count`))
    (:`  `
      (if (< _result (`self.Loops`))
        (goto _label)
        (else
          (`self.Deactivate`))))))

(event `start show text`
  (bind (_timeinterval _text) (break `/Game/Data/structs/Text_time` (`|GetArrayItem` (stale `play subtitles` _output_get))))
  (`/Game/UI/Widgets/Game/World/Projector/Projector_Screen.Update text` (`self.Get screen widget`) _text :!label _label_2)
  (bind (_min _max) (break `FloatInterval` _timeinterval))
  (set `self.current time` _min)
  (bind _returnvalue (- _max (`self.current time`)))
  (if (!= _returnvalue 0.0)
    (bind _returnvalue_2 (`KismetSystemLibrary.K2_SetTimerDelegate` (delegate `end show text`) _returnvalue))
    (set `self.end text timer` _returnvalue_2)
    (else
      (`/Game/UI/Widgets/Game/World/Projector/Projector_Screen.Clear text` (`self.Get screen widget`) :!label _label_3)
      (set `self.current time` _max)
      (`KismetArrayLibrary.Array_Remove` (`self.Subtitles buf`))
      (if (`KismetArrayLibrary.Array_IsNotEmpty` (stale `play subtitles` _output_get)) :!label _label_4
        (bind _returnvalue_3 (- _min (`self.current time`)))
        (if (!= _returnvalue_3 0.0)
          (bind _returnvalue_4 (`KismetSystemLibrary.K2_SetTimerDelegate` (delegate `start show text`) _returnvalue_3))
          (set `self.start text timer` _returnvalue_4)
          (else
            (goto _label_2)))))))

(event `end show text`
  (goto _label_3))

(event `play subtitles`
  (`KismetSystemLibrary.K2_ClearAndInvalidateTimerHandle` (`self.start text timer`))
  (`KismetSystemLibrary.K2_ClearAndInvalidateTimerHandle` (`self.end text timer`))
  (set `self.current time` 0.0)
  (bind _output_get (set `self.Subtitles buf` (`self.Subtitles`)))
  (goto _label_4))

(fn `Get screen widget`
  (returns (`Projector Screen` :type "/Game/UI/Widgets/Game/World/Projector/Projector_Screen Object Reference"))
  (return (cast `/Game/UI/Widgets/Game/World/Projector/Projector_Screen` (`WidgetComponent.GetWidget` (`self.Screen`)) :!pure true)))

(fn `UserConstructionScript`)