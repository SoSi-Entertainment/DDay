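; Black box recorder that stores timed movement frames (location, body angle, gun rotation, speed) and shots with hit info for later replay.
; Extract functions step through both arrays by index, re-basing frame times onto BornTime and returning shot times as intervals from the previous shot.
; Reset rewinds playback and applies a pending start-time offset, while clear functions trim history and flag it as coming from an old checkpoint.
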(fn `Add start time`
  (params (time :type "Float (double-precision)"))
  (set `self.Start time delta` (- time (`self.Born time`))))

(fn `Clear all Frames`
  (bind _shots (`self.Shots`))
  (set `self.From old checkpoint` true)
  (`KismetArrayLibrary.Array_Clear` (`self.Frames`))
  (bind _output_get (set `self.Shot buffer` (`|GetArrayItem` _shots (`KismetArrayLibrary.Array_LastIndex` _shots))))
  (`KismetArrayLibrary.Array_Clear` _shots)
  (`KismetArrayLibrary.Array_Add` _shots _output_get))

(fn `Clear past Frames`
  (set `self.From old checkpoint` true)
  (`/Engine/EditorBlueprintResources/StandardMacros.CompareInt` (`KismetArrayLibrary.Array_Length` (`self.Frames`)) 1
    (:`>`
      (for _ (range (+ (- (`self.Frame num`) 2) 1))
        (`KismetArrayLibrary.Array_Remove` (`self.Frames`)))
      (set `self.Frame num` 1)
      (for _ (range (+ (- (`self.Shot num`) 2) 1))
        (`KismetArrayLibrary.Array_Remove` (`self.Shots`)))
      (set `self.Shot num` 1))))

(fn `Extract Frame`
  (returns (Location :type "Vector Structure") (`Body angle` :type "Float (double-precision)") (Rotation :type "Rotator Structure") (Speed :type "Vector Structure") (Time :type "Float (double-precision)") (Done :type Boolean))
  (bind _output (`|GetArrayItem` (`self.Frames`) (`self.Frame num`)))
  (`/Engine/EditorBlueprintResources/StandardMacros.IsValid` _output
    (:`Is Valid`
      (bind _output_get (set `self.Frame bufer` _output))
      (`/Engine/EditorBlueprintResources/StandardMacros.IncrementInt` (`self.Frame num`)
        (:`  `
          (return (`/Game/Blueprints/recording/Frame_Info.Location` _output_get) (`/Game/Blueprints/recording/Frame_Info.Body angle` _output_get) (`/Game/Blueprints/recording/Frame_Info.Gun Rotation` _output_get) (`/Game/Blueprints/recording/Frame_Info.Speed` _output_get) (+ (`self.Born time`) (- (`/Game/Blueprints/recording/Frame_Info.Time` _output_get) (`self.Start time`))) true))))
    (:`Is Not Valid`
      (return (0.0 0.0 0.0) 0.0 (struct) (0.0 0.0 0.0) 0.0 false))))

(fn `Extract shot`
  (returns (extracted :type Boolean) (`shot time` :type "Float (double-precision)") (hit :type Boolean) (`Hits info` :type "Array of /Game/Blueprints/recording/Hit_Info Structure"))
  (locals (`prev shot  time` :type "Float (double-precision)"))
  (bind _output (`|GetArrayItem` (`self.Shots`) (`self.Shot num`)))
  (`/Engine/EditorBlueprintResources/StandardMacros.IsValid` _output
    (:`Is Valid`
      (bind _output_get (set `self.Shot buffer` _output))
      (`/Engine/EditorBlueprintResources/StandardMacros.CompareInt` (`self.Shot num`)
        (:`>`
          (set `local.prev shot  time` (`/Game/Blueprints/recording/Shot_Info.shot time` (`|GetArrayItem` (`self.Shots`) (- (`self.Shot num`) 1)))))
        (:`==`
          (set `local.prev shot  time` (`self.Start time`))))
      (`/Engine/EditorBlueprintResources/StandardMacros.IncrementInt` (`self.Shot num`)
        (:`  `
          (return true (- (`/Game/Blueprints/recording/Shot_Info.shot time` _output_get) (`local.prev shot  time`)) (`/Game/Blueprints/recording/Shot_Info.Is hit` _output_get) (`/Game/Blueprints/recording/Shot_Info.Hits` _output_get)))))
    (:`Is Not Valid`
      (return false 0.0 false))))

(fn `Finish writing`
  (bind _shots (`self.Shots`))
  (`KismetArrayLibrary.Array_Remove` _shots (`KismetArrayLibrary.Array_LastIndex` _shots)))

(fn `Get Root`
  (returns (location :type "Vector Structure") (`body rotation` :type "Rotator Structure"))
  (bind _output (`|GetArrayItem` (`self.Frames`)))
  (return (`/Game/Blueprints/recording/Frame_Info.Location` _output) (`KismetMathLibrary.MakeRotator` 0.0 0.0 (`/Game/Blueprints/recording/Frame_Info.Body angle` _output))))

(fn `Is Stillborn`
  (returns (Stillborn :type Boolean))
  (return (== (`KismetArrayLibrary.Array_Length` (`self.Frames`)) 1)))

(fn `New Shot`
  (returns (writing :type "/Game/Blueprints/recording/Shot_Info Object Reference"))
  (bind _returnvalue (`|GenericCreateObject` "/Game/Blueprints/recording/Shot_Info.Shot_Info_C"))
  (`KismetArrayLibrary.Array_Add` (`self.Shots`) _returnvalue)
  (return _returnvalue))

(fn `Reset`
  (set `self.Frame num` 0)
  (set `self.Start time` (+ (`self.Start time`) (`self.Start time delta`)))
  (set `self.Shot num` 0)
  (set `self.Start time delta` 0.0))

(fn `Save Frame`
  (params (Location :type "Vector Structure") (`Body angle` :type "Float (double-precision)") (Rotation :type "Rotator Structure") (Speed :type "Vector Structure") (Time :type "Float (double-precision)"))
  (bind _returnvalue (`|GenericCreateObject` "/Game/Blueprints/recording/Frame_Info.Frame_Info_C"))
  (set `/Game/Blueprints/recording/Frame_Info.Time` Time _returnvalue)
  (set `/Game/Blueprints/recording/Frame_Info.Location` Location _returnvalue)
  (set `/Game/Blueprints/recording/Frame_Info.Body angle` `Body angle` _returnvalue)
  (set `/Game/Blueprints/recording/Frame_Info.Gun Rotation` Rotation _returnvalue)
  (set `/Game/Blueprints/recording/Frame_Info.Speed` Speed _returnvalue)
  (`KismetArrayLibrary.Array_Add` (`self.Frames`) _returnvalue))