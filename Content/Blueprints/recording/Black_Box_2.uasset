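; Black Box recorder that stores movement steps and transform frames so they can be read back in order.
; Save Step appends pause and direction entries, while Save Frame appends rotation, location and shot flag entries, each as a newly constructed info object.
; The Extract functions return the next entry from their own index counter, with Done false when none is valid.
; Reset rewinds both counters without clearing the recorded arrays.
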(fn `Extract Frame`
  (returns (Rotation :type "Rotator Structure") (Location :type "Vector Structure") (Done :type Boolean) (Shot :type Boolean))
  (bind _output (`|GetArrayItem` (`self.Shots`) (`self.Shot num`)))
  (`/Engine/EditorBlueprintResources/StandardMacros.IsValid` _output
    (:`Is Valid`
      (bind _output_get (set `self.Shot bufer` _output))
      (`/Engine/EditorBlueprintResources/StandardMacros.IncrementInt` (`self.Shot num`)
        (:`  `
          (return (`/Game/Blueprints/recording/Frame_Info.Rotation` _output_get) (`/Game/Blueprints/recording/Frame_Info.Location` _output_get) true (`/Game/Blueprints/recording/Frame_Info.Shot` _output_get)))))
    (:`Is Not Valid`
      (return (struct) (0.0 0.0 0.0) false false))))

(fn `Extract Step`
  (returns (Pause :type "Float (double-precision)") (Direction :type "/Game/Blueprints/Navigation/Dirr Enum") (Done :type Boolean))
  (bind _output (`|GetArrayItem` (`self.Steps`) (`self.Step num`)))
  (`/Engine/EditorBlueprintResources/StandardMacros.IsValid` _output
    (:`Is Valid`
      (bind _output_get (set `self.Step bufer` _output))
      (`/Engine/EditorBlueprintResources/StandardMacros.IncrementInt` (`self.Step num`)
        (:`  `
          (return (`/Game/Blueprints/recording/Step_Info.Pause` _output_get) (`/Game/Blueprints/recording/Step_Info.Direction` _output_get) true))))
    (:`Is Not Valid`
      (return 0.0 "NewEnumerator4" false))))

(fn `Reset`
  (set `self.Step num` 0)
  (set `self.Shot num` 0))

(fn `Save Frame`
  (params (Rotation :type "Rotator Structure") (Location :type "Vector Structure") (Shot :type Boolean))
  (bind _returnvalue (`|GenericCreateObject` "/Game/Blueprints/recording/Frame_Info.Frame_Info_C"))
  (set `/Game/Blueprints/recording/Frame_Info.Shot` Shot _returnvalue)
  (set `/Game/Blueprints/recording/Frame_Info.Location` Location _returnvalue)
  (set `/Game/Blueprints/recording/Frame_Info.Rotation` Rotation _returnvalue)
  (`KismetArrayLibrary.Array_Add` (`self.Shots`) _returnvalue))

(fn `Save Step`
  (params (Pause :type "Float (double-precision)") (Direction :type "/Game/Blueprints/Navigation/Dirr Enum" :default "NewEnumerator4"))
  (bind _returnvalue (`|GenericCreateObject` "/Game/Blueprints/recording/Step_Info.Step_Info_C"))
  (set `/Game/Blueprints/recording/Step_Info.Pause` Pause _returnvalue)
  (set `/Game/Blueprints/recording/Step_Info.Direction` Direction _returnvalue)
  (`KismetArrayLibrary.Array_Add` (`self.Steps`) _returnvalue))