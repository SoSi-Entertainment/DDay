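; Enemy gun actor attached to a parent Base_Character that fires shells from its muzzle endpoint, gated by a cooldown.
; Fire optionally randomizes pitch for recoil, spawns the shell type, passes the target to Canon_Shell and reports whether it fired.
; Shot sound plays at location, unless a DDay_Controller override selects 2D playback; that override also scales volume.
; Helpers expose the muzzle location and an offset snipe point, found by temporarily shifting the endpoint.
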(event `cd delay`
  (set `self.on cd` true)
  (`KismetSystemLibrary.Delay` (`self.cd length`))
  (set `self.on cd` false))

(event `self.ReceiveBeginPlay`
  (bind _asbase_character (cast `/Game/Blueprints/Chars/Base_Character` (`self.GetParentActor` self)))
  (set `self.Body` _asbase_character))

(fn `Add recoil`
  (bind (_upangle _downangle) (break `/Game/Blueprints/Arms/Recoil_Angles` (`self.Recoil angles`)))
  (`self.K2_SetActorRotation` (`KismetMathLibrary.MakeRotator` (.roll (`self.K2_GetActorRotation`)) (`KismetMathLibrary.RandomFloatInRange` _downangle _upangle) (.yaw (`self.K2_GetActorRotation`)))))

(fn `Endpoint Location`
  (returns (Location :type "Vector Structure"))
  (return (`SceneComponent.K2_GetComponentLocation` (`self.end point`))))

(fn `Fire`
  (params (Target :type "Vector Structure") (`Generate Recoil` :type Boolean))
  (returns (Done :type Boolean))
  (bind _returnvalue (`self.K2_GetActorLocation`))
  (bind _shot_sound (`self.Shot Sound`))
  (if (`self.on cd`)
    (return false)
    (else
      (if `Generate Recoil`
        (`self.Add recoil`))
      (bind _returnvalue_2 (`|SpawnActorFromClass` (`self.shell type`) (`KismetMathLibrary.MakeTransform` (`SceneComponent.K2_GetComponentLocation` (`self.end point`)) (`SceneComponent.K2_GetComponentRotation` (`self.gun`))) "Undefined" "MultiplyWithRoot" (`self.GetParentActor` self) null))
      (bind _ascanon_shell (cast `/Game/Blueprints/Arms/Canon_Shell` _returnvalue_2)
        (:`then`
          (set `/Game/Blueprints/Arms/Canon_Shell.target` Target _ascanon_shell))
        (:`CastFailed`
          _))
      (`self.cd delay`)
      (bind _asdday_controller (cast `/Game/Blueprints/Controllers/DDay_Controller` (`Pawn.GetController` (`self.Body`)))
        (:`then`
          (bind _override_params (`/Game/Blueprints/Controllers/DDay_Controller.Get sound override` _asdday_controller))
          (bind (_2dsound _volumecoef) (break `/Game/Movies/Sound_Override` _override_params))
          (if _2dsound
            (`GameplayStatics.PlaySound2D` _shot_sound _volumecoef 1.0 0.0 null null)
            (else
              (`GameplayStatics.PlaySoundAtLocation` _shot_sound _returnvalue (struct) _volumecoef 1.0 0.0 null null null null))))
        (:`CastFailed`
          (`GameplayStatics.PlaySoundAtLocation` _shot_sound _returnvalue (struct) 1.0 1.0 0.0 null null null null)))
      (return true))))

(fn `SnipePoint Location`
  (returns (location :type "Vector Structure"))
  (bind _end_point (`self.end point`))
  (bind _returnvalue (`KismetMathLibrary.MakeVector` 0.0 (`self.Snipe point offset`)))
  (`SceneComponent.K2_AddRelativeLocation` _end_point _returnvalue false false)
  (bind _output_get (set `self.snipe loacation` (`SceneComponent.K2_GetComponentLocation` _end_point)))
  (`SceneComponent.K2_AddRelativeLocation` _end_point (`KismetMathLibrary.NegateVector` _returnvalue) false false)
  (return _output_get))

(fn `UserConstructionScript`)