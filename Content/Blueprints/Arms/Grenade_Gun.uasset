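; Grenade launcher weapon that fires a ballistic projectile toward a target location.
; Shoot refuses while the level win has started or during cooldown unless told to ignore it, otherwise it spawns the projectile, starts recoil and starts the cooldown timer.
; The projectile spawns at the gun endpoint with a normalized throw direction, the target location and the gun owner's speed.
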(fn `Shoot`
  (params (`Generate Spread` :type Boolean) (`shot info` :type "/Game/Blueprints/recording/Shot_Info Object Reference") (`ignore cd` :type Boolean) (`100%hit` :type Boolean) (`Target location` :type "Vector Structure") (`Add owner speed` :type Boolean) (`Hit Targets` :type "Array of /Game/Blueprints/Chars/Abstract/Base_Character Object Reference (by ref)"))
  (returns (Done :type Boolean))
  (bind _location (`self.Endpoint Location`))
  (if (not (`self.Inactive`))
    (if (`/Game/Blueprints/System/DDay_GameMode.Lvl Win started` (`/Game/Blueprints/System/Funtions/FunctionLibrary.Get GameMode Troops`))
      _
      (elif (and (`self.on cd`) (not (`local.ignore cd`)))
        _
        (else
          (bind _speed (`/Game/Blueprints/Vehicles/Components/GunOwner.Speed` (`self.Gun owner`)))
          (`|SpawnActorFromClass` "/Game/Blueprints/Arms/Shells/ballistic/ballistic.ballistic_C" (`KismetMathLibrary.MakeTransform` _location) "Undefined" "MultiplyWithRoot" (`self.Body`) 200.0 200.0 (`KismetMathLibrary.Normal` (- `Target location` _location)) _speed `Target location` null)
          (`self.Start recoil animation`)
          (`self.start cd timer`)
          (return true))))
    (return false)))

(fn `UserConstructionScript`
  (`parent.UserConstructionScript`))