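; Cannon shell projectile Blueprint that explodes on nearing its Target point, extending a parent class's Tick and Die logic.
; Tick checks the mesh's distance to Target; within a small radius it enables Sphere1 collision and, after a short Delay, calls Die.
; Die plays an explosion sound and spawns two Blast_bp actors differing in rotation and scale, then calls the parent.
; SpawnBlood places a flattened Blood_bp at the given actor's location.
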(event `self.ReceiveTick`
  (params (DeltaSeconds :type "Float (single-precision)"))
  (bind _shell_mesh (`self.Shell mesh`))
  (`parent.ReceiveTick` DeltaSeconds)
  (`/Engine/EditorBlueprintResources/StandardMacros.IsValid` _shell_mesh
    (:`Is Valid`
      (if (< (`KismetMathLibrary.Vector_Distance` (`self.target`) (`SceneComponent.K2_GetComponentLocation` _shell_mesh)) 100.0)
        (`PrimitiveComponent.SetCollisionEnabled` (`self.Sphere1`) "QueryAndPhysics")
        (`KismetSystemLibrary.Delay` 0.3)
        (`self.Die`)))))

(fn `Die`
  (bind _returnvalue (`SceneComponent.K2_GetComponentLocation` (`self.Shell mesh`)))
  (`GameplayStatics.PlaySoundAtLocation` "/Game/Movies/ShellExplosion_Cue.ShellExplosion_Cue" _returnvalue (struct) 1.0 1.0 0.0 null null null null)
  (`|SpawnActorFromClass` "/Game/Effects/blast_bp.blast_bp_C" (`KismetMathLibrary.MakeTransform` _returnvalue) "Undefined" "MultiplyWithRoot" null null)
  (`|SpawnActorFromClass` "/Game/Effects/blast_bp.blast_bp_C" (`KismetMathLibrary.MakeTransform` _returnvalue (struct :`Yaw` 60.0) (1.5 1.5 1.5)) "Undefined" "MultiplyWithRoot" null null)
  (`parent.Die`))

(fn `Spawn blood`
  (params (`Blood's owner` :type "/Game/Blueprints/Chars/Base_Character Object Reference"))
  (`|SpawnActorFromClass` "/Game/Effects/blood_bp.blood_bp_C" (`KismetMathLibrary.MakeTransform` (`self.K2_GetActorLocation` `Blood's owner`) (struct) (1.5 1.5 0.01)) "Undefined" "MultiplyWithRoot" null null))

(fn `UserConstructionScript`
  (`parent.UserConstructionScript`))