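; Gun smoke component that keeps a cooldown flag for smoking, enforcing a minimum interval.
; Updatetimer starts a one-shot timer of SmokeMinInterval and clears AlowedToSmoke, only when the stored timer's remaining time compares equal to zero.
; When the timer ends, DelayEnd sets the flag again and invalidates the handle.
; The graph only manages this gate and spawns no smoke itself.
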(event `Update timer`
  (`/Engine/EditorBlueprintResources/StandardMacros.CompareFloat` (`KismetSystemLibrary.K2_GetTimerRemainingTimeHandle` (`self.timer`))
    (:`==`
      (bind _returnvalue (`KismetSystemLibrary.K2_SetTimerDelegate` (delegate `delay end`) (`self.Smoke min Interval`)))
      (set `self.timer` _returnvalue)
      (set `self.alowed to smoke` false))))

(event `delay end`
  (set `self.alowed to smoke` true)
  (`KismetSystemLibrary.K2_InvalidateTimerHandle` (`self.timer`)))