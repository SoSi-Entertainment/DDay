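; Mortar gun weapon that throws TNT mines at a target location using an engineer throw animation.
; Shoot checks inactive state, level-win and cooldown, then starts the throw montage and cooldown timer.
; The montage's "throw" notify spawns a TNT_Mine at the skeleton's end socket with shell damage, substituting a range-limited target when out of range.
; An older spawn path and recoil call remain unexecuted, and Fall destroys the actor.
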(event `Start Throw process`
  (params (`target location` :type "Vector Structure"))
  (bind _notifyname (`|PlayMontage` (`self.gun skeleton`) "/Game/3D/Ally/main_guy/Engineer/Device/Animation/AS_engineer_TNT_device_Montage.AS_engineer_TNT_device_Montage" 2.5)
    (:`OnNotifyBegin`
      (if (== _notifyname "throw")
        (`self.Spawn ballistic` `target location`)))))

(fn `Endpoint Location`
  (returns (Location :type "Vector Structure"))
  (return (`SceneComponent.K2_GetComponentLocation` (`self.end point`))))

(fn `Fall`
  (`self.K2_DestroyActor`))

(fn `Shoot`
  (params (`Generate Spread` :type Boolean) (`shot info` :type "/Game/Blueprints/recording/Shot_Info Object Reference") (`ignore cd` :type Boolean) (`100%hit` :type Boolean) (`Target location` :type "Vector Structure") (`Add owner speed` :type Boolean) (`Hit Targets` :type "Array of /Game/Blueprints/System/Interfaces/Aimable Interface (by ref)") (`Is on screen` :type Boolean))
  (returns (Done :type Boolean))
  (if (not (`self.Inactive`))
    (if (`/Game/Blueprints/System/DDay_GameMode.Lvl Win started` (`/Game/Blueprints/System/Funtions/FunctionLibrary.Get GameMode Troops`))
      _
      (elif (and (`self.on cd`) (not (`local.ignore cd`)))
        _
        (else
          (`self.Start Throw process` `Target location`)
          (`self.start cd timer`)
          (return true))))
    (return false)))

(fn `Spawn ballistic`
  (params (`target location` :type "Vector Structure"))
  (bind _location (`self.Endpoint Location`))
  (`|SpawnActorFromClass` "/Game/Blueprints/Arms/Shells/ballistic/TNT_Mine.TNT_Mine_C" (`KismetMathLibrary.MakeTransform` (`SceneComponent.GetSocketLocation` (`self.gun skeleton`) "end")) "Undefined" "MultiplyWithRoot" (`self.body`) (`.Damage_4_92565BDC46D9DD7BC24E99895F525670` (break `/Game/Data/structs/Shell_params` (`self.Shell params`))) (select `bool` (> (`KismetMathLibrary.Vector_Distance2D` `target location` (`self.Endpoint Location`)) (`.Range_6_2DB35ABC4BD47F2073F3D69CB8CA5012` (break `/Game/Data/structs/Shell_params` (`self.Shell params`)))) :`false` `target location` :`true` (+ _location (* (`KismetMathLibrary.Normal` (- (`local.target location`) _location)) (`.Range_6_2DB35ABC4BD47F2073F3D69CB8CA5012` (break `/Game/Data/structs/Shell_params` (`self.Shell params`)))))) null))

(fn `UserConstructionScript`
  (`parent.UserConstructionScript`))