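; Gun actor held by a parent GunOwner that fires team-tagged shell actors for troop characters.
; Shoot checks cooldown and raise/lower state, applies random spread, then spawns the shell, cartridge and on-screen recoil, flash, smoke and sound.
; Vertical spread is trench-aware: cover traces choose a mode, then downward angle-stepped traces feed a curve-weighted chance of replacing default angles.
; It also handles raise/lower montages, outline, opacity and dropping as a physics object.
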(event `start cd timer`
  (set `self.on cd` true)
  (`KismetSystemLibrary.Delay` (`self.cd length`))
  (set `self.on cd` false))

(event `self.ReceiveBeginPlay`
  (bind _returnvalue (`self.GetParentActor` self))
  (`|ExecutionSequence`
    (:`then_0`
      (`self.Setup dynamic material`))
    (:`then_1`
      (bind _asbase_character (cast `/Game/Blueprints/Chars/Abstract/Base_Character` _returnvalue))
      (set `self.Body` _asbase_character))
    (:`then_2`
      (bind _asgun_owner (cast `/Game/Blueprints/Vehicles/Components/GunOwner` _returnvalue))
      (set `self.Gun owner` _asgun_owner))))

(event `Stop recoil animation`)

(event `Start recoil animation`
  (`|PlayMontage` (`self.gun skeleton`) (`self.Animation montage`)))

(event `set gun down`
  (params (down :type Boolean))
  (bind _gun_skeleton (`self.gun skeleton`))
  (bind _output_get (set `self.last required downed` down))
  (if (!= (`self.current downed`) _output_get)
    (if (not (`self.down/up process`))
      (bind _output_get_2 (set `self.current downed` down))
      (set `self.down/up process` true)
      (if _output_get_2
        (bind _notifyname (`|PlayMontage` _gun_skeleton "/Game/Anim/Guns/rifle_down_m.rifle_down_m")
          (:`OnNotifyBegin`
            (if (== _notifyname "End")
              (`KismetSystemLibrary.Delay` 0.1 :!label _label)
              (set `self.down/up process` false)
              (if (!= (`self.current downed`) (`self.last required downed`))
                (`self.set gun down` (`self.last required downed`))))))
        (else
          (bind _notifyname_2 (`|PlayMontage` _gun_skeleton "/Game/Anim/Guns/rifle_up_m.rifle_up_m")
            (:`OnNotifyBegin`
              (if (== _notifyname_2 "End")
                (goto _label)))))))))

(fn `Apply Spread`
  (params (`Spread angles` :type "/Game/Blueprints/Arms/Hands/Direction_Values Structure"))
  (bind (_horisontal _vertical) (break `/Game/Blueprints/Arms/Hands/Direction_Values` `Spread angles`))
  (`SceneComponent.K2_SetRelativeRotation` (`self.Spread Layer`) (`KismetMathLibrary.MakeRotator` 0.0 _vertical _horisontal) false false))

(fn `Calculate spread mode`
  (params (Target :type "/Game/Blueprints/System/Interfaces/Aimable Interface"))
  (returns (`Spread mode` :type "/Game/Data/enums/Spread_Mode Enum"))
  (locals (`leg barier type` :type "Array of EObjectTypeQuery Enum"))
  (bind _location (`/Game/Blueprints/System/Interfaces/Aimable.Get Location` Target))
  (bind _tile (`/Game/Blueprints/System/Funtions/Tile_Functions.Get Aboba Under new` _location))
  (bind _tile_2 (`/Game/Blueprints/System/Funtions/Tile_Functions.Get Aboba Under new` (`self.K2_GetActorLocation` (`self.Body`))))
  (bind _location_2 (`/Game/Blueprints/System/Interfaces/Aimable.Get Downside location` Target))
  (bind (_outhit _returnvalue) (`KismetSystemLibrary.LineTraceSingleForObjects` :`Start` (`self.Snipe Point Location New`) :`End` _location_2 :`ObjectTypes` (`local.leg barier type`) :`TraceColor` (struct :`G` 0.756592 :`B` 1.0 :`A` 1.0) :`TraceHitColor` (struct :`R` 1.0 :`G` 0.921747 :`A` 1.0) :`DrawTime` 0.5))
  (bind _returnvalue_2 (and _returnvalue (`.bSuccess` (cast `/Game/3D/platforms/Tile_2/Trench/Trench` (`/Game/3D/platforms/Tile.Get platform` _tile) :!pure true))))
  (return (select `bool` (and _returnvalue_2 (`.bSuccess` (cast `/Game/3D/platforms/Tile_2/Trench/Trench` (`/Game/3D/platforms/Tile.Get platform` _tile_2) :!pure true))) :`false` (select `bool` _returnvalue_2 :`false` "NewEnumerator0" :`true` "NewEnumerator1" :!type "/Game/Data/enums/Spread_Mode Enum") :`true` "NewEnumerator2")))

(fn `Calculate spread mode no target`
  (params (`target location` :type "Vector Structure"))
  (returns (`Spread mode` :type "/Game/Data/enums/Spread_Mode Enum"))
  (locals (`leg barier type` :type "Array of EObjectTypeQuery Enum"))
  (bind _tile (`/Game/Blueprints/System/Funtions/Tile_Functions.Get Aboba Under new` (`self.K2_GetActorLocation` (`self.Body`))))
  (bind _tile_2 (`/Game/Blueprints/System/Funtions/Tile_Functions.Get Aboba Under new` (+ `target location` (0.0 0.0 50.0))))
  (bind (_outhit _returnvalue) (`KismetSystemLibrary.LineTraceSingleForObjects` :`Start` (`self.Rotation Point`) :`End` (+ `target location` (0.0 0.0 5.0)) :`ObjectTypes` (`local.leg barier type`) :`TraceColor` (struct :`G` 0.756592 :`B` 1.0 :`A` 1.0) :`TraceHitColor` (struct :`R` 1.0 :`G` 0.921747 :`A` 1.0) :`DrawTime` 10.0))
  (bind _returnvalue_2 (and _returnvalue (`.bSuccess` (cast `/Game/3D/platforms/Tile_2/Trench/Trench` (`/Game/3D/platforms/Tile.Get platform` _tile_2) :!pure true))))
  (return (select `bool` (and _returnvalue_2 (`.bSuccess` (cast `/Game/3D/platforms/Tile_2/Trench/Trench` (`/Game/3D/platforms/Tile.Get platform` _tile) :!pure true))) :`false` (select `bool` _returnvalue_2 :`false` "NewEnumerator0" :`true` "NewEnumerator1" :!type "/Game/Data/enums/Spread_Mode Enum") :`true` "NewEnumerator2")))

(fn `Drop cartridge`
  (params (drop :type Boolean))
  (bind _gun_skeleton (`self.gun skeleton`))
  (bind (_type _speed _speedrandomcoef _backspeed _backrandomadd) (break `/Game/Data/structs/Cartridge_Settings` (`self.Cartridge settings`)))
  (if drop
    (bind _returnvalue (`|SpawnActorFromClass` _type (`KismetMathLibrary.MakeTransform` (`SceneComponent.K2_GetComponentLocation` (`self.Cartridge drop`)) (`SceneComponent.K2_GetComponentRotation` _gun_skeleton)) "Undefined" "MultiplyWithRoot" null null))
    (`/Engine/EditorBlueprintResources/StandardMacros.IsValid` _returnvalue
      (:`Is Valid`
        (bind _speed_2 (`/Game/Blueprints/Vehicles/Components/GunOwner.Speed` (`self.Gun owner`)))
        (`PrimitiveComponent.SetPhysicsLinearVelocity` (`/Game/Blueprints/Arms/Abobus/Cartridge.CartridgeMesh` _returnvalue) (- (+ (* _speed_2 0.9) (* (`KismetMathLibrary.Conv_RotatorToVector` (`SceneComponent.K2_GetComponentRotation` (`self.Cartridge drop`))) (`KismetMathLibrary.RandomFloatInRange` _speed (* _speed _speedrandomcoef)))) (* (`SceneComponent.GetRightVector` _gun_skeleton) (`KismetMathLibrary.RandomFloatInRange` (- _backspeed _backrandomadd) (+ _backspeed _backrandomadd)))) false "None")))))

(fn `End range point`
  (returns (Location :type "Vector Structure"))
  (return (+ (`self.Endpoint Location`) (* (`self.Get Forward Unspread`) (`.Range_6_2DB35ABC4BD47F2073F3D69CB8CA5012` (break `/Game/Data/structs/Shell_params` (`self.Shell params`)))))))

(fn `Endpoint Location`
  (returns (Location :type "Vector Structure"))
  (return (`SceneComponent.GetSocketLocation` (`self.gun skeleton`) "end")))

(fn `Fall`
  (locals (`trace for fall` :type "Array of EObjectTypeQuery Enum"))
  (bind _point_location (`self.Rotation Point`))
  (bind _gun_skeleton (`self.gun skeleton`))
  (bind _stream (`/Game/Blueprints/Chars/Abstract/Base_Character.Get current run stream` (`self.Get character`)))
  (bind _returnvalue (`KismetMathLibrary.RandomFloatInRangeFromStream` _stream -50.0 50.0))
  (`self.Hide arms`)
  (if (`PrimitiveComponent.K2_IsPhysicsCollisionEnabled` (`self.gun skeleton`))
    _
    (elif (`self.Stationary`)
      _
      (elif (> (`KismetSystemLibrary.GetGameTimeInSeconds`) 0.5)
        (`|ExecutionSequence`
          (:`then_0`
            (`self.Stop recoil animation`)
            (`PrimitiveComponent.SetCollisionEnabled` _gun_skeleton "QueryAndPhysics" :!label _label)
            (`PrimitiveComponent.SetSimulatePhysics` _gun_skeleton true))
          (:`then_1`
            (`PrimitiveComponent.AddImpulse` (`self.gun skeleton`) (+ (* (`SceneComponent.GetRightVector` (`self.gun skeleton`)) -100.0) (`KismetMathLibrary.MakeVector` _returnvalue _returnvalue (`KismetMathLibrary.RandomFloatInRangeFromStream` _stream 100.0 200.0))) "None" false)))
        (else
          (`self.K2_AddActorLocalRotation` (struct :`Roll` 90.0))
          (`SceneComponent.K2_AddLocalOffset` (`self.gun skeleton`) (`KismetMathLibrary.MakeVector` 0.0 -50.0 (+ (* (.z (`KismetMathLibrary.InverseTransformLocation` (`self.GetTransform` (`self.Get character`)) (`self.Rotation Point`))) -1.0) 20.0)) false false)
          (bind _outhit (`KismetSystemLibrary.LineTraceSingleForObjects` _point_location (- _point_location (0.0 0.0 200.0)) (`local.trace for fall`)))
          (`SceneComponent.K2_AddWorldOffset` (`self.gun skeleton`) (`KismetMathLibrary.MakeVector` 0.0 0.0 (- (`self.high to tp fall on start`) (`.Distance` (`GameplayStatics.BreakHitResult` _outhit)))) false false)
          (goto _label))))))

(fn `Get character`
  (returns (Character :type "/Game/Blueprints/Chars/Abstract/Base_Character Object Reference"))
  (return (`self.Body`)))

(fn `Get Forward Unspread`
  (returns (`Forward vector` :type "Vector Structure"))
  (return (`self.GetActorForwardVector`)))

(fn `Get range`
  (returns (`range distance` :type "Float (double-precision)"))
  (return (`.Range_6_2DB35ABC4BD47F2073F3D69CB8CA5012` (break `/Game/Data/structs/Shell_params` (`self.Shell params`)))))

(fn `Hide arms`
  (`SkinnedMeshComponent.HideBoneByName` (`self.gun skeleton`) "hands" "PBO_None"))

(fn `Init settings`
  (params (`Unit stats` :type "/Game/Data/structs/Balance_State Structure"))
  (bind (_price _health _speed _cd _bulletdamage _bulletspeed _bulletrange) (break `/Game/Data/structs/Balance_State` `Unit stats`))
  (set `self.cd length` _cd)
  (set `self.Shell params` (make `/Game/Data/structs/Shell_params` (`KismetMathLibrary.Conv_IntToDouble` _bulletspeed) _bulletdamage (`KismetMathLibrary.Conv_IntToDouble` _bulletrange))))

(fn `Left hand location`
  (returns (location :type "Vector Structure"))
  (return (`SceneComponent.K2_GetComponentLocation` (`self.left hand point`))))

(fn `Play shoot sound`
  (locals (`sound stats` :type "/Game/Sounds/Sound_Override Structure"))
  (bind _shot_sound (`self.Shot Sound`))
  (bind _body (`self.Body`))
  (`/Engine/EditorBlueprintResources/StandardMacros.IsValid` _body
    (:`Is Valid`
      (bind _astroops_controller_i (cast `/Game/Blueprints/Controllers/Troops_Controller_I` (`Pawn.GetController` _body)))
      (bind _override_params (`/Game/Blueprints/Controllers/Troops_Controller_I.Get sound override` _astroops_controller_i))
      (bind _output_get (set `local.sound stats` _override_params)))
    (:`Is Not Valid`
      (bind _player (`/Game/Blueprints/Vehicles/Components/GunOwner.Is player` (`self.Gun owner`)))
      (set `local.sound stats` (make `/Game/Sounds/Sound_Override` _player))))
  (bind (_2dsound _volumecoef) (break `/Game/Sounds/Sound_Override` _output_get))
  (if _2dsound
    (`GameplayStatics.PlaySound2D` _shot_sound _volumecoef 1.0 0.0 null null)
    (else
      (`GameplayStatics.PlaySoundAtLocation` _shot_sound (`self.K2_GetActorLocation`) (struct) _volumecoef 1.0 0.0 null null null null))))

(fn `Record shot_info`
  (params (`Shot info` :type "/Game/Blueprints/recording/Shot_Info Object Reference") (`spread angles` :type "/Game/Blueprints/Arms/Hands/Direction_Values Structure"))
  (`/Engine/EditorBlueprintResources/StandardMacros.IsValid` `Shot info`
    (:`Is Valid`
      (set `/Game/Blueprints/recording/Shot_Info.shot time` (`KismetSystemLibrary.GetGameTimeInSeconds`) `Shot info`)
      (set `/Game/Blueprints/recording/Shot_Info.spread angles` `spread angles` `Shot info`))))

(fn `Rotation Point`
  (returns (`Point location` :type "Vector Structure"))
  (return (`self.K2_GetActorLocation`)))

(fn `Set gun visibility`)

(fn `Set outline`
  (params (outlined :type Boolean) (stencil :type Integer))
  (bind _gun_skeleton (`self.gun skeleton`))
  (`PrimitiveComponent.SetRenderCustomDepth` _gun_skeleton outlined)
  (`PrimitiveComponent.SetCustomDepthStencilValue` _gun_skeleton stencil))

(fn `Set transperent`
  (params (Alfa :type "Float (single-precision)"))
  (`MaterialInstanceDynamic.SetScalarParameterValue` (`self.Dynamic material`) "Opacity" Alfa))

(fn `Set vert recoil angle`
  (params (angle :type "Float (double-precision)"))
  (bind _gun_skeleton (`self.gun skeleton`))
  (`SceneComponent.K2_SetRelativeRotation` _gun_skeleton (`KismetMathLibrary.MakeRotator` (* angle -1.0) (.pitch (`SceneComponent.RelativeRotation` _gun_skeleton)) (.yaw (`SceneComponent.RelativeRotation` _gun_skeleton))) false true))

(fn `Setup dynamic material`
  (bind _returnvalue (`PrimitiveComponent.CreateDynamicMaterialInstance` (`self.gun skeleton`) 0 null "None"))
  (set `self.Dynamic material` _returnvalue))

(fn `Shoot`
  (params (`Generate Spread` :type Boolean) (`shot info` :type "/Game/Blueprints/recording/Shot_Info Object Reference") (`ignore cd` :type Boolean) (`100%hit` :type Boolean) (`Target location` :type "Vector Structure") (`Add owner speed` :type Boolean) (`Hit Targets` :type "Array of /Game/Blueprints/System/Interfaces/Aimable Interface (by ref)") (`Is on screen` :type Boolean :default true))
  (returns (Done :type Boolean))
  (if (`self.Inactive`)
    _
    (elif (`/Game/Blueprints/System/DDay_GameMode.Lvl Win started` (`/Game/Blueprints/System/Funtions/FunctionLibrary.Get GameMode Troops`))
      (return false)
      (elif (and (`self.on cd`) (not (`local.ignore cd`)))
        (return false)
        (elif (`self.down/up process`)
          (return false)
          (elif (`self.current downed`)
            (return false)
            (else
              (`|ExecutionSequence`
                (:`then_0`
                  (if (`local.Generate Spread`)
                    (bind _vertical_spread (`self.Update Spread` (`|GetArrayItem` (`local.Hit Targets`)) (`local.Target location`)))
                    (bind _horisontal_spread (`self.Update Horisontal spread`))
                    (bind _output_get (set `self.Current spread` (make `/Game/Blueprints/Arms/Hands/Direction_Values` _horisontal_spread _vertical_spread)))
                    (`self.Apply Spread` _output_get)))
                (:`then_1`
                  (`self.Record shot_info` (`local.shot info`) (`self.Current spread`))
                  (`|ExecutionSequence`
                    (:`then_0`
                      (if (`local.Is on screen`)
                        (`self.Start recoil animation`)))
                    (:`then_1`
                      (`self.Spawn shell` (`local.shot info`) (`local.100%hit`) (`local.Add owner speed`) (`local.Hit Targets`) (`local.Target location`) (`local.Is on screen`))
                      (`self.Drop cartridge` true)
                      (`|ExecutionSequence`
                        (:`then_0`
                          (if (`local.Is on screen`)
                            (`self.Spawn fire`)
                            (`self.Spawn smoke`)
                            (`self.Play shoot sound`)))
                        (:`then_1`
                          (`self.start cd timer`)
                          (`self.Shoot event`)
                          (return true))))))))))))))

(fn `Snipe Point Location New`
  (returns (location :type "Vector Structure"))
  (return (`self.K2_GetActorLocation`)))

(fn `Snipe Point Location Old`
  (returns (location :type "Vector Structure"))
  (bind _end_point (`self.end point`))
  (bind _returnvalue (`KismetMathLibrary.MakeVector` 0.0 (`self.Snipe point offset`)))
  (`SceneComponent.K2_AddRelativeLocation` _end_point _returnvalue false false)
  (bind _output_get (set `self.snipe loacation` (`SceneComponent.K2_GetComponentLocation` _end_point)))
  (`SceneComponent.K2_AddRelativeLocation` _end_point (`KismetMathLibrary.NegateVector` _returnvalue) false false)
  (return _output_get))

(fn `Spawn fire`
  (bind _speed (`/Game/Blueprints/Vehicles/Components/GunOwner.Speed` (`self.Gun owner`)))
  (bind _returnvalue (`|SpawnActorFromClass` "/Game/Effects/FireStart/fire_start_bp.fire_start_bp_C" (`KismetMathLibrary.MakeTransform` (`self.Endpoint Location`) (`KismetMathLibrary.MakeRotator` (+ (.roll (`SceneComponent.K2_GetComponentRotation` (`self.gun skeleton`))) 90.0) (.pitch (`SceneComponent.K2_GetComponentRotation` (`self.gun skeleton`))) (.yaw (`SceneComponent.K2_GetComponentRotation` (`self.gun skeleton`)))) (`KismetMathLibrary.Conv_DoubleToVector` (`self.Fire Size`))) "Undefined" "MultiplyWithRoot" null _speed (`self.Single bullet`) null))
  (`self.K2_AttachToComponent` _returnvalue (`self.gun skeleton`) "end" "KeepWorld" "KeepWorld" "KeepWorld" false))

(fn `Spawn shell`
  (params (`Shot info` :type "/Game/Blueprints/recording/Shot_Info Object Reference") (`100%hit` :type Boolean) (`Add owner speed` :type Boolean) (`Hit Targets` :type "Array of /Game/Blueprints/System/Interfaces/Aimable Interface") (`Clone target loc` :type "Vector Structure") (`Is on screen` :type Boolean :default true))
  (locals (teamable :type "/Game/Blueprints/System/Interfaces/Teamable Interface"))
  (bind _body (`self.Body`))
  (bind _result (`/Engine/EditorBlueprintResources/StandardMacros.IncrementInt` (`self.shell count`))
    (:`  `
      (bind _speed (`/Game/Blueprints/Vehicles/Components/GunOwner.Speed` (`self.Gun owner`)))
      (`|ExecutionSequence`
        (:`then_0`
          (bind _asteamable (cast `/Game/Blueprints/System/Interfaces/Teamable` _body)
            (:`then`
              (set `local.teamable` _asteamable))
            (:`CastFailed`
              (bind _asteamable_2 (cast `/Game/Blueprints/System/Interfaces/Teamable` (`self.GetParentActor` self)))
              (set `local.teamable` _asteamable_2))))
        (:`then_1`
          (bind _team (`/Game/Blueprints/System/Interfaces/Teamable.Get Team` (`local.teamable`)))
          (`|SpawnActorFromClass` (`self.shell type`) (`KismetMathLibrary.MakeTransform` (`self.Endpoint Location`) (`SceneComponent.K2_GetComponentRotation` (`self.gun skeleton`))) "Undefined" "MultiplyWithRoot" (select `bool` (`KismetSystemLibrary.IsValid` _body) :`false` (`self.GetParentActor`) :`true` _body :!type "Actor Object Reference") _team (`local.Shot info`) (`self.Shell params`) _speed (`local.100%hit`) _result (`local.Add owner speed`) (`self.impulse strength`) (`self.Body`) (`local.Hit Targets`) (`local.Clone target loc`) (`local.Is on screen`) null))))))

(fn `Spawn smoke`
  (bind _gun_smoker_component (`self.Gun_Smoker_Component`))
  (if (`/Game/Blueprints/Arms/Gun_Components/Gun_Smoker_Component.alowed to smoke` _gun_smoker_component)
    (`/Game/Blueprints/Arms/Gun_Components/Gun_Smoker_Component.Update timer` _gun_smoker_component)
    (`|SpawnActorFromClass` (`self.Shot smoke type`) (`KismetMathLibrary.MakeTransform` (`self.Endpoint Location`) (`SceneComponent.K2_GetComponentRotation` (`self.gun skeleton`))) "Undefined" "MultiplyWithRoot" (`self.Body`) null)))

(fn `Update Horisontal spread`
  (returns (`Horisontal spread` :type "Float (double-precision)"))
  (bind (_upangle _downangle) (break `/Game/Data/structs/Spread_Angles` (`self.Horisontal Spread angles`)))
  (return (`KismetMathLibrary.RandomFloatInRange` _downangle _upangle)))

(fn `Update Spread`
  (params (`Shoot target` :type "/Game/Blueprints/System/Interfaces/Aimable Interface") (`target location` :type "Vector Structure"))
  (returns (`Vertical Spread` :type "Float (double-precision)"))
  (locals (`Trace types` :type "Array of EObjectTypeQuery Enum") (`Trace down angle` :type Integer :default 10) (`leg barier type` :type "Array of EObjectTypeQuery Enum") (`spread mode` :type "/Game/Data/enums/Spread_Mode Enum" :default "NewEnumerator0") (`Last angle trace hit` :type "HitResult Structure"))
  (bind _location (`self.Snipe Point Location New`))
  (bind _point_location (`self.Rotation Point`))
  (bind _returnvalue (`self.GetActorUpVector`))
  (bind _point_location_2 (`self.Rotation Point`))
  (bind _spread_mode (`local.spread mode`))
  (bind _shoot_target (`local.Shoot target`))
  (bind (_upangle _downangle) (break `/Game/Data/structs/Spread_Angles` (`self.Default Spread angles`)))
  (bind _returnvalue_2 (`|EnumEquality` (`/Game/Blueprints/Chars/Abstract/Base_Character.Unit Variation` (`self.Body`)) "NewEnumerator0"))
  (`/Game/Blueprints/System/Funtions/Macro_Library.Is Valid I` `Shoot target`
    (:`Is Valid`
      (bind _location_2 (`/Game/Blueprints/System/Interfaces/Aimable.Get Target Location` _shoot_target))
      (bind (_forced _up_point _down_point) (`/Game/Blueprints/System/Interfaces/Aimable.Is Forced high Interval` _shoot_target))
      (if _forced
        (bind _returnvalue_3 (- _location_2 _point_location_2))
        (return (`KismetMathLibrary.RandomFloatInRange` (`KismetMathLibrary.FMax` _downangle (- (`/Game/Blueprints/System/Funtions/FunctionLibrary.Angle between vectors signed` _returnvalue_3 _returnvalue (- _point_location_2 _down_point)) 180.0)) (`KismetMathLibrary.FMin` _upangle (`/Game/Blueprints/System/Funtions/FunctionLibrary.Angle between vectors signed` _returnvalue_3 _returnvalue (- _up_point _point_location_2)))))
        (else
          (bind _spread_mode_2 (`self.Calculate spread mode` _shoot_target))
          (set `local.spread mode` _spread_mode_2))))
    (:`Is Not Valid`
      (bind _spread_mode_3 (`self.Calculate spread mode no target` `target location`))
      (set `local.spread mode` _spread_mode_3)))
  (switch `/Game/Data/enums/Spread_Mode` _spread_mode
    (:`NewEnumerator0`
      (`KismetArrayLibrary.Array_RemoveItem` (`local.Trace types`) "ObjectTypeQuery7"))
    (:`NewEnumerator1`
      _)
    (:`NewEnumerator2`
      _))
  (for _index (range (+ (`local.Trace down angle`) 1))
    (`/Game/Blueprints/System/Funtions/Macro_Library.Is Valid I` (`local.Shoot target`)
      (:`Is Valid`
        (bind _returnvalue_4 (`KismetMathLibrary.Conv_IntToDouble` _index))
        (bind (_outhit _returnvalue_5) (`KismetSystemLibrary.LineTraceSingleByProfile` :`Start` _point_location :`End` (+ _point_location (`KismetMathLibrary.RotateAngleAxis` (- _location_2 _point_location) _returnvalue_4 (`self.GetActorRightVector`))) :`ProfileName` "Aim" :`DrawTime` 0.5))
        (set `local.Last angle trace hit` _outhit)
        (if _returnvalue_5
          (break)))
      (:`Is Not Valid`
        (bind (_outhit_2 _returnvalue_6) (`KismetSystemLibrary.LineTraceSingleByProfile` :`Start` _location :`End` (+ _location (`KismetMathLibrary.RotateAngleAxis` (* (`KismetMathLibrary.Normal` (- (`/Game/Blueprints/Controllers/Player_Controller.Get Plane Aim Location ` (`/Game/Blueprints/System/Funtions/FunctionLibrary.Get PlayerController Troops`)) _location)) (`.Range_6_2DB35ABC4BD47F2073F3D69CB8CA5012` (break `/Game/Data/structs/Shell_params` (`self.Shell params`)))) _returnvalue_4 (`self.GetActorRightVector`))) :`ProfileName` "Aim" :`DrawTime` 0.5))
        (set `local.Last angle trace hit` _outhit_2)
        (if _returnvalue_6
          (break)))))
  (bind _returnvalue_7 (* (`CurveFloat.GetFloatValue` (`self.Trench spread curve`) (`KismetMathLibrary.Conv_IntToDouble` _index)) (select `/Game/Data/enums/Spread_Mode` _spread_mode :`NewEnumerator0` (`KismetMathLibrary.SelectFloat` 0.0 1.0 _returnvalue_2) :`NewEnumerator1` (`KismetMathLibrary.SelectFloat` 0.0 1.0 _returnvalue_2) :`NewEnumerator2` (`KismetMathLibrary.SelectFloat` 0.0 (`self.Trench to trench coef`) _returnvalue_2)) (`self.Gun spread coef`)))
  (`/Game/Blueprints/Chars/Abstract/Base_Character.Say` (`self.Get character`) (`KismetStringLibrary.Concat_StrStr` (`KismetStringLibrary.GetSubstring` (`KismetStringLibrary.Conv_DoubleToString` _returnvalue_7) 0 4) " / " (`|GetEnumeratorNameAsString` _spread_mode)) 2.0)
  (bind _returnvalue_8 (* (`KismetMathLibrary.Conv_IntToDouble` _index) -1.0))
  (bind (_upangle_2 _downangle_2) (break `/Game/Data/structs/Spread_Angles` (select `bool` (`KismetMathLibrary.RandomBoolWithWeight` _returnvalue_7) :`false` (`self.Default Spread angles`) :`true` (make `/Game/Data/structs/Spread_Angles` _returnvalue_8 (- _returnvalue_8 1.0)))))
  (return (`KismetMathLibrary.RandomFloatInRange` _downangle_2 _upangle_2)))

(fn `UserConstructionScript`)