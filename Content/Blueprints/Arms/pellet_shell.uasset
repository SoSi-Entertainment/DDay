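; Pellet shell projectile that fans out into a multi-pellet spread when it spawns.
; On BeginPlay, an origin pellet spawns a copy of Pellet_shell for each PelletsAngles entry, rotated by that entry's deviations (horizontal as yaw, vertical as roll).
; Copies inherit owner, team, shell params and parent speed, with OriginPellet off to prevent recursive spawning.
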(event `self.ReceiveBeginPlay`
  (`parent.ReceiveBeginPlay`)
  (if (`self.Origin pellet`)
    (for _array_element (`self.Pellets angles`)
      (bind (_horizontaldeviation _verticaldeviation) (break `/Game/Data/structs/Shell_angle_deviation` _array_element))
      (`|SpawnActorFromClass` "pellet_shell_C" (`KismetMathLibrary.MakeTransform` (.location (`self.GetTransform`)) (`KismetMathLibrary.ComposeRotators` (.rotation (`self.GetTransform`)) (`KismetMathLibrary.MakeRotator` _verticaldeviation 0.0 _horizontaldeviation)) (.scale (`self.GetTransform`))) "Undefined" "MultiplyWithRoot" (`self.GetOwner`) false (`self.Team`) (`self.shell params`) (`self.Parent speed`) null))))

(fn `UserConstructionScript`
  (`parent.UserConstructionScript`))