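; Shield gun is an arm Blueprint that carries a Shield as a child actor in place of a firing weapon.
; Its Shoot function does nothing and returns false.
; Setup dynamic material creates a dynamic material instance on the child Shield's Cube mesh and stores it in DynamicMaterial.
; The event graph and construction script add no logic of their own.
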(fn `Setup dynamic material`
  (bind _returnvalue (`PrimitiveComponent.CreateDynamicMaterialInstance` (`/Game/Blueprints/Abilities/Shield.Cube` (cast `/Game/Blueprints/Abilities/Shield` (`ChildActorComponent.ChildActor` (`self.ChildActor`)) :!pure true)) 0 null "None"))
  (set `self.Dynamic material` _returnvalue))

(fn `Shoot`
  (params (`Generate Spread` :type Boolean) (`shot info` :type "/Game/Blueprints/recording/Shot_Info Object Reference") (`ignore cd` :type Boolean) (`100%hit` :type Boolean) (`Target location` :type "Vector Structure") (`Add owner speed` :type Boolean) (`Hit Targets` :type "Array of /Game/Blueprints/Chars/Abstract/Base_Character Object Reference (by ref)"))
  (returns (Done :type Boolean))
  (return false))

(fn `UserConstructionScript`
  (`parent.UserConstructionScript`))