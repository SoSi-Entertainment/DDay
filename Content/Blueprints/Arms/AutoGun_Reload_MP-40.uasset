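; MP-40 automatic gun Blueprint that adds a magazine and timed reload on top of its parent weapon's shooting.
; The magazine fills on BeginPlay, and the Shoot override calls the parent while rounds remain, spending one only when that shot succeeds.
; Shooting on an empty magazine returns false and triggers Reloadmagazine, which refills to full after a Delay, with no reserve ammo involved.
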(event `self.ReceiveBeginPlay`
  (`parent.ReceiveBeginPlay`)
  (set `self.Bullets in magazine` (`self.Magazine size`)))

(event `Reload magazine`
  (`KismetSystemLibrary.Delay` (`self.Magazine Reload time`))
  (set `self.Bullets in magazine` (`self.Magazine size`)))

(fn `Shoot`
  (params (`Generate Spread` :type Boolean) (`shot info` :type "/Game/Blueprints/recording/Shot_Info Object Reference") (`ignore cd` :type Boolean) (`100%hit` :type Boolean) (`Target location` :type "Vector Structure") (`Add owner speed` :type Boolean) (`Hit Targets` :type "Array of /Game/Blueprints/System/Interfaces/Aimable Interface (by ref)") (`Is on screen` :type Boolean))
  (returns (Done :type Boolean))
  (`/Engine/EditorBlueprintResources/StandardMacros.CompareInt` (`self.Bullets in magazine`)
    (:`>`
      (bind _done (`parent.Shoot` `Generate Spread` `shot info` `ignore cd` `100%hit` `Target location` `Add owner speed` `Hit Targets` true))
      (if _done
        (`/Engine/EditorBlueprintResources/StandardMacros.DecrementInt` (`self.Bullets in magazine`)
          (:`  `
            _)))
      (return _done))
    (:`==`
      (`self.Reload magazine`)
      (return false))))

(fn `UserConstructionScript`
  (`parent.UserConstructionScript`))