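; Controller that replays a recorded clone's life from a BlackBox onto a Clone_Main pawn.
; Tick applies time-synced movement and aim frames, while delayed loops replay shots and ability events.
; Shots re-resolve recorded targets and lead live ones, with optional offset limits.
; When the recording runs out, targets die or vehicle state diverges, a health check either turns the clone into an NPC or replays its death.
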(event `self.ReceivePossess`
  (params (PossessedPawn :type "Pawn Object Reference"))
  ;[1 1 1] setup
  (set `self.Body` (cast `/Game/Blueprints/Chars/Clones/Clone_Main` PossessedPawn :!pure true)))

(event `start checking for no targets`
  ;[1 1 1] Checking for no targets
  (`KismetSystemLibrary.Delay` 0.5 :!label _label)
  (bind _dead (`self.Are All Targets Dead`))
  (if (and _dead (`self.All events extracted`))
    (`self.Try to save`)
    (else
      (goto _label))))

(event `start reading shots`
  (bind _body (`self.Body`))
  ;[1 1 1] Shots
  (bind (_extracted _shot_time _hit _hits_info _spread_angles _hit_location _shot_info) (`/Game/Blueprints/recording/Black_Box.Extract shot` (`self.Black box`) :!label _label_2))
  (if _extracted
    (set `self.gun aim blocked` false)
    (`KismetSystemLibrary.Delay` _shot_time)
    (if (not _hit)
      (`/Game/Blueprints/Chars/Clones/Clone_Main.Repeat Shot` _body false (stale _targets) _spread_angles _hit_location)
      (else
        (set `self.gun aim blocked` true)
        (bind (_has_dead_target _targets) (`self.Find shot targets` _hits_info))
        (`/Engine/EditorBlueprintResources/StandardMacros.CompareInt` (`KismetArrayLibrary.Array_Length` _targets) 1
          (:`>`
            (if (`/Game/Blueprints/recording/Shot_Info.aim on mid of hits` _shot_info)
              (bind _location (`self.Mid Of Targets` _targets))
              (set `self.Target location` _location)
              (else
                (set `self.Target location` (`/Game/Blueprints/System/Funtions/FunctionLibrary.Calculate Preemption` (`|GetArrayItem` _targets) (`self.Body`)) :!label _label_3)
                (bind _target (`self.Find shot target` (`|GetArrayItem` _hits_info)))
                (bind _alive (`/Game/Blueprints/System/Interfaces/Aimable.Is Alive` _target))
                (bind _hit_location_2 (`/Game/Blueprints/recording/Shot_Info.Hit location` _shot_info))
                (if (and (`/Game/Blueprints/recording/Shot_Info.Limited acceptable offset` _shot_info) (or (> (`KismetMathLibrary.Vector_Distance2D` _hit_location_2 (`self.Target location`)) (`/Game/Blueprints/recording/Shot_Info.Acceptable offset` _shot_info)) (not _alive)))
                  (set `self.Target location` _hit_location_2))))
            (`self.Aim on character` (`self.Target location`))
            (`/Game/Blueprints/Chars/Clones/Clone_Main.Repeat Shot` _body true _targets _spread_angles _hit_location))
          (:`==`
            (goto _label_3))
          (:`<`
            _))))
    (if (and (`self.IsActorTickEnabled`) (`/Game/Blueprints/Chars/Clones/Clone_Main.Repeater` (`self.Body`)))
      (goto _label_2))
    (else
      (set `self.no ammo` true))))

(event `Start reading events`
  (bind _body (`self.Body`))
  ;[1 1 1] Read ability events
  (bind (_extracted _shot_time _event _addittional_info) (`/Game/Blueprints/recording/Black_Box.Extract Event` (`self.Black box`) :!label _label_4))
  (if _extracted
    (`KismetSystemLibrary.Delay` _shot_time)
    (if (`/Game/Blueprints/Chars/Clones/Clone_Main.Repeater` (`self.Body`))
      (`|ExecutionSequence`
        (:`then_0`
          (switch `/Game/Blueprints/recording/events/Save_Event_Type` _event
            (:`NewEnumerator0`
              (`/Game/Blueprints/Chars/Clones/Clone_Main.Repeat Ability` _body _addittional_info))
            (:`NewEnumerator1`
              (`/Game/Blueprints/Chars/Abstract/Base_Character.Abort Ability` _body _addittional_info))
            (:`NewEnumerator3`
              (`/Game/Blueprints/Chars/Abstract/Base_Character.Suicide` _body))
            (:`NewEnumerator4`
              (bind _asplace_event_info (cast `/Game/Blueprints/recording/events/place_event_info` _addittional_info))
              (`self.Spawn MG` (`/Game/Blueprints/recording/events/place_event_info.location` _asplace_event_info)))
            (:`NewEnumerator5`
              (`/Game/Blueprints/Chars/Abstract/Base_Character.Interact` _body))
            (:`NewEnumerator6`
              (`/Game/Blueprints/Chars/Clones/Clone_Main.Repeat wire hit` _body _addittional_info))
            (:`NewEnumerator7`
              (`/Game/Blueprints/Chars/Clones/Clone_Main.Repeat Rotation Anim` _body _addittional_info))
            (:`NewEnumerator8`
              (`/Game/Blueprints/Chars/Abstract/Base_Character.Trench Jump` _body))))
        (:`then_1`
          (goto _label_4))))
    (else
      (set `self.All events extracted` true))))

(event `self.ReceiveTick`
  (params (DeltaSeconds :type "Float (single-precision)"))
  ;[1 1 1] Body
  (set `self.wait condition` true)
  (while (and (`self.wait condition`) (not (`self.skip frame`)))
    (bind (_done _frame_info) (`/Game/Blueprints/recording/Black_Box.Extract Frame` (`self.Black box`)))
    (if _done
      (bind _returnvalue (- (`.Time_13_04C1D17A43DB371DED676DA11498CAF4` (break `/Game/Blueprints/recording/Frame_Info` _frame_info)) (`KismetSystemLibrary.GetGameTimeInSeconds`)))
      (bind _output_get (set `self.delta frames` (/ _returnvalue DeltaSeconds)))
      (`/Engine/EditorBlueprintResources/StandardMacros.CompareInt` (`KismetMathLibrary.FTrunc` _output_get)
        (:`>`
          (set `self.delta time` _returnvalue)
          (set `self.skip frame` true))
        (:`==`
          (set `self.wait condition` false)))
      (else
        (set `self.wait condition` false))))
  (if (`self.skip frame`)
    (`KismetSystemLibrary.Delay` (`self.delta time`))
    (set `self.skip frame` false))
  (if _done
    (`self.Control Body` _frame_info)
    (else
      (set `/Game/Blueprints/Chars/Clones/Clone_Main.Speed_0` (0.0 0.0 0.0) (`self.Body`))
      (if (`self.no ammo`) :!label _label_5
        (`self.Try to save`)
        (else
          (`KismetSystemLibrary.Delay` 0.1)
          (goto _label_5))))))

(event `Try to save`
  (bind _body (`self.Body`))
  (bind _body_2 (`self.Body`))
  (bind _death_info (`/Game/Blueprints/recording/Black_Box.Death info` (`self.Black box`)))
  ;[1 1 1] saving life
  (if (`/Game/Blueprints/Chars/Clones/Clone_Main.Repeater` (`self.Body`))
    (`self.SetActorTickEnabled` false)
    (if (not (`/Game/Blueprints/Chars/Abstract/Base_Character.suiciding` _body))
      (`/Game/Blueprints/Chars/Clones/Clone_Main.Stop Rotating Anim` _body)
      (if (`self.Saved Condition`)
        (set `/Game/Blueprints/Chars/Clones/Clone_Main.Repeater` false _body_2)
        (`/Game/Blueprints/Chars/Abstract/Base_Character.Turn off ability` _body_2)
        (`KismetSystemLibrary.Delay` 1.0)
        (if (`self.Saved Condition`)
          (set `/Game/Blueprints/Chars/Clones/Clone_Main.Black box` (`self.Black box`) _body_2)
          (`self.UnPossess`)
          (`/Game/Blueprints/Chars/Clones/Clone_Main.Setup as NPC` _body_2)
          (else
            (bind _target (`self.Find shot target` (`/Game/Blueprints/recording/Death_info.killer character` _death_info) :!label _label_6))
            (`/Game/Blueprints/Chars/Abstract/Base_Character.Die` (`self.Body`) null false (`/Game/Blueprints/recording/Death_info.Death impulse` _death_info) (`/Game/Blueprints/recording/Death_info.Hit location` _death_info) (`/Game/Blueprints/recording/Death_info.Death impulse common` _death_info) false (cast `/Game/Blueprints/Chars/Abstract/Base_Character` _target :!pure true))))
        (else
          (goto _label_6))))))

(fn `Aim on character`
  (params (Location :type "Vector Structure"))
  (`/Game/Blueprints/Chars/Abstract/Base_Character.Set gun angle` (`self.Body`) Location 1.0))

(fn `Are All Targets Dead`
  (returns (dead :type Boolean))
  (bind _targets (`/Game/Blueprints/recording/Black_Box.Targets` (`self.Black box`)))
  (`/Engine/EditorBlueprintResources/StandardMacros.CompareInt` (`KismetArrayLibrary.Array_Length` _targets)
    (:`>`
      (for _array_element _targets
        (bind _target (`self.Find shot target` _array_element))
        (`/Game/Blueprints/System/Funtions/Macro_Library.Is Valid I` _target
          (:`Is Valid`
            (bind _alive (`/Game/Blueprints/System/Interfaces/Aimable.Is Alive` _target))
            (if _alive
              (return false)))
          (:`Is Not Valid`
            (return false))))
      (return true))
    (:`==`
      (return false))))

(fn `Control Body`
  (params (`Frame info` :type "/Game/Blueprints/recording/Frame_Info Structure"))
  (bind (_time _location _bodyangle _speed _health _wantbeinvehicle _aimlocation _invehicle _armsstate _rightarmangles _midarmangle) (break `/Game/Blueprints/recording/Frame_Info` `Frame info`))
  (bind _body (`self.Body`))
  (if (== (`/Game/Blueprints/Chars/Abstract/Base_Character.In vehicle` (`self.Body`)) _invehicle)
    (set `/Game/Blueprints/Chars/Clones/Clone_Main.Recorded aim location` _aimlocation (`self.Body`))
    (`|ExecutionSequence`
      (:`then_0`
        (if _invehicle
          (set `/Game/Blueprints/Chars/Clones/Clone_Main.Speed_0` (0.0 0.0 0.0) (`self.Body`))
          (else
            (`/Game/Blueprints/Chars/Clones/Clone_Main.Rotate body repeater` (`self.Body`) _bodyangle)
            (`self.K2_SetActorLocation` (`self.Body`) _location false false)
            (set `/Game/Blueprints/Chars/Clones/Clone_Main.Speed_0` _speed (`self.Body`)))))
      (:`then_1`
        (set `/Game/Blueprints/Chars/Abstract/Base_Character.Want be in vehicle` _wantbeinvehicle (`self.Body`))
        (`|ExecutionSequence`
          (:`then_0`
            (if (not (`self.gun aim blocked`))
              (`/Game/Blueprints/Arms/Hands/Arsenal.Repeat Aim` (`/Game/Blueprints/Chars/Abstract/Base_Character.Get Arsenal` _body) _armsstate _rightarmangles _midarmangle)))
          (:`then_1`
            (if (`self.First read`)
              (`/Game/Blueprints/Chars/Abstract/Base_Character.Apply health` _body _health)
              (set `self.First read` false))))))
    (else
      (`self.Try to save`))))

(fn `Find shot target`
  (params (Hit_Info :type "/Game/Blueprints/recording/Serialized_Target Structure (by ref)"))
  (returns (Target :type "/Game/Blueprints/System/Interfaces/Aimable Interface"))
  (locals (`Result target` :type "/Game/Blueprints/System/Interfaces/Aimable Interface"))
  (bind (_target _indexinspawn) (break `/Game/Blueprints/recording/Serialized_Target` Hit_Info))
  (bind _asactor (cast `Actor` (`/Game/Blueprints/System/Funtions/FunctionLibrary.Find object by string` _target) :!pure true))
  (bind _asspawners (cast `/Game/Blueprints/Logics/Components/Spawners` _asactor)
    (:`then`
      (bind _spawned (`/Game/Blueprints/Logics/Components/Spawners.Get spawned` _asspawners))
      (bind _output (`|GetArrayItem` _spawned _indexinspawn))
      (`/Engine/EditorBlueprintResources/StandardMacros.IsValid` _output
        (:`Is Valid`
          (bind _output_get (set `local.Result target` _output)))
        (:`Is Not Valid`
          (return null))))
    (:`CastFailed`
      (set `local.Result target` (cast `/Game/Blueprints/System/Interfaces/Aimable` _asactor :!pure true))))
  (return _output_get))

(fn `Find shot targets`
  (params (`Hits info` :type "Array of /Game/Blueprints/recording/Serialized_Target Structure"))
  (returns (`has dead target` :type Boolean) (Targets :type "Array of /Game/Blueprints/System/Interfaces/Aimable Interface"))
  (locals (`Shot targets` :type "Array of /Game/Blueprints/System/Interfaces/Aimable Interface") (`there is dead target` :type Boolean :default false))
  (for _array_element `Hits info`
    (bind _target (`self.Find shot target` _array_element))
    (`/Game/Blueprints/System/Funtions/Macro_Library.Is Valid I` _target
      (:`Is Valid`
        (bind _alive (`/Game/Blueprints/System/Interfaces/Aimable.Is Alive` _target))
        (if _alive
          (`KismetArrayLibrary.Array_Add` (`local.Shot targets`) _target)
          (else
            (set `local.there is dead target` true))))))
  (return (`local.there is dead target`) (`local.Shot targets`)))

(fn `Get grid walker`
  (returns (`grid walker` :type "/Game/Blueprints/Navigation/Grid_Walker Object Reference"))
  (return null))

(fn `Get sound override`
  (returns (`Override params` :type "/Game/Sounds/Sound_Override Structure"))
  (return (`self.Sound overrides`)))

(fn `Insert Black Box`
  (params (`Black box` :type "/Game/Blueprints/recording/Black_Box Object Reference"))
  (bind _black_box (`self.Black box`))
  (set `self.Black box` `Black box`)
  (set `/Game/Blueprints/recording/Black_Box.locked` false _black_box)
  (`/Game/Blueprints/Chars/Clones/Clone_Main.init memory` (`self.Body`) (`/Game/Blueprints/recording/Black_Box.Clone number` _black_box) (`/Game/Blueprints/recording/Black_Box.Name` _black_box))
  (`self.start checking for no targets`)
  (`self.start reading shots`)
  (`self.Start reading events`))

(fn `Mid Of Targets`
  (params (Targets :type "Array of /Game/Blueprints/System/Interfaces/Aimable Interface"))
  (returns (Location :type "Vector Structure"))
  (locals (`Sum location` :type "Vector Structure"))
  (for _array_element Targets
    (set `local.Sum location` (+ (`local.Sum location`) (`/Game/Blueprints/System/Funtions/FunctionLibrary.Calculate Preemption` _array_element (`self.Body`)))))
  (return (/ (`local.Sum location`) (`KismetArrayLibrary.Array_Length` Targets))))

(fn `Saved Condition`
  (returns (Saved :type Boolean))
  (locals (`NPC posses health edge` :type "Float (double-precision)" :default 30.0) (`NPC posses health% edge` :type "Float (double-precision)" :default 50.0))
  (bind _body (`self.Body`))
  (return (>= (`/Game/Blueprints/Chars/Abstract/Base_Character.Health` _body) (`/Game/Blueprints/Chars/Clones/Clone_Main.Hp to save` _body))))

(fn `Spawn MG`
  (params (Location :type "Vector Structure"))
  (bind _tile (`/Game/Blueprints/System/Funtions/Tile_Functions.Get Tile Under` Location 50.0))
  (bind _returnvalue (`|SpawnActorFromClass` "/Game/Blueprints/Vehicles/Rotating_MG_Emplacement.Rotating_MG_Emplacement_C" (`KismetMathLibrary.MakeTransform` Location (struct :`Yaw` 180.0)) "Undefined" "MultiplyWithRoot" null null))
  (set `/Game/3D/platforms/Tile.placed thing` _returnvalue _tile))

(fn `UserConstructionScript`)