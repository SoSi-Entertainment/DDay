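; AI controller for NPC characters, handling grid patrols, alert states and persistence.
; A walk loop feeds PathManager directions to GridWalker, pausing to shoot on paths that allow it.
; Noticing an enemy warns nearby allied controllers, with a timer returning to Chill.
; On checkpoint or level close it saves transform, health, gun and path progress, polling for corpses to settle, and restores them on possess; clones and spawned NPCs save through InstanseTroops.
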(event `self.ReceivePossess`
  (params (PossessedPawn :type "Pawn Object Reference"))
  (bind _troops_instance (`/Game/Blueprints/System/FunctionLibrary.Get Instanse Troops`))
  (bind _asbase_character (cast `/Game/Blueprints/Chars/Abstract/Base_Character` PossessedPawn :!pure true))
  (bind _body (`self.body`))
  (bind _grid_walker (`self.Grid_Walker`))
  (bind _path_manager (`self.Path_manager`))
  (bind _body_2 (`self.body`))
  (bind _path_iterator (`self.Path iterator`))
  (bind _instance_saver (`self.Instance_Saver`))
  (bind _want_to_shoot (`/Game/Blueprints/Chars/Components/Aim_component.Want to shoot` (`self.Aim_component`)))
  (bind _path (`/Game/Blueprints/Navigation/Path_manager.path` (`self.Path_manager`)))
  (set `self.Path` (`/Game/Blueprints/Chars/Abstract/Base_Character.Path` _asbase_character))
  (bind _output_get (set `self.body` _asbase_character))
  (add `/Game/Blueprints/Chars/Abstract/Base_Character.Inited` _output_get (delegate `Body inited`))
  (add `/Game/Blueprints/System/DDay_Instance.Checkpoint reached` _troops_instance (delegate `Checkpoint reached`))
  (add `/Game/Blueprints/System/DDay_Instance.Level close` _troops_instance (delegate `level close`))
  (`|ExecutionSequence`
    (:`then_0`
      (`KismetSystemLibrary.Delay` 0.2)
      (set `/Game/Blueprints/Navigation/Path_manager.path` (`/Game/Blueprints/Chars/Abstract/Base_Character.Path` (`self.body`)) (`self.Path_manager`))
      (if (and (not (and (not (`/Game/Blueprints/Navigation/Path_holder.Looped` _path)) (== (`KismetArrayLibrary.Array_Length` (`/Game/Blueprints/Navigation/Path_holder.Points` _path)) _path_iterator))) (> _path_iterator 0))
        (set `/Game/Blueprints/Navigation/Path_holder.iterator` _path_iterator _path))
      (bind _newparam (`/Game/Blueprints/Navigation/Path_manager.Get direction` _path_manager :!label _label))
      (if (not (`/Game/Blueprints/Chars/Abstract/Base_Character.Dead` _body))
        (bind _returnvalue (`|EnumEquality` _newparam "NewEnumerator4"))
        (bind _output_get_2 (set `self.Waiting` (and (not _want_to_shoot) _returnvalue)))
        (set `/Game/Blueprints/Chars/Components/Sway_Component.Turn on` _output_get_2 (`/Game/Blueprints/Chars/Abstract/Base_Character.Sway_Component` _body))
        (if (or (and _want_to_shoot (`/Game/Blueprints/Navigation/Path_holder.Stop to shoot` (`/Game/Blueprints/Navigation/Path_manager.path` _path_manager))) _returnvalue)
          (`/Game/Blueprints/Navigation/Grid_Walker.Ungo` _grid_walker false)
          (else
            (bind _walk_started (`/Game/Blueprints/Navigation/Grid_Walker.Go` _grid_walker _newparam))
            (if _walk_started
              (`self.Set walking` true)
              (`/Game/Blueprints/System/DDayMacroLibrary.Wait condition` (`/Game/Blueprints/Navigation/Grid_Walker.OnTile` _grid_walker)
                (:`true`
                  (`self.Set walking` false)
                  (goto _label)))
              (else
                _))))
        (`KismetSystemLibrary.Delay` 0.1)
        (goto _label)))
    (:`then_1`
      ;[1 1 1] Load
      (`/Game/Blueprints/System/Instance_Saver.Add Custom Owner` _instance_saver (`self.body`))
      (bind (_success _save) (`/Game/Blueprints/System/Instance_Saver.Get save from instance` _instance_saver 0))
      (if _success
        (bind _data (`/Game/Blueprints/System/Instanse_Save.Data` _save))
        (bind _returnvalue_2 (`KismetStringLibrary.Conv_StringToDouble` (`|GetArrayItem` _data 2)))
        (`/Engine/EditorBlueprintResources/StandardMacros.CompareFloat` _returnvalue_2
          (:`>`
            (set `self.Path iterator` (- (`KismetStringLibrary.Conv_StringToInt` (`|GetArrayItem` _data 6)) 1))
            (bind _outconvertedvector (`KismetStringLibrary.Conv_StringToVector` (`|GetArrayItem` _data)))
            (`self.K2_SetActorLocation` _body_2 _outconvertedvector false true)
            (`/Game/Blueprints/Chars/Abstract/Base_Character.Apply health` _body_2 _returnvalue_2)
            (bind _outconvertedrotator (`KismetStringLibrary.Conv_StringToRotator` (`|GetArrayItem` _data 1)))
            (`self.K2_SetActorRotation` _body_2 _outconvertedrotator true))
          (:`==`
            (`KismetSystemLibrary.Delay` 0.2)
            (`/Game/Blueprints/Chars/Abstract/Base_Character.Die on start` _body_2 true (`KismetMathLibrary.Conv_IntToBool` (`KismetStringLibrary.Conv_StringToInt` (`|GetArrayItem` _data 5))) _outconvertedvector _outconvertedrotator (`KismetStringLibrary.Conv_StringToVector` (`|GetArrayItem` _data 3)) (`KismetStringLibrary.Conv_StringToRotator` (`|GetArrayItem` _data 4)))))))))

(event `Body inited`
  (params (Character :type "/Game/Blueprints/Chars/Abstract/Base_Character Object Reference"))
  (`self.Get field radius` Character))

(event `level close`
  ;[1 1 1] Save
  (if (and (`self.should be saved`) (not (`self.was saved`)))
    (`self.Save Restore Position` 0.0 true)
    (set `self.was saved` true)))

(event `Checkpoint reached`
  (params (`Checkpoint number` :type Integer) (`Distance reached` :type "Float (double-precision)"))
  (bind _mesh (`Character.Mesh` (`self.body`)))
  ;[1 1 1] Save
  (`/Engine/EditorBlueprintResources/StandardMacros.CompareFloat` (`/Game/Blueprints/System/FunctionLibrary.Angle between vectors` (`KismetMathLibrary.Vector_Up`) (`SceneComponent.GetUpVector` _mesh)) 5.0
    (:`>`
      _)
    (:`==`
      _)
    (:`<`
      (`KismetSystemLibrary.Delay` 0.5)))
  (set `self.should be saved` true)
  (if (`/Game/Blueprints/Chars/Abstract/Base_Character.Dead` (`self.body`))
    (`/Engine/EditorBlueprintResources/StandardMacros.CompareFloat` (`KismetMathLibrary.VSize` (`PrimitiveComponent.GetPhysicsAngularVelocityInDegrees` _mesh "None")) 5.0 :!label _label_2
      (:`>`
        (`KismetSystemLibrary.Delay` 0.5 :!label _label_3)
        (if (not (`self.was saved`))
          (goto _label_2)))
      (:`==`
        (goto _label_3))
      (:`<`
        (`self.Save Restore Position` `Distance reached` :!label _label_4)
        (set `self.was saved` true)))
    (else
      (goto _label_4))))

(fn `add path`
  (params (path :type "/Game/Blueprints/Navigation/Path_holder Object Reference"))
  (set `/Game/Blueprints/Navigation/Path_manager.path` path (`self.Path_manager`)))

(fn `Body dead`
  (set `self.ai state` "NewEnumerator3"))

(fn `Call`
  (params (reason :type "/Game/Data/enums/Call_Type Enum" :default "NewEnumerator0"))
  (switch `/Game/Data/enums/Call_Type` reason
    (:`NewEnumerator0`
      (bind _was_chilled_before (`self.Set warned`))
      (if _was_chilled_before
        (`/Game/Blueprints/Chars/Abstract/Base_Character.Say` (`self.body`) "warned" 3.0)))))

(fn `CanSeePlayer`
  (returns (see :type Boolean))
  (bind (_outhit _returnvalue) (`KismetSystemLibrary.LineTraceSingle` :`Start` (`self.K2_GetActorLocation` (`self.K2_GetPawn`)) :`End` (`self.K2_GetActorLocation` (`GameplayStatics.GetPlayerPawn` 0)) :`TraceChannel` "TraceTypeQuery1" :`DrawDebugType` "ForOneFrame"))
  (return (not _returnvalue)))

(fn `Chill`
  (switch `/Game/Data/enums/Ai_state` (`self.ai state`)
    (:`NewEnumerator1`
      _)
    (:`NewEnumerator2`
      _))
  (set `self.ai state` "NewEnumerator0")
  (`/Game/Blueprints/Chars/Abstract/Base_Character.Say` (`self.body`) "Chill" 2.0))

(fn `Enemy Noticed`
  (params (`noticed charcter` :type "/Game/Blueprints/Chars/Abstract/Base_Character Object Reference"))
  (bind _body (`self.body`))
  (bind _was_chilled_before (`self.Set warned`))
  (if _was_chilled_before
    (`/Game/Blueprints/Chars/Abstract/Base_Character.Say` _body "noticed" 3.0)
    (`/Game/Blueprints/Chars/Abstract/Base_Character.On enemy noticed` _body `noticed charcter`)
    (bind (_found _nearby_allies) (`/Game/Blueprints/Chars/Abstract/Base_Character.Find Allies Nerby` _body))
    (for _array_element _nearby_allies
      (bind _asbase_character (cast `/Game/Blueprints/Chars/Abstract/Base_Character` _array_element))
      (bind _asnpc_ai_controller (cast `/Game/Blueprints/Controllers/NPC_Ai_Controller` (`AIBlueprintHelperLibrary.GetAIController` _asbase_character)))
      (`self.Call` _asnpc_ai_controller "NewEnumerator0"))))

(fn `Find path`
  (params (Target :type "Vector Structure"))
  (returns (`Path tiles` :type "Array of /Game/3D/platforms/Tile Object Reference"))
  (locals (Tiles :type "Array of /Game/3D/platforms/Tile Object Reference"))
  (bind _tiles (`local.Tiles`))
  (bind _surface_location (`/Game/Blueprints/System/FunctionLibrary.Get platform under` Target))
  (bind _surface_location_2 (`/Game/Blueprints/System/FunctionLibrary.Get platform under` (`self.K2_GetActorLocation` (`self.body`))))
  (bind _returnvalue (`NavigationSystemV1.FindPathToLocationSynchronously` _surface_location_2 _surface_location null null))
  (for _array_element (`NavigationPath.PathPoints` _returnvalue)
    (bind (_surface_location_3 _platform) (`/Game/Blueprints/System/FunctionLibrary.Get platform under` _array_element))
    (`/Engine/EditorBlueprintResources/StandardMacros.IsValid` _platform
      (:`Is Valid`
        (`KismetArrayLibrary.Array_AddUnique` (`local.Tiles`) (`/Game/3D/platforms/Default_Platform_bp.Get tile` _platform)))))
  (`KismetArrayLibrary.Array_Remove` _tiles)
  (return _tiles))

(fn `Get field radius`
  (params (`Base character` :type "/Game/Blueprints/Chars/Abstract/Base_Character Object Reference"))
  (bind _stats (`/Game/Blueprints/System/FunctionLibrary.Get Balanced stats` (`/Game/Blueprints/Chars/Abstract/Base_Character.Unit type` `Base character`) "NewEnumerator1"))
  (`SphereComponent.SetSphereRadius` (`self.Field`) (/ (`KismetMathLibrary.Conv_IntToDouble` (`.Viewrange_50_E10048E24E5C6AD922443CB64BFCF419` (break `/Game/Data/structs/Balance_State` _stats))) (`KismetMathLibrary.BreakVector3f` (`SceneComponent.K2_GetComponentScale` (`self.Field`)))) true))

(fn `Get grid walker`
  (returns (`grid walker` :type "/Game/Blueprints/Navigation/Grid_Walker Object Reference"))
  (return (`self.Grid_Walker`)))

(fn `Get sound override`
  (returns (`Override params` :type "/Game/Sounds/Sound_Override Structure"))
  (return (`self.Sound overrides`)))

(fn `Go to location`
  (params (Location :type "Vector Structure"))
  (if (not (`/Game/Blueprints/Chars/Abstract/Base_Character.Dead` (`self.body`)))
    (bind _path_tiles (`self.Find path` Location))
    (for _array_element _path_tiles
      (`/Game/Blueprints/Navigation/Path_manager.Load new path` (`self.Path_manager`) _path_tiles))))

(fn `Save Restore Position`
  (params (`Distance reached` :type "Float (double-precision)") (`Force clear` :type Boolean))
  (bind _troops_instance (`/Game/Blueprints/System/FunctionLibrary.Get Instanse Troops`))
  (bind _body (`self.body`))
  (bind _instance_saver (`self.Instance_Saver`))
  (bind _body_2 (`self.body`))
  (bind _returnvalue (`self.K2_GetActorRotation` _body))
  (bind _path (`/Game/Blueprints/Navigation/Path_manager.path` (`self.Path_manager`)))
  (bind _gun_skeleton (`/Game/Blueprints/Arms/Gun.gun skeleton` (`/Game/Blueprints/Chars/Abstract/Base_Character.Get gun` _body)))
  (bind _returnvalue_2 (and (`|EnumEquality` (`/Game/Blueprints/Chars/Abstract/Base_Character.Team` _body_2) "NewEnumerator1") (< (.x (`self.K2_GetActorLocation` _body_2)) `Distance reached`)))
  (bind _asclone_main (cast `/Game/Blueprints/Chars/Clones/Clone_Main` _body_2)
    (:`then`
      (`/Game/Blueprints/System/DDay_Instance.Resave clone to NPC` _troops_instance _asclone_main))
    (:`CastFailed`
      (if (`/Game/Blueprints/Chars/Abstract/Base_Character.Spawned` _body_2)
        (`/Game/Blueprints/System/DDay_Instance.Add New dead spawned NPC` _troops_instance false _body_2 `Distance reached`)
        (else
          (`/Game/Blueprints/System/Instance_Saver.Add Custom Owner` _instance_saver _body_2)
          (bind (_success _save) (`/Game/Blueprints/System/Instance_Saver.Get save from instance` _instance_saver 0))
          (if _success
            (`/Engine/EditorBlueprintResources/StandardMacros.CompareFloat` (`KismetStringLibrary.Conv_StringToDouble` (`|GetArrayItem` (`/Game/Blueprints/System/Instanse_Save.Data` _save) 2))
              (:`>`
                _)))
          (bind _instance_save (`/Game/Blueprints/System/Instance_Saver.Create save in instance` _instance_saver 0 true))
          (bind _data (`/Game/Blueprints/System/Instanse_Save.Data` _instance_save))
          (`KismetArrayLibrary.Array_Set` _data 0 (`KismetStringLibrary.Conv_VectorToString` (`self.K2_GetActorLocation` _body)) true)
          (`KismetArrayLibrary.Array_Set` _data 1 (`KismetStringLibrary.Conv_RotatorToString` (select `bool` `Force clear` :`false` _returnvalue :`true` (`KismetMathLibrary.MakeRotator` 0.0 0.0 (.yaw _returnvalue)))) true)
          (`KismetArrayLibrary.Array_Set` _data 2 (`KismetStringLibrary.Conv_DoubleToString` (`KismetMathLibrary.SelectFloat` 0.0 (`/Game/Blueprints/Chars/Abstract/Base_Character.Health` _body) _returnvalue_2)) true)
          (`KismetArrayLibrary.Array_Set` _data 3 (`KismetStringLibrary.Conv_VectorToString` (`SceneComponent.K2_GetComponentLocation` _gun_skeleton)) true)
          (`KismetArrayLibrary.Array_Set` _data 4 (`KismetStringLibrary.Conv_RotatorToString` (`SceneComponent.K2_GetComponentRotation` _gun_skeleton)) true)
          (`KismetArrayLibrary.Array_Set` _data 5 (`KismetStringLibrary.Conv_IntToString` (`KismetMathLibrary.Conv_BoolToInt` (or (and _returnvalue_2 (not (`/Game/Blueprints/Chars/Abstract/Base_Character.Dead` _body_2))) `Force clear`))) true)
          (`/Engine/EditorBlueprintResources/StandardMacros.IsValid` _path
            (:`Is Valid`
              (`KismetArrayLibrary.Array_Set` _data 6 (`KismetStringLibrary.Conv_IntToString` (`/Game/Blueprints/Navigation/Path_holder.iterator` _path)) true))))))))

(fn `Set walking`
  (params (`is walking` :type Boolean))
  (set `/Game/Blueprints/Chars/Components/Aim_component.Walking` `is walking` (`self.Aim_component`))
  (set `/Game/Blueprints/Chars/Abstract/Base_Character.walking` `is walking` (`self.body`)))

(fn `Set warned`
  (returns (`Was chilled before` :type Boolean))
  (locals (`Was chilled` :type Boolean))
  (switch `/Game/Data/enums/Ai_state` (`self.ai state`)
    (:`NewEnumerator0`
      (set `local.Was chilled` true))
    (:`NewEnumerator1`
      _)
    (:`NewEnumerator2`
      (return false))
    (:`NewEnumerator3`
      (return false)))
  (set `self.ai state` "NewEnumerator1")
  (`KismetSystemLibrary.K2_SetTimer` null "Chill" (`self.Time before chill`))
  (return (`local.Was chilled`)))

(fn `test draw`
  (`KismetSystemLibrary.DrawDebugCircle` (`self.K2_GetActorLocation` (`self.K2_GetPawn`)) 50.0 50 (struct :`G` 1.0 :`B` 0.058979 :`A` 1.0) 2.0 5.0 (0.0 1.0 0.0) (1.0 0.0 0.0)))

(fn `UserConstructionScript`)