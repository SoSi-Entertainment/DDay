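; AI controller that replays a clone's recorded run from a BlackBox on a Clone_Main body.
; Tick applies time-matched movement frames while parallel delay loops replay shots and ability events.
; Recorded hits re-aim at the live targets using lead prediction, averaged for multiple targets.
; When targets are dead, recordings run out or vehicle state diverges, TryToSave turns a healthy clone into an NPC or kills it with recorded death info.
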(event `self.ReceivePossess`
  (params (PossessedPawn :type "Pawn Object Reference"))
  ;[1 1 1] setup
  (set `self.Body` (cast `/Game/Blueprints/Chars/Clones/Clone_Main` PossessedPawn :!pure true)))

(event `start checking for no targets`
  ;[1 1 1] Checking for no targets
  (`KismetSystemLibrary.Delay` 0.5 :!label _label)
  (bind _dead (`self.Are All Targets Dead`))
  (if (and _dead (`self.All events extracted`))
    (`self.Try to save`)
    (else
      (goto _label))))

(event `start reading shots`
  (bind _body (`self.Body`))
  ;[1 1 1] Shots
  (bind (_extracted _shot_time _hit _hits_info) (`/Game/Blueprints/recording/Black_Box.Extract shot` (`self.Black box`) :!label _label_2))
  (if _extracted
    (set `self.gun aim blocked` false)
    (`KismetSystemLibrary.Delay` _shot_time)
    (if _hit
      (set `self.gun aim blocked` true)
      (bind _targets (`self.Find shot targets` _hits_info))
      (`/Engine/EditorBlueprintResources/StandardMacros.CompareInt` (`KismetArrayLibrary.Array_Length` _targets) 1
        (:`>`
          (bind _location (`self.Mid Of Targets` _targets))
          (set `self.Target location` _location)
          (`self.Aim on character` (`self.Target location`) :!label _label_3)
          (`/Game/Blueprints/Chars/Abstract/Base_Character.Gun Shoot` _body null true (0.0 0.0 0.0) false _targets))
        (:`==`
          (set `self.Target location` (`/Game/Blueprints/System/FunctionLibrary.Calculate Preemption` (`|GetArrayItem` _targets) (`self.Body`)))
          (goto _label_3))
        (:`<`
          _))
      (else
        (`/Game/Blueprints/Chars/Abstract/Base_Character.Gun Shoot` _body null false (0.0 0.0 0.0) true _targets)))
    (if (and (`self.IsActorTickEnabled`) (`/Game/Blueprints/Chars/Clones/Clone_Main.Repeater` (`self.Body`)))
      (goto _label_2))
    (else
      (set `self.no ammo` true))))

(event `Start reading events`
  ;[1 1 1] Read ability events
  (bind (_extracted _shot_time _event) (`/Game/Blueprints/recording/Black_Box.Extract Event` (`self.Black box`) :!label _label_4))
  (if _extracted
    (`KismetSystemLibrary.Delay` _shot_time)
    (if (`/Game/Blueprints/Chars/Clones/Clone_Main.Repeater` (`self.Body`))
      (`|ExecutionSequence`
        (:`then_0`
          (switch `/Game/Blueprints/recording/Save_Event_Type` _event
            (:`NewEnumerator0`
              (`/Game/Blueprints/Chars/Abstract/Base_Character.Use Ability` (`self.Body`)))))
        (:`then_1`
          (goto _label_4))))
    (else
      (set `self.All events extracted` true))))

(event `self.ReceiveTick`
  (params (DeltaSeconds :type "Float (single-precision)"))
  ;[1 1 1] Body
  (set `self.wait condition` true)
  (while (and (`self.wait condition`) (not (`self.skip frame`)))
    (bind (_done _frame_info) (`/Game/Blueprints/recording/Black_Box.Extract Frame` (`self.Black box`)))
    (if _done
      (bind _returnvalue (- (`.Time_13_04C1D17A43DB371DED676DA11498CAF4` (break `/Game/Blueprints/recording/Frame_Info` _frame_info)) (`KismetSystemLibrary.GetGameTimeInSeconds`)))
      (bind _output_get (set `self.delta frames` (/ _returnvalue DeltaSeconds)))
      (`/Engine/EditorBlueprintResources/StandardMacros.CompareInt` (`KismetMathLibrary.FTrunc` _output_get)
        (:`>`
          (set `self.delta time` _returnvalue)
          (set `self.skip frame` true))
        (:`==`
          (set `self.wait condition` false)))
      (else
        (set `self.wait condition` false))))
  (if (`self.skip frame`)
    (`KismetSystemLibrary.Delay` (`self.delta time`))
    (set `self.skip frame` false))
  (if _done
    (`self.Control Body` _frame_info)
    (else
      (set `/Game/Blueprints/Chars/Clones/Clone_Main.Speed_0` (0.0 0.0 0.0) (`self.Body`))
      (if (`self.no ammo`) :!label _label_5
        (`self.Try to save`)
        (else
          (`KismetSystemLibrary.Delay` 0.1)
          (goto _label_5))))))

(event `Try to save`
  (bind _body (`self.Body`))
  (bind _death_info (`/Game/Blueprints/recording/Black_Box.Death info` (`self.Black box`)))
  ;[1 1 1] saving life
  (if (`/Game/Blueprints/Chars/Clones/Clone_Main.Repeater` (`self.Body`))
    (`self.SetActorTickEnabled` false)
    (if (`self.Saved Condition`)
      (set `/Game/Blueprints/Chars/Clones/Clone_Main.Repeater` false _body)
      (`/Game/Blueprints/Chars/Abstract/Base_Character.Turn off ability` _body)
      (`KismetSystemLibrary.Delay` 1.0)
      (if (`self.Saved Condition`)
        (set `/Game/Blueprints/Chars/Clones/Clone_Main.Black box` (`self.Black box`) _body)
        (`self.UnPossess`)
        (`/Game/Blueprints/Chars/Clones/Clone_Main.Setup as NPC` _body)
        (else
          (`/Game/Blueprints/Chars/Abstract/Base_Character.Die` (`self.Body`) null false (`/Game/Blueprints/recording/Death_info.Death impulse` _death_info) (`/Game/Blueprints/recording/Death_info.Hit location` _death_info) :!label _label_6)))
      (else
        (goto _label_6)))))

(fn `Aim on character`
  (params (Location :type "Vector Structure"))
  (bind _body (`self.Body`))
  (bind _returnvalue (`KismetMathLibrary.MakeRotator` 0.0 (.pitch (`self.Origin rotation`)) (`KismetMathLibrary.RadiansToDegrees` (`KismetMathLibrary.Vector_HeadingAngle` (- Location (`/Game/Blueprints/Chars/Abstract/Base_Character.SnipePoint Location` (`self.Body`)))))))
  (`/Game/Blueprints/Chars/Abstract/Base_Character.Set gun angle` _body _returnvalue)
  (`/Game/Blueprints/Chars/Abstract/Base_Character.Set gun angle` _body _returnvalue))

(fn `Are All Targets Dead`
  (returns (dead :type Boolean))
  (bind _targets (`/Game/Blueprints/recording/Black_Box.Targets` (`self.Black box`)))
  (`/Engine/EditorBlueprintResources/StandardMacros.CompareInt` (`KismetArrayLibrary.Array_Length` _targets)
    (:`>`
      (for _array_element _targets
        (bind _target (`self.Find shot target` _array_element))
        (`/Engine/EditorBlueprintResources/StandardMacros.IsValid` _target
          (:`Is Valid`
            (if (not (`/Game/Blueprints/Chars/Abstract/Base_Character.Dead` _target))
              (return false)))
          (:`Is Not Valid`
            (return false))))
      (return true))
    (:`==`
      (return false))))

(fn `Control Body`
  (params (`Frame info` :type "/Game/Blueprints/recording/Frame_Info Structure"))
  (bind (_time _location _gunrotation _bodyangle _speed _health _wantbeinvehicle _aimlocation _invehicle) (break `/Game/Blueprints/recording/Frame_Info` `Frame info`))
  (bind _body (`self.Body`))
  (if (== (`/Game/Blueprints/Chars/Abstract/Base_Character.In vehicle` (`self.Body`)) _invehicle)
    (set `/Game/Blueprints/Chars/Clones/Clone_Main.Recorded aim location` _aimlocation (`self.Body`))
    (`|ExecutionSequence`
      (:`then_0`
        (if _invehicle
          (set `/Game/Blueprints/Chars/Clones/Clone_Main.Speed_0` (0.0 0.0 0.0) (`self.Body`))
          (else
            (`/Game/Blueprints/Chars/Clones/Clone_Main.Rotate body repeater` (`self.Body`) _bodyangle)
            (`self.K2_SetActorLocation` (`self.Body`) _location false false)
            (set `/Game/Blueprints/Chars/Clones/Clone_Main.Speed_0` _speed (`self.Body`)))))
      (:`then_1`
        (set `/Game/Blueprints/Chars/Abstract/Base_Character.Want be in vehicle` _wantbeinvehicle (`self.Body`))
        (bind _output_get (set `self.Origin rotation` _gunrotation))
        (`|ExecutionSequence`
          (:`then_0`
            (if (not (`self.gun aim blocked`))
              (`/Game/Blueprints/Chars/Abstract/Base_Character.Set gun angle` _body _output_get)))
          (:`then_1`
            (if (`self.First read`)
              (`/Game/Blueprints/Chars/Abstract/Base_Character.Apply health` _body _health)
              (set `self.First read` false))))))
    (else
      (`self.Try to save`))))

(fn `Find shot target`
  (params (Hit_Info :type "/Game/Blueprints/recording/Hit_Info Structure (by ref)"))
  (returns (Target :type "/Game/Blueprints/Chars/Abstract/Base_Character Object Reference"))
  (locals (Result :type "/Game/Blueprints/Chars/Abstract/Base_Character Object Reference"))
  (bind (_target _indexinspawn) (break `/Game/Blueprints/recording/Hit_Info` Hit_Info))
  (bind _asactor (cast `Actor` (`/Game/Blueprints/System/FunctionLibrary.Find object by string` _target) :!pure true))
  (bind _asspawners (cast `/Game/Blueprints/Logics/Components/Spawners` _asactor)
    (:`then`
      (bind _spawned (`/Game/Blueprints/Logics/Components/Spawners.Get spawned` _asspawners))
      (bind _output (`|GetArrayItem` _spawned _indexinspawn))
      (`/Engine/EditorBlueprintResources/StandardMacros.IsValid` _output
        (:`Is Valid`
          (set `local.Result` _output))
        (:`Is Not Valid`
          (return null))))
    (:`CastFailed`
      (set `local.Result` (cast `/Game/Blueprints/Chars/Abstract/Base_Character` _asactor :!pure true))))
  (return (`local.Result`)))

(fn `Find shot targets`
  (params (`Hits info` :type "Array of /Game/Blueprints/recording/Hit_Info Structure"))
  (returns (Targets :type "Array of /Game/Blueprints/Chars/Abstract/Base_Character Object Reference") (`has dead target` :type Boolean))
  (locals (`Shot targets` :type "Array of /Game/Blueprints/Chars/Abstract/Base_Character Object Reference"))
  (for _array_element `Hits info`
    (bind _target (`self.Find shot target` _array_element))
    (`/Engine/EditorBlueprintResources/StandardMacros.IsValid` _target
      (:`Is Valid`
        (if (not (`/Game/Blueprints/Chars/Abstract/Base_Character.Dead` _target))
          (`KismetArrayLibrary.Array_Add` (`local.Shot targets`) _target)))))
  (return (`local.Shot targets`) false))

(fn `Get grid walker`
  (returns (`grid walker` :type "/Game/Blueprints/Navigation/Grid_Walker Object Reference"))
  (return null))

(fn `Get sound override`
  (returns (`Override params` :type "/Game/Sounds/Sound_Override Structure"))
  (return (`self.Sound overrides`)))

(fn `Insert Black Box`
  (params (`Black box` :type "/Game/Blueprints/recording/Black_Box Object Reference"))
  (bind _black_box (`self.Black box`))
  (set `self.Black box` `Black box`)
  (set `/Game/Blueprints/recording/Black_Box.locked` false _black_box)
  (set `/Game/Blueprints/Chars/Clones/Clone_Main.Clone number` (`/Game/Blueprints/recording/Black_Box.Clone number` _black_box) (`self.Body`))
  (`self.start checking for no targets`)
  (`self.start reading shots`)
  (`self.Start reading events`))

(fn `Mid Of Targets`
  (params (Targets :type "Array of /Game/Blueprints/Chars/Abstract/Base_Character Object Reference"))
  (returns (Location :type "Vector Structure"))
  (locals (`Sum location` :type "Vector Structure"))
  (for _array_element Targets
    (set `local.Sum location` (+ (`local.Sum location`) (`/Game/Blueprints/System/FunctionLibrary.Calculate Preemption` _array_element (`self.Body`)))))
  (return (/ (`local.Sum location`) (`KismetArrayLibrary.Array_Length` Targets))))

(fn `Saved Condition`
  (returns (Saved :type Boolean))
  (locals (`NPC posses health edge` :type "Float (double-precision)" :default 30.0) (`NPC posses health% edge` :type "Float (double-precision)" :default 50.0))
  (return (>= (`/Game/Blueprints/Chars/Abstract/Base_Character.Health` (`self.Body`)) (`local.NPC posses health edge`))))

(fn `UserConstructionScript`)