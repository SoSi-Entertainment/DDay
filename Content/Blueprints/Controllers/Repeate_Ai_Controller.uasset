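; AI controller that replays a BlackBox recording of movement, shooting and death on a Repeater pawn.
; Tick syncs recorded frames to game time, dropping late ones and delaying early ones, then applies transform, gun rotation and speed.
; A parallel shot loop resolves recorded victims by name or spawn index, overriding gun yaw toward their predicted positions for guaranteed hits.
; Once frames and shots run out, the body dies with the recorded impulse.
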(event `self.ReceivePossess`
  (params (PossessedPawn :type "Pawn Object Reference"))
  ;[1 1 1] setup
  (set `self.Body` (cast `/Game/Blueprints/Chars/Clones/Repeater` PossessedPawn :!pure true)))

(event `read black box`
  (bind _body (`self.Body`))
  ;[1 1 1] Shots
  (bind (_extracted _shot_time _hit _hits_info) (`/Game/Blueprints/recording/Black_Box.Extract shot` (`self.Black box`) :!label _label))
  (if _extracted
    (if _hit
      (`KismetSystemLibrary.Delay` _shot_time)
      (set `self.gun aim blocked` true)
      (bind _targets (`self.Find shot targets` _hits_info))
      (`/Engine/EditorBlueprintResources/StandardMacros.CompareInt` (`KismetArrayLibrary.Array_Length` _targets) 1
        (:`>`
          (bind _location (`self.Mid Of Targets` _targets))
          (set `self.Target location` _location)
          (`self.Aim on character` (`self.Target location`) :!label _label_2)
          (`/Game/Blueprints/Chars/Abstract/Base_Character.Gun Shoot` _body null true (0.0 0.0 0.0) false _targets)
          (goto _label))
        (:`==`
          (set `self.Target location` (`/Game/Blueprints/System/FunctionLibrary.Calculate Preemption` (`|GetArrayItem` _targets) (`self.Body`)))
          (goto _label_2))
        (:`<`
          (set `self.gun aim blocked` false)))
      (else
        (set `self.gun aim blocked` false)
        (`KismetSystemLibrary.Delay` _shot_time)))
    (`/Game/Blueprints/Chars/Abstract/Base_Character.Gun Shoot` _body null false (0.0 0.0 0.0) true _targets)
    (goto _label)
    (else
      (set `self.no ammo` true))))

(event `self.ReceiveTick`
  (params (DeltaSeconds :type "Float (single-precision)"))
  (bind _body (`self.Body`))
  (bind _death_info (`/Game/Blueprints/recording/Black_Box.Death info` (`self.Black box`)))
  ;[1 1 1] Body
  (set `self.wait condition` true)
  (while (and (`self.wait condition`) (not (`self.skip frame`)))
    (bind (_location _body_angle _rotation _speed _time _done) (`/Game/Blueprints/recording/Black_Box.Extract Frame` (`self.Black box`)))
    (if _done
      (bind _returnvalue (- _time (`KismetSystemLibrary.GetGameTimeInSeconds`)))
      (bind _output_get (set `self.delta frames` (/ _returnvalue DeltaSeconds)))
      (`/Engine/EditorBlueprintResources/StandardMacros.CompareInt` (`KismetMathLibrary.FTrunc` _output_get)
        (:`>`
          (set `self.delta time` _returnvalue)
          (set `self.skip frame` true))
        (:`==`
          (set `self.wait condition` false)))
      (else
        (set `self.wait condition` false))))
  (if (`self.skip frame`)
    (`KismetSystemLibrary.Delay` (`self.delta time`))
    (set `self.skip frame` false))
  (if _done
    (`self.Control Body` _location _body_angle _rotation _speed)
    (else
      (if (`self.no ammo`) :!label _label_3
        (if (not (`/Game/Blueprints/Chars/Abstract/Base_Character.Dead` _body))
          (`/Game/Blueprints/Chars/Abstract/Base_Character.Die` _body null (`/Game/Blueprints/recording/Death_info.Death impulse` _death_info) (`/Game/Blueprints/recording/Death_info.Hit location` _death_info))
          (`self.SetActorTickEnabled` false))
        (else
          (`KismetSystemLibrary.Delay` 0.1)
          (goto _label_3))))))

(fn `Aim on character`
  (params (Location :type "Vector Structure"))
  (bind _body (`self.Body`))
  (bind _returnvalue (`KismetMathLibrary.MakeRotator` 0.0 (.pitch (`self.Origin rotation`)) (`KismetMathLibrary.RadiansToDegrees` (`KismetMathLibrary.Vector_HeadingAngle` (- Location (`/Game/Blueprints/Chars/Abstract/Base_Character.SnipePoint Location` (`self.Body`)))))))
  (`/Game/Blueprints/Chars/Abstract/Base_Character.Set gun angle` _body _returnvalue)
  (`/Game/Blueprints/Chars/Abstract/Base_Character.Set gun angle` _body _returnvalue))

(fn `Control Body`
  (params (Location :type "Vector Structure") (`Body angle` :type "Float (double-precision)") (`Gun rotation` :type "Rotator Structure") (Speed :type "Vector Structure"))
  (`/Game/Blueprints/Chars/Clones/Repeater.Rotate body repeater` (`self.Body`) `Body angle`)
  (`self.K2_SetActorLocation` (`self.Body`) Location false false)
  (set `/Game/Blueprints/Chars/Clones/Repeater.Speed` Speed (`self.Body`))
  (bind _output_get (set `self.Origin rotation` `Gun rotation`))
  (if (not (`self.gun aim blocked`))
    (`/Game/Blueprints/Chars/Abstract/Base_Character.Set gun angle` (`self.Body`) _output_get)))

(fn `Find shot target`
  (params (`Target Name` :type String) (Index :type Integer))
  (returns (Target :type "/Game/Blueprints/Chars/Abstract/Base_Character Object Reference"))
  (locals (Result :type "/Game/Blueprints/Chars/Abstract/Base_Character Object Reference"))
  (bind _asactor (cast `Actor` (`|ConvertAsset` (`KismetSystemLibrary.Conv_SoftObjPathToSoftObjRef` (`KismetSystemLibrary.MakeSoftClassPath` `Target Name`))) :!pure true))
  (bind _asspawners (cast `/Game/Blueprints/Logics/Components/Spawners` _asactor)
    (:`then`
      (bind _spawned (`/Game/Blueprints/Logics/Components/Spawners.Get spawned` _asspawners))
      (bind _output (`|GetArrayItem` _spawned Index))
      (`/Engine/EditorBlueprintResources/StandardMacros.IsValid` _output
        (:`Is Valid`
          (set `local.Result` _output))
        (:`Is Not Valid`
          (return null))))
    (:`CastFailed`
      (set `local.Result` (cast `/Game/Blueprints/Chars/Abstract/Base_Character` _asactor :!pure true))))
  (return (`local.Result`)))

(fn `Find shot targets`
  (params (`Hits info` :type "Array of /Game/Blueprints/recording/Hit_Info Structure"))
  (returns (Targets :type "Array of /Game/Blueprints/Chars/Abstract/Base_Character Object Reference"))
  (locals (`Shot targets` :type "Array of /Game/Blueprints/Chars/Abstract/Base_Character Object Reference"))
  (for _array_element `Hits info`
    (bind (_target _indexinspawn) (break `/Game/Blueprints/recording/Hit_Info` _array_element))
    (bind _target_2 (`self.Find shot target` _target _indexinspawn))
    (`KismetArrayLibrary.Array_Add` (`local.Shot targets`) _target_2))
  (return (`local.Shot targets`)))

(fn `Get sound override`
  (returns (`Override params` :type "/Game/Sounds/Sound_Override Structure"))
  (return (`self.Sound overrides`)))

(fn `Insert Black Box`
  (params (`Black box` :type "/Game/Blueprints/recording/Black_Box Object Reference"))
  (set `self.Black box` `Black box`)
  (`self.read black box`))

(fn `Mid Of Targets`
  (params (Targets :type "Array of /Game/Blueprints/Chars/Abstract/Base_Character Object Reference"))
  (returns (Location :type "Vector Structure"))
  (locals (`Sum location` :type "Vector Structure"))
  (for _array_element Targets
    (set `local.Sum location` (+ (`local.Sum location`) (`/Game/Blueprints/System/FunctionLibrary.Calculate Preemption` _array_element (`self.Body`)))))
  (return (/ (`local.Sum location`) (`KismetArrayLibrary.Array_Length` Targets))))

(fn `UserConstructionScript`)