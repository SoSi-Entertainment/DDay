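; Short-lived fire ignition effect actor that flashes a point light and emits sparks, then removes itself.
; On BeginPlay it plays the FireIntense timeline at a sped-up rate to drive light intensity, scaled higher when the Single flag is set.
; After a brief delay it destroys the sparks particle component and then the actor.
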(event `self.ReceiveBeginPlay`
  (`self.control light`)
  (`KismetSystemLibrary.Delay` 0.1)
  (`ActorComponent.K2_DestroyComponent` (`self.P_Sparks_C`))
  (`self.K2_DestroyActor`))

(event `control light`
  (`TimelineComponent.SetPlayRate` (`self.fire intense`) (/ 1.0 0.2))
  (bind (_direction _intense) (`Timeline|fire intense`)
    (:`Update`
      (`LightComponent.SetIntensity` (`self.PointLight`) (* _intense (`KismetMathLibrary.SelectFloat` 300.0 150.0 (`self.single`)))))))

(fn `UserConstructionScript`)