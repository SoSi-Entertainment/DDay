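; BP_Thunder is an effect actor that fakes lightning by flashing a point light at random intervals.
; BeginPlay starts an endless Delay-driven loop that keeps the light dark for a random few seconds, then double-flashes it at LightIntens with short fixed gaps.
; The loop runs by wiring the last Delay back to the first intensity reset, so it needs no Tick, and it plays no sound.
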(event `self.ReceiveBeginPlay`
  (`LightComponent.SetIntensity` (`self.PointLight`) 0.0 :!label _label)
  (`KismetSystemLibrary.Delay` (`KismetMathLibrary.RandomFloatInRange` 5.0 10.0))
  (`LightComponent.SetIntensity` (`self.PointLight`) (`self.LightIntens`))
  (`KismetSystemLibrary.Delay` 0.1)
  (`LightComponent.SetIntensity` (`self.PointLight`) 0.0)
  (`KismetSystemLibrary.Delay` 0.1)
  (`LightComponent.SetIntensity` (`self.PointLight`) (`self.LightIntens`))
  (`KismetSystemLibrary.Delay` 0.1)
  (goto _label))

(fn `UserConstructionScript`)