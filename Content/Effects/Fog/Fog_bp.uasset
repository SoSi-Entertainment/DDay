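; Fog actor that renders a configurable fog effect on a Plane component through a dynamic instance of M_New_Fog_Gradient.
; The construction script creates the instance and InitParams copies the actor's variables into it: color, density, fades, mask, scroll speeds and gradient settings.
; InitDrop creates and stores a separate instance as DropDynamicMaterial, whose opacity SetDropOpacity later drives with a squared value.
; The event graph holds no active logic.
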(fn `Init drop`
  (bind _returnvalue (`PrimitiveComponent.CreateDynamicMaterialInstance` (`self.Plane`) 0 "/Game/Effects/Fog/Fogs/M_New_Fog_Gradient.M_New_Fog_Gradient" "None"))
  (bind _output_get (set `self.drop dynamic material` _returnvalue))
  (`self.Init params` _output_get))

(fn `Init params`
  (params (`dynamic mat inst` :type "MaterialInstanceDynamic Object Reference"))
  (`MaterialInstanceDynamic.SetVectorParameterValue` `dynamic mat inst` "Color" (`self.Color`))
  (`MaterialInstanceDynamic.SetScalarParameterValue` `dynamic mat inst` "Density" (`self.Density`))
  (`MaterialInstanceDynamic.SetScalarParameterValue` `dynamic mat inst` "DistanceFade" (`self.DistanceFade`))
  (`MaterialInstanceDynamic.SetScalarParameterValue` `dynamic mat inst` "FalloffExponent" (`self.FalloffExponent`))
  (`MaterialInstanceDynamic.SetScalarParameterValue` `dynamic mat inst` "Mask Size" (`self.Mask Size`))
  (`MaterialInstanceDynamic.SetScalarParameterValue` `dynamic mat inst` "Opacity" (`self.Opacity`))
  (`MaterialInstanceDynamic.SetScalarParameterValue` `dynamic mat inst` "Speed X" (`self.Speed X`))
  (`MaterialInstanceDynamic.SetScalarParameterValue` `dynamic mat inst` "Speed Y" (`self.Speed Y`))
  (`MaterialInstanceDynamic.SetTextureParameterValue` `dynamic mat inst` "Mask" (`self.Mask`))
  (`MaterialInstanceDynamic.SetScalarParameterValue` `dynamic mat inst` "GradientEdge" (`self.GradientEdge`))
  (`MaterialInstanceDynamic.SetScalarParameterValue` `dynamic mat inst` "IsGradient" (`KismetMathLibrary.Conv_BoolToDouble` (`self.UseGradient`)))
  (`MaterialInstanceDynamic.SetScalarParameterValue` `dynamic mat inst` "FadeIn/Out" (`KismetMathLibrary.Conv_BoolToDouble` (`self.FadeIn/Out`))))

(fn `Set drop opacity`
  (params (opacity :type "Float (double-precision)"))
  (`MaterialInstanceDynamic.SetScalarParameterValue` (`self.drop dynamic material`) "Opacity" (* opacity (`self.Opacity`))))

(fn `UserConstructionScript`
  (bind _returnvalue (`PrimitiveComponent.CreateDynamicMaterialInstance` (`self.Plane`) 0 "/Game/Effects/Fog/Fogs/M_New_Fog_Gradient.M_New_Fog_Gradient" "None"))
  (`self.Init params` _returnvalue))