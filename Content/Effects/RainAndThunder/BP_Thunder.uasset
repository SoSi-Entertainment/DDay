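; BP_Thunder is a looping lightning and thunder effect that flashes a point light at random positions.
; Each cycle moves the actor to a random X and Y within set intervals, waits a random time, then plays the thunder cue and a timeline.
; The timeline curve scales the light intensity to shape the flash, and its finish starts the next cycle.
; An older delay-based flicker loop remains unconnected.
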(event `self.ReceiveBeginPlay`
  (bind (_min _max) (break `FloatInterval` (`self.time interval`)))
  (bind (_min_2 _max_2) (break `FloatInterval` (`self.y interval`)))
  (bind (_min_3 _max_3) (break `FloatInterval` (`self.x interval`)))
  (`AudioComponent.Stop` (`self.Thunders_Cue`))
  (`self.K2_SetActorLocation` (`KismetMathLibrary.MakeVector` (`KismetMathLibrary.RandomFloatInRange` _min_3 _max_3) (`KismetMathLibrary.RandomFloatInRange` _min_2 _max_2) (.z (`self.K2_GetActorLocation`))) :!label _label)
  (`KismetSystemLibrary.Delay` (`KismetMathLibrary.RandomFloatInRange` _min _max))
  (`AudioComponent.Play` (`self.Thunders_Cue`) 0.0)
  (bind (_direction _intensity_coef) (`Timeline|Timeline` :!via `PlayFromStart`)
    (:`Update`
      (`LightComponent.SetIntensity` (`self.PointLight`) (* _intensity_coef (`self.LightIntens`))))
    (:`Finished`
      (goto _label))))

(fn `UserConstructionScript`)